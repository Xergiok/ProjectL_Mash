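; Camera modifier for the Concentration effect, adding radial blur and a vignette to the view.
; BlueprintModifyPostProcess lazily creates a dynamic instance of PP_RadialBlur and returns it as a full-weight post-process blendable.
; The modifier's Alpha drives both the clamped blur parameter and the vignette intensity, so both strengthen as it blends in.
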(fn `BlueprintModifyPostProcess`
  (params (DeltaTime :type "Float (double-precision)"))
  (returns (PostProcessBlendWeight :type "Float (double-precision)") (PostProcessSettings :type "PostProcessSettings Structure"))
  (`/Engine/EditorBlueprintResources/StandardMacros.IsValid` (`self.RadialBlur`)
    (:`Is Valid`
      _)
    (:`Is Not Valid`
      (bind _returnvalue (`KismetMaterialLibrary.CreateDynamicMaterialInstance` "/Game/Materials-Visual/VisualEffects_byJenya/PP_RadialBlur.PP_RadialBlur"))
      (set `self.RadialBlur` _returnvalue)))
  (`MaterialInstanceDynamic.SetScalarParameterValue` (`self.RadialBlur`) (`self.BlurParam_Name`) (`KismetMathLibrary.FClamp` (* (`self.Alpha`) 0.6) 0.0 0.6))
  (return 1.0 (make `PostProcessSettings` :`VignetteIntensity` (`KismetMathLibrary.FClamp` (+ (* (`self.Alpha`) 0.6) 0.4) 0.4) :`WeightedBlendables` (make `WeightedBlendables` (`|MakeArray` (make `WeightedBlendable` 1.0 (`self.RadialBlur`)))))))