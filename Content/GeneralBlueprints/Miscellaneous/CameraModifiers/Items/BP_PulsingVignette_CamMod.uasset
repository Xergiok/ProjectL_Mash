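; Camera modifier that gives the player's view a pulsing field of view and, as its name indicates, a vignette.
; Game time wrapped by PulsePeriod is remapped and fed through PulsingFunction to offset the camera manager's default FOV, replacing the incoming FOV.
; A fully weighted post-process pass takes its strength from a clamped Alpha, which nothing here updates.
; The Pulsing Function graph holds an unconnected logarithmic curve expression.
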(fn `BlueprintModifyCamera`
  (params (DeltaTime :type "Float (double-precision)") (ViewLocation :type "Vector Structure") (ViewRotation :type "Rotator Structure") (FOV :type "Float (double-precision)"))
  (returns (NewViewLocation :type "Vector Structure") (NewViewRotation :type "Rotator Structure") (NewFOV :type "Float (double-precision)"))
  (return ViewLocation ViewRotation (+ (`PlayerCameraManager.DefaultFOV` (`GameplayStatics.GetPlayerCameraManager` 0)) (* 3 (`self.Pulsing Function` (`KismetMathLibrary.MapRangeClamped` (mod (`KismetSystemLibrary.GetGameTimeInSeconds`) (`self.PulsePeriod`)) 0.0 (`self.PulsePeriod`) -1.0))))))

(fn `BlueprintModifyPostProcess`
  (params (DeltaTime :type "Float (double-precision)"))
  (returns (PostProcessBlendWeight :type "Float (double-precision)") (PostProcessSettings :type "PostProcessSettings Structure"))
  (return 1.0 (make `PostProcessSettings` :`VignetteIntensity` (`KismetMathLibrary.FClamp` (`self.Alpha`) 0.0 0.6))))