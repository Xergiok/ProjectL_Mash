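; Parent storage actor, apparently a base for storage items, with hooks for input control and paired item and character animation.
; BeginPlay caches BP_DefaultGameMode, and two events enable or disable the actor's input through the default player controller.
; PlaySequence and PlayMontage are empty stubs, as their synchronized animation calls are disconnected.
; The player and storage component setup and the animation-playing check are also unwired.
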(event `self.ReceiveBeginPlay`
  ;[1 1 1] Event BeginPlay
  (bind _asbp_default_game_mode (cast `/Game/GeneralBlueprints/Main/GameMods/BP_DefaultGameMode` (`GameplayStatics.GetGameMode`)))
  (bind _output_get (set `self.GameMode` _asbp_default_game_mode))
  (bind _playercharacter (`/Game/GeneralBlueprints/Main/GameMods/BP_DefaultGameMode.PlayerCharacter` _output_get)
    (:`then`)
    (:`else`)))

(event `Enable_Input_from_Item`
  ;[1 1 1] Control Actor Input
  (`self.EnableInput` (`/Game/GeneralBlueprints/Main/MacroLibrary/MCL_Actor_MacroLibrary.MCL_Get_DPController`)))

(event `Disable_Input_from_Item`
  ;[1 1 1] Control Actor Input
  (`self.DisableInput` (`/Game/GeneralBlueprints/Main/MacroLibrary/MCL_Actor_MacroLibrary.MCL_Get_DPController`)))

(event `Play Sequence`
  (params (Stop_existing :type Boolean) (Queued_playback :type Boolean) (Item_anim :type "AnimSequence Object Reference") (Character_anim :type "AnimSequence Object Reference") (InPlayRate :type "Float (double-precision)") (LoopCount :type Integer) (DynamicSlot :type Name))
  ;[1 1 1] Events that start playing animations together for the character and the item being used
)

(event `Play Montage`
  (params (Stop_existing :type Boolean) (Queued_playback :type Boolean) (Item_anim :type "AnimMontage Object Reference") (Character_anim :type "AnimMontage Object Reference") (InPlayRate :type "Float (double-precision)"))
  ;[1 1 1] Events that start playing animations together for the character and the item being used
)

(fn `UserConstructionScript`)