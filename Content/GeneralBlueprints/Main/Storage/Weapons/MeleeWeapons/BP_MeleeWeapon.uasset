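; BP_MeleeWeapon is a melee weapon actor that damages susceptible actors overlapping its DamageZone component.
; Hits send the weapon's Damage through an interface message and spawn a debug floating damage number at the sweep location.
; Actor collision is disabled on BeginPlay; the stab-animation and collision-toggling logic is left disconnected, so nothing here re-enables it.
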(event `self.ReceiveBeginPlay`
  (`parent.ReceiveBeginPlay`)
  (`self.SetActorEnableCollision` self false))

(event `self.DamageZone.OnComponentBeginOverlap`
  (params (OverlappedComponent :type "PrimitiveComponent Object Reference") (OtherActor :type "Actor Object Reference") (OtherComp :type "PrimitiveComponent Object Reference") (OtherBodyIndex :type Integer) (bFromSweep :type Boolean) (SweepResult :type "HitResult Structure (by ref)"))
  (bind (_bblockinghit _binitialoverlap _time _distance _location _impactpoint _normal _impactnormal _physmat _hitactor) (`GameplayStatics.BreakHitResult` SweepResult))
  (bind _damage (`self.Damage`))
  (`/Game/GeneralBlueprints/Main/MacroLibrary/MCL_Object_MacroLibrary.MCL_Susceptible_to_damage` _hitactor
    (:`T`
      (message `/Game/GeneralBlueprints/Main/Interfaces/BPI_DamageInterface.Taking_Damage_BPIF` _hitactor _damage "NewEnumerator0" self)
      ;[1 0 0.2187] Debug
      (`|SpawnActorFromClass` "/Game/GeneralBlueprints/Widget/debugHUD/BP_FloatingText.BP_FloatingText_C" (`KismetMathLibrary.MakeTransform` _location) "Undefined" "OverrideRootScale" null (`KismetTextLibrary.Conv_DoubleToText` _damage "HalfToEven" false true 1 324 0 0) null))))

(fn `UserConstructionScript`
  (`parent.UserConstructionScript`))