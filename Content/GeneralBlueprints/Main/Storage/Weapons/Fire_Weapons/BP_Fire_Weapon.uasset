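; Base firearm Blueprint that handles shooting, ammo and reloading, loading stats and animations from DataTables by row name.
; Shots trace from the player or sight camera, then spawn a revolver bullet from the muzzle toward that point, with doubled damage on the last round.
; Ammo checks route firing, blank shots and optional auto-reload; interface events move rounds during reloads.
; Part reload, custom fire animation and model refresh are empty hooks.
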(event `self.ReceiveBeginPlay`
  ;[1 1 1] Event Begin Play
  (`parent.ReceiveBeginPlay`)
  ;;[1 1 1] Initial filling of the magazine when picking up weapons of this type
  (`self.Update_bullet` (`KismetMathLibrary.Clamp` (`self.InitialAmmo`) 0 (`.Magazine_Size_34_F5BCAC034039685CAE4838AD2A77C316` (break `/Game/GeneralBlueprints/Miscellanious/Weapon/ST_FireWeaponParams` (`self.WeaponParams`))))))

(event `StartFire`
  ;[1 1 1] Shot processing, trajectory calculation and bullet launch
  (switch `/Game/GeneralBlueprints/Miscellanious/Weapon/E_FireMode` "NewEnumerator0"
    (:`NewEnumerator0`
      (`/Engine/EditorBlueprintResources/StandardMacros.Gate` false :!label _label
        (:`Exit`
          (`|ExecutionSequence`
            (:`then_0`
              (`KismetSystemLibrary.Delay` 0.2)
              (`self.Spawn Projectile and Shot`)
              (goto _label :!via `Close`))
            (:`then_1`
              (`KismetSystemLibrary.Delay` 0.2)
              (goto _label :!via `Open`))))))
    (:`NewEnumerator1`
      (`|ExecutionSequence`
        (:`then_0`
          (goto _label_2 :!via `Open`))
        (:`then_1`
          (`/Engine/EditorBlueprintResources/StandardMacros.Gate` true :!label _label_2
            (:`Exit`
              (`|ExecutionSequence`
                (:`then_0`
                  (`KismetSystemLibrary.Delay` 0.2)
                  (goto _label_2))
                (:`then_1`
                  (`self.Spawn Projectile and Shot`))))))))))

(event `StopFire`
  ;[1 1 1] Shot processing, trajectory calculation and bullet launch
  (goto _label_2 :!via `Close`))

(event `Update_bullet`
  (params (set_bullets :type Integer) (add :type Boolean))
  (bind (_firemode _muzzlename _firerate _fireinputdelay _standart_weaponspread _mindamage _maxdamage _currentammunition _maxammunition _magazine_size _currentammo) (break `/Game/GeneralBlueprints/Miscellanious/Weapon/ST_FireWeaponParams` (`self.WeaponParams`)))
  ;[1 1 1] Updating the number of rounds in the magazine and changing the number of cartridges in the clip (after firing or reloading)
  (set `self.WeaponParams` (make `/Game/GeneralBlueprints/Miscellanious/Weapon/ST_FireWeaponParams` _firemode _muzzlename _firerate _fireinputdelay _standart_weaponspread _mindamage _maxdamage _currentammunition _maxammunition _magazine_size (`self.Calculate_CurrentAmmo` _currentammo set_bullets add)))
  (if (and (`self.Enable_Autoreload`) (== (`self.Get_CurrentAmmo`) 0))
    (`self.AutoReload`))
  (`self.Refresh_PhysModel`))

(event `Update_CurrenAmmunition`
  (params (Set_CurrentAmmunition :type Integer) (Add :type Boolean))
  (bind (_firemode _muzzlename _firerate _fireinputdelay _standart_weaponspread _mindamage _maxdamage _currentammunition _maxammunition _magazine_size _currentammo) (break `/Game/GeneralBlueprints/Miscellanious/Weapon/ST_FireWeaponParams` (`self.WeaponParams`)))
  ;[1 1 1] Comment
  (set `self.WeaponParams` (make `/Game/GeneralBlueprints/Miscellanious/Weapon/ST_FireWeaponParams` _firemode _muzzlename _firerate _fireinputdelay _standart_weaponspread _mindamage _maxdamage (`self.Calculate_MaxAmmo` _currentammunition Set_CurrentAmmunition Add) _maxammunition _magazine_size _currentammo)))

(event `Start_Reload`
  ;[1 1 1] Reload Events
  (if (`self.Reloading?`)
    (if (`self.Use_Part_Reload`)
      (`self.Put_One_Bullet`))
    (else
      (`self.Check_Ammo`
        (:`Magazine full`
          _)
        (:`Has some ammo in the magazine`
          _)
        (:`Empty magazine (has ammo)`
          _))
      (`self.ReloadWeapon`))))

(event `AutoReload`
  ;[1 1 1] Reload Events
  (`self.Check_Ammo`
    (:`Empty magazine (has ammo)`
      (`self.ReloadWeapon`))))

(event `ReloadWeapon`
  (bind (_animmontage_weapon_reload _animmontage_character_reload) (`self.Get_Reload_Anims`))
  ;[1 1 1] Reload Events
  (set `self.Reloading?` true)
  (if (`self.Use_Part_Reload`)
    (`self.Part_Reload`)
    (else
      (`self.Play Montage` true false _animmontage_weapon_reload _animmontage_character_reload 1.0)
      (`KismetSystemLibrary.Delay` (`KismetMathLibrary.FMax` (`AnimSequenceBase.SequenceLength` _animmontage_weapon_reload) (`AnimSequenceBase.SequenceLength` _animmontage_character_reload)))
      (set `self.Reloading?` false))))

(event `/Game/GeneralBlueprints/Main/Interfaces/BPI_CharacterAnimInterface.AddOneBullet_BPIF`
  ;[1 1 1] Interface Events
  (`self.Check_Ammo`
    (:`Has some ammo in the magazine`
      _)
    (:`Empty magazine (has ammo)`
      _))
  (`self.Update_CurrenAmmunition` -1 true)
  (`self.update_bullet` 1 true))

(event `/Game/GeneralBlueprints/Main/Interfaces/BPI_CharacterAnimInterface.DropAllMagazine_BPIF`
  ;[1 1 1] Interface Events
  (`self.Check_Ammo`
    (:`Magazine full`
      _)
    (:`Has some ammo in the magazine`
      _))
  (`self.update_bullet` 0))

(fn `Calculate_CurrentAmmo`
  (params (CurrentAmmo :type Integer) (Variation :type Integer) (Add :type Boolean))
  (returns (ReturnValue :type Integer))
  (return (`KismetMathLibrary.Clamp` (`KismetMathLibrary.SelectInt` (+ CurrentAmmo Variation) Variation Add) 0 (`.Magazine_Size_34_F5BCAC034039685CAE4838AD2A77C316` (break `/Game/GeneralBlueprints/Miscellanious/Weapon/ST_FireWeaponParams` (`self.WeaponParams`))))))

(fn `Calculate_Damage`
  (returns (ReturnValue :type "Float (double-precision)"))
  (bind ((`MinDamage_12_327A9AEF4F86C2BEFED3739B7F182B45` _mindamage) (`MaxDamage_14_26045AE34A2C92DDFAF5868FD9FA5C1E` _maxdamage) (`CurrentAmmo_23_0D7E572E4839A74EDEC6EEB35228A84B` _currentammo)) (break `/Game/GeneralBlueprints/Miscellanious/Weapon/ST_FireWeaponParams` (`self.WeaponParams`)))
  (bind _returnvalue (`KismetMathLibrary.RandomFloatInRange` _mindamage _maxdamage))
  (return (`KismetMathLibrary.SelectFloat` (* _returnvalue 2.0) _returnvalue (== _currentammo 1))))

(fn `Calculate_Direction`
  (returns (Location :type "Vector Structure") (Rotation :type "Rotator Structure"))
  (bind _returnvalue (`self.Get_MuzzlePosition`))
  (bind _player (`self.Player`)
    (:`then`
      (bind (_returnvalue_location _returnvalue_rotation) (`KismetMathLibrary.BreakTransform` (`SceneComponent.K2_GetComponentToWorld` (select `bool` (`/Game/GeneralBlueprints/Main/Characters/Player/BP_HumanCharacter.Aiming` _player) :`false` (`/Game/GeneralBlueprints/Main/Characters/Player/BP_HumanCharacter.FP Camera` _player) :`true` (`self.Sight camera`)))))
      (bind _returnvalue_2 (`KismetMathLibrary.GetForwardVector` _returnvalue_rotation))
      (bind _returnvalue_3 (+ _returnvalue_location (* _returnvalue_2 100000.0)))
      (bind (_outhit _returnvalue_4) (`KismetSystemLibrary.LineTraceSingleForObjects` :`Start` (+ _returnvalue_location (* _returnvalue_2 (`KismetMathLibrary.VSize` (- _returnvalue_location (`self.Get_MuzzlePosition`))))) :`End` _returnvalue_3 :`ObjectTypes` (`|MakeArray` "ObjectTypeQuery1" :!type "EObjectTypeQuery Enum") :`DrawDebugType` "ForDuration" :`TraceColor` (struct :`R` 0.006503 :`B` 0.601042 :`A` 1.0) :`TraceHitColor` (struct :`R` 0.274446 :`G` 1.0 :`A` 1.0)))
      (return _returnvalue (`KismetMathLibrary.FindLookAtRotation` _returnvalue (`KismetMathLibrary.SelectVector` (`.ImpactPoint` (`GameplayStatics.BreakHitResult` _outhit)) _returnvalue_3 _returnvalue_4))))
    (:`else`)))

(fn `Calculate_FinalDirection`
  (params (StartLoc :type "Vector Structure") (StartRot :type "Rotator Structure"))
  (returns (Transform :type "Transform Structure"))
  (bind _returnvalue (* 0.0 -1.0))
  (return (`KismetMathLibrary.MakeTransform` StartLoc (`KismetMathLibrary.ComposeRotators` StartRot (`KismetMathLibrary.MakeRotator` (`KismetMathLibrary.RandomFloatInRange` _returnvalue) (`KismetMathLibrary.RandomFloatInRange` _returnvalue) (`KismetMathLibrary.RandomFloatInRange` _returnvalue))))))

(fn `Calculate_MaxAmmo`
  (params (Current :type Integer) (Variation :type Integer) (Add :type Boolean))
  (returns (ReturnValue :type Integer))
  (return (`KismetMathLibrary.Clamp` (`KismetMathLibrary.SelectInt` (+ Current Variation) Variation Add) 0 (`.MaxAmmunition_70_97D5F94547DB25A8B66B68980F20BE78` (break `/Game/GeneralBlueprints/Miscellanious/Weapon/ST_FireWeaponParams` (`self.WeaponParams`))))))

(fn `Custom_FireAnim`)

(fn `Part_Reload`)

(fn `Put_One_Bullet`)

(fn `Refresh_PhysModel`)

(fn `Spawn Projectile and Shot`
  (bind (_animmontage_weapon_fire _animmontage_character_fire _animmontage_weapon_blankshot _animmontage_character_blankshot) (`self.Get_Fire_Anims`))
  (bind (_animmontage_weapon_fire_2 _animmontage_character_fire_2) (`self.Get_Fire_Anims`))
  (`|ExecutionSequence`
    (:`then_0`
      (if (`self.Reloading?`)
        (`self.Play Sequence` true false null null 1.0 1)
        (set `self.Reloading?` false)))
    (:`then_1`
      (`self.Check_Ammo`
        (:`Magazine full`
          (bind (_location _rotation) (`self.Calculate_Direction` :!label _label))
          (bind _transform (`self.Calculate_FinalDirection` _location _rotation))
          (`/Engine/EditorBlueprintResources/StandardMacros.IsValid` (`self.Player`)
            (:`Is Valid`
              (`|ExecutionSequence`
                (:`then_0`
                  (if (`self.UseCustomFireAnim`)
                    (`self.Custom_FireAnim`)
                    (else
                      (`self.Play Montage` true false _animmontage_weapon_fire_2 _animmontage_character_fire_2 1.0))))
                (:`then_1`
                  (if (> (`self.Get_CurrentAmmo`) 0)
                    (`|SpawnActorFromClass` "/Game/GeneralBlueprints/Main/Storage/Weapons/Bullets/Pistol_Bullets/BP_Revolver_Bullet.BP_Revolver_Bullet_C" _transform "Undefined" "OverrideRootScale" null (`self.Calculate_Damage`) null)
                    (`/Game/GeneralBlueprints/Main/Storage/Weapons/Fire_Weapons/Revolver/BP_Weapon_Revolver.update_bullet` -1 true)))))))
        (:`Has some ammo in the magazine`
          (goto _label))
        (:`Empty magazine (has ammo)`
          (`self.Play Montage` true false _animmontage_weapon_blankshot _animmontage_character_blankshot 1.0 :!label _label_2))
        (:`No ammo at all`
          (goto _label_2))))))

(fn `UserConstructionScript`
  (`parent.UserConstructionScript`)
  (bind _returnvalue (`|GetDataTableRow` "/Game/GeneralBlueprints/Miscellanious/Weapon/DT_FireWeaponsParams.DT_FireWeaponsParams" (`self.WeaponRowName`))
    (:`then`
      (set `self.WeaponParams` _returnvalue)
      (bind _returnvalue_2 (`|GetDataTableRow` "/Game/GeneralBlueprints/Miscellanious/Weapon/DT_FireWeaponsAnimations.DT_FireWeaponsAnimations" (`self.WeaponRowName`))
        (:`then`
          (set `self.WeaponAnims` _returnvalue_2))))))