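; Base bullet actor that deals damage on hit and expires after a fixed lifespan.
; On hit, damageable actors receive an interface damage message, doubled for head or neck bones, plus debug floating damage text.
; Other actors get an impact emitter, and physics-simulating components receive a velocity-scaled impulse.
; The bullet then destroys itself unless flagged Permanent.
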(event `self.ReceiveBeginPlay`
  (`self.SetLifeSpan` 30.0))

(event `self.ReceiveHit`
  (params (MyComp :type "PrimitiveComponent Object Reference") (Other :type "Actor Object Reference") (OtherComp :type "PrimitiveComponent Object Reference") (bSelfMoved :type Boolean) (HitLocation :type "Vector Structure") (HitNormal :type "Vector Structure") (NormalImpulse :type "Vector Structure") (Hit :type "HitResult Structure (by ref)"))
  (bind (_bblockinghit _binitialoverlap _time _distance _location _impactpoint _normal _impactnormal _physmat _hitactor _hitcomponent _hitbonename) (`GameplayStatics.BreakHitResult` Hit))
  (bind _damage (`self.Damage`))
  (bind _returnvalue (`self.Select_Hitbox` _hitbonename))
  (`/Game/GeneralBlueprints/Main/MacroLibrary/MCL_Object_MacroLibrary.MCL_Susceptible_to_damage` _hitactor
    (:`T`
      (message `/Game/GeneralBlueprints/Main/Interfaces/BPI_DamageInterface.Taking_Damage_BPIF` _hitactor (select `/Game/GeneralBlueprints/Miscellanious/Hitbox/E_NPC_Hitbox` _returnvalue :`NewEnumerator0` _damage :`NewEnumerator1` (* _damage 2.0)) _returnvalue self)
      ;[1 0 0.2187] Debug
      (`self.Debug_FloatDamageText` _location (`KismetTextLibrary.Conv_StringToText` (select `/Game/GeneralBlueprints/Miscellanious/Hitbox/E_NPC_Hitbox` _returnvalue :`NewEnumerator0` (`KismetTextLibrary.Conv_TextToString` (`KismetTextLibrary.Conv_DoubleToText` _damage "HalfToEven")) :`NewEnumerator1` "Head"))))
    (:`F`
      (`GameplayStatics.SpawnEmitterAtLocation` null _location)))
  (`self.Simulating_physics?` _hitcomponent
    (:`true`
      (`PrimitiveComponent.AddImpulseAtLocation` OtherComp (* (`self.GetVelocity`) 10.0) (`self.K2_GetActorLocation`) "None"))
    (:`false`
      _))
  (if (not (`self.Permanent`))
    (`self.K2_DestroyActor`)))

(fn `Debug_FloatDamageText`
  (params (SpawnTransform_Location :type "Vector Structure") (Value :type Text))
  (`|SpawnActorFromClass` "/Game/GeneralBlueprints/Widget/debugHUD/BP_FloatingText.BP_FloatingText_C" (`KismetMathLibrary.MakeTransform` SpawnTransform_Location) "Undefined" "OverrideRootScale" null Value null))

(fn `Select_Hitbox`
  (params (Bone_Name :type Name))
  (returns (ReturnValue :type "/Game/GeneralBlueprints/Miscellanious/Hitbox/E_NPC_Hitbox Enum"))
  (return (select `bool` (or (== Bone_Name "neck_01") (== Bone_Name "head")) :`false` "NewEnumerator0" :`true` "NewEnumerator1" :!type "/Game/GeneralBlueprints/Miscellanious/Hitbox/E_NPC_Hitbox Enum")))

(fn `UserConstructionScript`)