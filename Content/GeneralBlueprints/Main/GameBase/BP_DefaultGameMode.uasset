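; Default game mode Blueprint that caches references to the human player and relays input settings to it.
; On BeginPlay it casts and stores player 0's character, its controller, and the human animation instance from the character's skeletal mesh.
; A separate update function copies hold-input options for crouch, walk and sprint from its input settings struct to the character.
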(event `self.ReceiveBeginPlay`
  (`self.Add_Maintain_References`))

(fn `Add_Maintain_References`
  (`|ExecutionSequence`
    (:`then_0`
      (bind _asbp_char_human (cast `/Game/GeneralBlueprints/Main/Characters/Player/BP_Char_Human` (`GameplayStatics.GetPlayerCharacter` 0)))
      (set `self.PlayerCharacter` _asbp_char_human))
    (:`then_1`
      (bind _asbp_default_player_controller (cast `/Game/GeneralBlueprints/Main/Control/PlayerControllers/BP_DefaultPlayerController` (`GameplayStatics.GetPlayerController` 0)))
      (set `self.PlayerController` _asbp_default_player_controller))
    (:`then_2`
      (bind _playercharacter (`self.PlayerCharacter`)
        (:`then`
          (bind _asabp_general_human_character (cast `/Game/AnimAssets/Characters/TestChar/Animations/TestCharAnims/CharAnimationInstances/ABP_General_HumanCharacter` (`SkeletalMeshComponent.GetAnimInstance` (`self.GetComponentByClass` _playercharacter "/Script/Engine.SkeletalMeshComponent"))))
          (set `self.Player Animation` _asabp_general_human_character))
        (:`else`)))))

(fn `Update_PlayerSettings`
  (`|ExecutionSequence`
    (:`then_0`
      (set `/Game/GeneralBlueprints/Main/Characters/Player/BP_Char_Human.crouch_settings_hold` (`.InputSettings_Crouch_Hold_3_59ED9E7F4470D4E8892935B6FA4A0FC3` (break `/Game/GeneralBlueprints/Miscellaneous/KeySettings/ST_Player_KeypressSettings` (`self.ST_Input_Settings`))) (`self.PlayerCharacter`)))
    (:`then_1`
      (set `/Game/GeneralBlueprints/Main/Characters/Player/BP_Char_Human.walk_settings_hold` (`.InputSettings_Walk_Hold_4_C5E9AA7142969297911FE49B5829AC61` (break `/Game/GeneralBlueprints/Miscellaneous/KeySettings/ST_Player_KeypressSettings` (`self.ST_Input_Settings`))) (`self.PlayerCharacter`)))
    (:`then_2`
      (set `/Game/GeneralBlueprints/Main/Characters/Player/BP_Char_Human.sprint_settings_hold` (`.InputSettings_Sprint_Hold_5_26A9FF3E489CB4926C0588AF4987C67E` (break `/Game/GeneralBlueprints/Miscellaneous/KeySettings/ST_Player_KeypressSettings` (`self.ST_Input_Settings`))) (`self.PlayerCharacter`)))))

(fn `UserConstructionScript`)