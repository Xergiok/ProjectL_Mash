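; Default player camera manager that limits how far the player can look, with separate boundaries for normal and inventory modes.
; A shared setter applies a boundaries struct to view pitch and yaw limits, and optionally roll, starting from normal boundaries at construction.
; Inventory mode caps upward pitch and centers a yaw window on the pawn's aim.
; An optional looping timer re-centers yaw limits on pawn forward, and returning to normal can realign control yaw.
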(event `Boundaries_NormalMode`
  (params (Reset_PlayerRotation :type Boolean))
  (bind _returnvalue (`GameplayStatics.GetPlayerController` 0))
  (bind (_returnvalue_roll _returnvalue_pitch) (`KismetMathLibrary.BreakRotator` (`Controller.GetControlRotation` _returnvalue)))
  (`self.Set_Boundaries` (`self.Normal_Boundaries`))
  (if Reset_PlayerRotation
    (`Controller.SetControlRotation` _returnvalue (`KismetMathLibrary.MakeRotator` _returnvalue_roll _returnvalue_pitch (`KismetMathLibrary.GetYawPitchFromVector` (`self.GetActorForwardVector` (`GameplayStatics.GetPlayerPawn` 0)))))))

(event `Boundaries_InventoryMode`
  (bind _boundaries_pitch_rangeminmax (break `/Game/GeneralBlueprints/Miscellaneous/CharacterDefaults/Camera/ST_CameraBoundaries` (`self.Boundaries`)))
  (bind (_returnvalue_roll _returnvalue_pitch _returnvalue_yaw) (`KismetMathLibrary.BreakRotator` (`Pawn.GetBaseAimRotation` (`GameplayStatics.GetPlayerPawn` 0))))
  (`self.Set_Boundaries` (make `/Game/GeneralBlueprints/Miscellaneous/CharacterDefaults/Camera/ST_CameraBoundaries` (`KismetMathLibrary.MakeVector2D` (`KismetMathLibrary.BreakVector2D` _boundaries_pitch_rangeminmax) -50.0) (`KismetMathLibrary.MakeVector2D` (- _returnvalue_yaw 70.0) (+ _returnvalue_yaw 70.0)))))

(event `Should_UpdateBoundaries`
  (params (Update :type Boolean))
  (if Update
    (bind _returnvalue (`KismetSystemLibrary.K2_SetTimerDelegate` (delegate `Update_YawBoundaries`) 0.1 true))
    (set `self.Boundaries_Timer` _returnvalue)
    (else
      (`KismetSystemLibrary.K2_ClearAndInvalidateTimerHandle` (`self.Boundaries_Timer`)))))

(event `Update_YawBoundaries`
  (bind _boundaries_pitch_rangeminmax (break `/Game/GeneralBlueprints/Miscellaneous/CharacterDefaults/Camera/ST_CameraBoundaries` (`self.Boundaries`)))
  (bind (_x _y) (`KismetMathLibrary.BreakVector2D` _boundaries_pitch_rangeminmax))
  (bind _yaw (`KismetMathLibrary.GetYawPitchFromVector` (`self.GetActorForwardVector` (`GameplayStatics.GetPlayerPawn` 0))))
  (set `self.ViewPitchMin` _x)
  (set `self.ViewPitchMax` _y)
  (set `self.ViewYawMin` (- _yaw 70.0))
  (set `self.ViewYawMax` (+ _yaw 70.0)))

(fn `Set Pitch Range`
  (params (ViewPitchMax :type "Float (double-precision)") (ViewPitchMin :type "Float (double-precision)"))
  (set `self.ViewPitchMax` ViewPitchMax)
  (set `self.ViewPitchMin` ViewPitchMin))

(fn `Set_Boundaries`
  (params (Boundaries :type "/Game/GeneralBlueprints/Miscellaneous/CharacterDefaults/Camera/ST_CameraBoundaries Structure") (Roll :type Boolean))
  (bind _output_get (set `self.Boundaries` Boundaries))
  (`|ExecutionSequence`
    (:`then_0`
      (bind (_x _y) (`KismetMathLibrary.BreakVector2D` (break `/Game/GeneralBlueprints/Miscellaneous/CharacterDefaults/Camera/ST_CameraBoundaries` _output_get)))
      (set `self.ViewPitchMin` _x)
      (set `self.ViewPitchMax` _y)
      (bind (_x_2 _y_2) (`KismetMathLibrary.BreakVector2D` (`.Yaw_RangeMinMax_26_32A996C6431F2BBDB35DE0895831ACD4` (break `/Game/GeneralBlueprints/Miscellaneous/CharacterDefaults/Camera/ST_CameraBoundaries` _output_get))))
      (set `self.ViewYawMin` _x_2)
      (set `self.ViewYawMax` _y_2))
    (:`then_1`
      (if Roll
        (bind (_x_3 _y_3) (`KismetMathLibrary.BreakVector2D` (`.Roll_RangeMinMax_27_26DE2100488875D031386C9C65DEBF49` (break `/Game/GeneralBlueprints/Miscellaneous/CharacterDefaults/Camera/ST_CameraBoundaries` _output_get))))
        (set `self.ViewRollMin` _x_3)
        (set `self.ViewRollMax` _y_3)))))

(fn `UserConstructionScript`
  (`self.Set_Boundaries` (`self.Normal_Boundaries`) true))