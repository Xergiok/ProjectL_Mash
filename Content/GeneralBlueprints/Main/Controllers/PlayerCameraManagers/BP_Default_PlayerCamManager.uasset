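; Default player camera manager that limits view pitch and yaw through a boundaries struct, initialized with defaults on construction.
; Yaw limits can be recentred on the pawn's forward vector, narrowed around aim yaw for inventory mode, or restored to defaults, optionally realigning control yaw with the pawn.
; A toggleable distortion effect pairs a camera modifier with an FOV oscillation shake, keeping both instances for removal.
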(event `Set_Boundaries`
  (params (Boundaries :type "/Game/GeneralBlueprints/Miscellaneous/CharacterDefaults/Camera/ST_CameraBoundaries Structure"))
  (bind _output_get (set `self.Boundaries` Boundaries))
  (set `self.ViewPitchMin` (break `/Game/GeneralBlueprints/Miscellaneous/CharacterDefaults/Camera/ST_CameraBoundaries` _output_get))
  (set `self.ViewPitchMax` (`.Pitch_Max_6_F410AC8B472EE63D8E90CD8DFB826A15` (break `/Game/GeneralBlueprints/Miscellaneous/CharacterDefaults/Camera/ST_CameraBoundaries` _output_get)))
  (set `self.ViewYawMin` (`.Yaw_Min_8_64B30B63490D1BBBAA082482CB4B99EE` (break `/Game/GeneralBlueprints/Miscellaneous/CharacterDefaults/Camera/ST_CameraBoundaries` _output_get)))
  (set `self.ViewYawMax` (`.Yaw_Max_7_53A8C05B4729C6BCDB1106963FB17DD6` (break `/Game/GeneralBlueprints/Miscellaneous/CharacterDefaults/Camera/ST_CameraBoundaries` _output_get))))

(event `Update Yaw Boundaries`
  (bind (_boundaries_pitch_min _boundaries_pitch_max _boundaries_yaw_min _boundaries_yaw_max) (break `/Game/GeneralBlueprints/Miscellaneous/CharacterDefaults/Camera/ST_CameraBoundaries` (`self.Boundaries`)))
  (bind _yaw (`KismetMathLibrary.GetYawPitchFromVector` (`self.GetActorForwardVector` (`GameplayStatics.GetPlayerPawn` 0))))
  (`self.Set_Boundaries` (make `/Game/GeneralBlueprints/Miscellaneous/CharacterDefaults/Camera/ST_CameraBoundaries` _boundaries_pitch_min _boundaries_pitch_max (- _yaw _boundaries_yaw_min) (+ _yaw _boundaries_yaw_max))))

(event `Start_DistortionEffect`
  (bind _returnvalue (`self.AddNewCameraModifier` "/Game/GeneralBlueprints/Miscellaneous/CameraModifiers/BP_Distortion_CamMod.BP_Distortion_CamMod_C"))
  (bind _returnvalue_2 (`self.PlayCameraShake` "/Game/GeneralBlueprints/Miscellaneous/CameraShake/FOV_Ocillation.FOV_Ocillation_C" 0.5)))

(event `Stop_DistortionEffect`
  (`self.RemoveCameraModifier` (stale `Start_DistortionEffect` _returnvalue))
  (`self.StopCameraShake` (stale `Start_DistortionEffect` _returnvalue_2) false))

(event `Boundaries_InventoryMode`
  (bind (_boundaries_pitch_min _boundaries_pitch_max) (break `/Game/GeneralBlueprints/Miscellaneous/CharacterDefaults/Camera/ST_CameraBoundaries` (`self.Boundaries`)))
  (bind (_returnvalue_roll _returnvalue_pitch _returnvalue_yaw) (`KismetMathLibrary.BreakRotator` (`Pawn.GetBaseAimRotation` (`GameplayStatics.GetPlayerPawn` 0))))
  (`self.Set_Boundaries` (make `/Game/GeneralBlueprints/Miscellaneous/CharacterDefaults/Camera/ST_CameraBoundaries` _boundaries_pitch_min _boundaries_pitch_max (- _returnvalue_yaw 70.0) (+ _returnvalue_yaw 70.0))))

(event `Boundaries_NormalMode`
  (params (Reset_PlayerRotation :type Boolean))
  (bind _returnvalue (`GameplayStatics.GetPlayerController` 0))
  (bind (_returnvalue_roll _returnvalue_pitch) (`KismetMathLibrary.BreakRotator` (`Controller.GetControlRotation` _returnvalue)))
  (`self.Set_Boundaries` (make `/Game/GeneralBlueprints/Miscellaneous/CharacterDefaults/Camera/ST_CameraBoundaries` -80.0))
  (if Reset_PlayerRotation
    (`Controller.SetControlRotation` _returnvalue (`KismetMathLibrary.MakeRotator` _returnvalue_roll _returnvalue_pitch (`KismetMathLibrary.GetYawPitchFromVector` (`self.GetActorForwardVector` (`GameplayStatics.GetPlayerPawn` 0)))))))

(fn `Set Pitch Range`
  (params (ViewPitchMax :type "Float (double-precision)") (ViewPitchMin :type "Float (double-precision)"))
  (set `self.ViewPitchMax` ViewPitchMax)
  (set `self.ViewPitchMin` ViewPitchMin))

(fn `UserConstructionScript`
  (`self.Set_Boundaries` (make `/Game/GeneralBlueprints/Miscellaneous/CharacterDefaults/Camera/ST_CameraBoundaries` -80.0)))