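; Default player controller that handles pause, interaction, evidence pickup, danger detection, clamped FOV and smoothed control rotation.
; Tick sphere-traces for enemies; sighting one or being in a danger zone sets IsInDanger, cleared through a retriggerable delay.
; Main and side actions go to the pawn's interaction component, while Detective traces and destroys evidence, only printing an inventory message.
; Physics-handle grab and drop helpers exist, but the held-object target update is unwired.
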(event `self.ReceiveBeginPlay`
  ;[1 0.4676 0] Event BeginPlay
  (`self.Set_ClampedFOV` (`self.Base_FOV`)))

(event `self.ReceiveTick`
  (params (DeltaSeconds :type "Float (single-precision)"))
  (`|ExecutionSequence`
    (:`then_0`
      ;[1 1 1] danger trigger
      (bind (_returnvalue _last_hit_actor) (`/Game/GeneralBlueprints/Main/FunctionLibrary/BFL_Camera.BFL_Simple_SphereTrace` self 500.0 10.0))
      (cast `/Game/GeneralBlueprints/Main/World/LevelActors/Temp_Tim/BP_enemy` _last_hit_actor
        (:`then`
          (set `self.is_looking_at_an_enemy` true))
        (:`CastFailed`
          (set `self.is_looking_at_an_enemy` false)))
      (if (or (`self.is_looking_at_an_enemy`) (`self.is_in_danger_zone`))
        (set `self.is_in_danger` true)
        (`KismetSystemLibrary.RetriggerableDelay` 3.0)
        (set `self.is_in_danger` false)))
    (:`then_1`
      (`|ExecutionSequence`))))

(event `InputAction|PauseGame`
  (params (Key :type "Key Structure"))
  ;[0 0.6682 1] Pause
  (:`Pressed`
    (bind _isa (`/Engine/EditorBlueprintResources/StandardMacros.FlipFlop`)
      (:`A`
        _)
      (:`B`
        _))
    (`GameplayStatics.SetGamePaused` _isa)))

(event `InputAction|MainAction`
  (params (Key :type "Key Structure"))
  (bind (_isactive _interactioncomponent) (`/Game/GeneralBlueprints/Main/FunctionLibrary/BFL_Interaction_Use.BFL_Get_Actor_InteractionComponent` (`self.K2_GetPawn`)))
  ;[0 0.6682 1] Line Trace
  (:`Pressed`
    (if _isactive
      (message `/Game/GeneralBlueprints/Main/Interfaces/Components/BPI_BaseInteraction.Main_Action` _interactioncomponent))))

(event `InputAction|Detective`
  (params (Key :type "Key Structure"))
  ;[1 1 1] Inspect evidence
  (:`Pressed`
    (bind (_returnvalue _last_hit_actor) (`/Game/GeneralBlueprints/Main/FunctionLibrary/BFL_Camera.BFL_Simple_SphereTrace` self 500.0 2.0 "ForOneFrame"))
    (if _returnvalue
      (bind _asbp_evidence_element (cast `/Game/GeneralBlueprints/Main/World/LevelActors/Temp_Tim/BP_evidence_element` _last_hit_actor))
      (`self.K2_DestroyActor` _asbp_evidence_element)
      (`KismetSystemLibrary.PrintString` "evidence added to inventory"))))

(event `InputAction|SideAction`
  (params (Key :type "Key Structure"))
  (bind (_isactive _interactioncomponent) (`/Game/GeneralBlueprints/Main/FunctionLibrary/BFL_Interaction_Use.BFL_Get_Actor_InteractionComponent` (`self.K2_GetPawn`)))
  ;[0 0.6682 1] Line Trace
  (:`Pressed`
    (if _isactive
      (message `/Game/GeneralBlueprints/Main/Interfaces/Components/BPI_BaseInteraction.Side_Action` _interactioncomponent))))

(fn `Drop Component`
  (`PhysicsHandleComponent.ReleaseComponent` (`/Game/GeneralBlueprints/Main/Characters/Player/BP_Char_Human.PhysicsHandle` (`/Game/GeneralBlueprints/Main/MacroLibrary/MCL_Actor_MacroLibrary.MCL_Get_DPlayerCharacter`)))
  (set `self.HoldComponent` false))

(fn `Get_InteractionComponent`
  (returns (IsActive :type Boolean) (InteractionComponent :type "/Game/GeneralBlueprints/Main/Components/BP_Base_InteractionComponent Object Reference"))
  (bind _ascharacter (cast `Character` (`self.K2_GetPawn`)))
  (bind (_isactive _interactioncomponent) (`/Game/GeneralBlueprints/Main/FunctionLibrary/BFL_Interaction_Use.BFL_Get_Character_InteractionComponent` _ascharacter))
  (return _isactive _interactioncomponent))

(fn `Grab Component`
  (params (Component :type "PrimitiveComponent Object Reference"))
  (`/Engine/EditorBlueprintResources/StandardMacros.IsValid` Component
    (:`Is Valid`
      (if (`SceneComponent.IsSimulatingPhysics` Component "None")
        (if (< (`PrimitiveComponent.GetMass` Component) 100.0)
          (if (not (`self.HoldComponent`))
            (set `self.HoldComponent` true)
            (`PhysicsHandleComponent.GrabComponentAtLocation` (`/Game/GeneralBlueprints/Main/Characters/Player/BP_Char_Human.PhysicsHandle` (`/Game/GeneralBlueprints/Main/MacroLibrary/MCL_Actor_MacroLibrary.MCL_Get_DPlayerCharacter`)) Component "None" (`SceneComponent.K2_GetComponentLocation` Component))))))))

(fn `Set_ClampedFOV`
  (params (Value :type "Float (double-precision)"))
  (set `PlayerCameraManager.DefaultFOV` (`KismetMathLibrary.FClamp` Value 5.0 170.0) (`self.PlayerCameraManager`)))

(fn `Set_DesiredControl_Rotation`
  (params (Rot :type "Rotator Structure") (InterpSpeed :type "Float (double-precision)"))
  (`self.SetControlRotation` (`KismetMathLibrary.RInterpTo` (`self.GetControlRotation`) Rot (`GameplayStatics.GetWorldDeltaSeconds`) InterpSpeed)))

(fn `UserConstructionScript`
  (bind _asbp_default_game_mode (cast `/Game/GeneralBlueprints/Main/GameMods/BP_DefaultGameMode` (`GameplayStatics.GetGameMode`)))
  (set `self.GameMode` _asbp_default_game_mode)
  (bind _asbp_game_inst_default (cast `/Game/GeneralBlueprints/Main/GameInstance/BP_GameInst_Default` (`GameplayStatics.GetGameInstance`)))
  (set `self.GameInstance` _asbp_game_inst_default))