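; Base interaction component that lets its owner focus, interact with and inspect what the camera is looking at.
; Each tick, an object-type sphere trace from the camera tracks the Item in sight, sending focus-in on a new Item and focus-out when the trace hits nothing.
; Main and side actions run a separate Visibility sphere trace and send interact or inspect messages to the hit actor.
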(event `self.ReceiveTick`
  (params (DeltaSeconds :type "Float (single-precision)"))
  (`self.Check Line Of Sight Intersection`))

(event `/Game/GeneralBlueprints/Main/Interfaces/Components/BPI_BaseInteraction.Main_Action`
  (bind (_returnvalue _last_hit_actor) (`self.Simple Sphere Trace` (`self.Trace Default Length`) (`self.Trace Default Radius`)))
  (if _returnvalue
    (message `/Game/GeneralBlueprints/Main/Interfaces/Items/BPI_Interactable.Interact` _last_hit_actor)))

(event `/Game/GeneralBlueprints/Main/Interfaces/Components/BPI_BaseInteraction.Side_Action`
  (bind (_returnvalue _last_hit_actor) (`self.Simple Sphere Trace` (`self.Trace Default Length`) (`self.Trace Default Radius`)))
  (if _returnvalue
    (message `/Game/GeneralBlueprints/Main/Interfaces/Items/BPI_Inspectable.Inspect` _last_hit_actor)))

(event `Item At Sight Gained`
  (message `/Game/GeneralBlueprints/Main/Interfaces/Items/BPI_InFocus.FocusedInto_BPIF` (`self.Last Item At Sight`) (`self.GetOwner`)))

(event `Item At Sight Lost`
  (message `/Game/GeneralBlueprints/Main/Interfaces/Items/BPI_InFocus.FucusedOut_BPIF` (`self.Last Item At Sight`) (`self.GetOwner`)))

(fn `Check Line Of Sight Intersection`
  (locals (`Hit Item` :type "/Game/GeneralBlueprints/Main/ItemSystem/Item Object Reference"))
  (bind (_location _rotation) (`/Game/GeneralBlueprints/Main/FunctionLibrary/BFL_StandartFunctions.BFL_Get_CurrentCamera_Location/Rotation`))
  (bind (_outhit _returnvalue) (`KismetSystemLibrary.SphereTraceSingleForObjects` _location (+ _location (* (`KismetMathLibrary.GetForwardVector` _rotation) (`self.Trace Default Length`))) (`self.Trace Default Radius`) (`|MakeArray` "ObjectTypeQuery7" :!type "EObjectTypeQuery Enum") true (`|MakeArray` (`self.GetOwner`))))
  (if _returnvalue
    (bind _asitem (cast `/Game/GeneralBlueprints/Main/ItemSystem/Item` (`.HitActor` (`GameplayStatics.BreakHitResult` _outhit))))
    (set `local.Hit Item` _asitem)
    (`self.Switch_IsSeeingItem`
      (:`T`
        (if (not (== (`local.Hit Item`) (`self.Last Item At Sight`)))
          (set `self.Sees Item` true :!label _label)
          (set `self.Last Item At Sight` (`local.Hit Item`))
          (`self.Item At Sight Gained`)))
      (:`F`
        (goto _label)))
    (else
      (`self.Switch_IsSeeingItem`
        (:`T`
          (set `self.Sees Item` false)
          (`self.Item At Sight Lost`))))))

(fn `Component_Initialization`
  (`parent.Component_Initialization`))

(fn `Simple Sphere Trace`
  (params (Length :type "Float (double-precision)") (Radius :type "Float (double-precision)") (DrawDebugType :type "EDrawDebugTrace Enum" :default "None"))
  (returns (ReturnValue :type Boolean) (Last_Hit_Actor :type "Actor Object Reference") (Last_Hit_ActorComp :type "PrimitiveComponent Object Reference"))
  (bind (_location _rotation) (`/Game/GeneralBlueprints/Main/FunctionLibrary/BFL_StandartFunctions.BFL_Get_CurrentCamera_Location/Rotation`))
  (if (and (> Length 0.0) (> Radius 0.0))
    (bind (_outhit _returnvalue) (`KismetSystemLibrary.SphereTraceSingle` _location (+ _location (* (`KismetMathLibrary.GetForwardVector` _rotation) (`local.Length`))) (`local.Radius`) "TraceTypeQuery1" true (`|MakeArray` (`self.GetOwner`)) (`local.DrawDebugType`)))
    (if _returnvalue
      (bind (_bblockinghit _binitialoverlap _time _distance _location_2 _impactpoint _normal _impactnormal _physmat _hitactor _hitcomponent) (`GameplayStatics.BreakHitResult` _outhit))
      (`/Engine/EditorBlueprintResources/StandardMacros.IsValid` _hitactor
        (:`Is Valid`
          (`/Engine/EditorBlueprintResources/StandardMacros.IsValid` _hitcomponent
            (:`Is Valid`
              (return true _hitactor _hitcomponent))
            (:`Is Not Valid`
              _)))
        (:`Is Not Valid`
          _)))
    (return false null null)))