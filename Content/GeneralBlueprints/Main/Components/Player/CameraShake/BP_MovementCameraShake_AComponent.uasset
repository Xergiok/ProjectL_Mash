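; Player component that drives movement camera shake and velocity-based camera tilt for BP_Char_Human.
; Over a persistent noise shake, character dispatchers swap idle noise and moving noise, forward-pitch and sideways-roll shakes chosen by stance and gait.
; Tick scales moving shakes by normalized speed, with roll also weighted by camera-to-velocity angle.
; It also interpolates a velocity camera modifier's additive rotation from character-to-velocity angle and speed, easing to zero when stopped.
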(event `self.ReceiveBeginPlay`
  (`self.Component_Initialization`)
  (bind _camera_manager (`self.Camera_Manager`)
    (:`then`
      (bind _returnvalue (`PlayerCameraManager.PlayCameraShake` :`self` _camera_manager :`ShakeClass` "/Game/GeneralBlueprints/Miscellaneous/CameraShake/Movement/Idle/BP_CamShake_PersistentNoise.BP_CamShake_PersistentNoise_C"))
      (set `self.CS_PersistentNoise` _returnvalue)
      (`self.IdleSwitch_CS`))
    (:`else`)))

(event `self.ReceiveTick`
  (params (DeltaSeconds :type "Float (single-precision)"))
  (`self.Update_VelocityModifier`)
  (`self.Update_CameraShakes`))

(event `Update_Set_Gait`
  (bind _playerh_character (`self.PlayerH_Character`)
    (:`then`
      (bind _out_a (`/Game/GeneralBlueprints/Main/MacroLibrary/BPML_Object.MCL_DoOnly_IfDifferent(Byte)` (`/Game/GeneralBlueprints/Main/Characters/Player/BP_Char_Human.Current_GaitType` _playerh_character) (`self.Player_Gait`))
        (:`true`
          (set `self.Player_Gait` _out_a)
          (`self.Switch_IsMoving`
            (:`T`
              (`self.IdleSwitch_CS`))))))
    (:`else`)))

(event `Update_Set_ControlType`
  (bind _playerh_character (`self.PlayerH_Character`)
    (:`then`
      (bind _out_a (`/Game/GeneralBlueprints/Main/MacroLibrary/BPML_Object.MCL_DoOnly_IfDifferent(Byte)` (`/Game/GeneralBlueprints/Main/Characters/Player/BP_Char_Human.Current_PawnControlType` _playerh_character) (`self.Player_ControlType`))
        (:`true`
          (set `self.Player_ControlType` _out_a)
          (`self.Switch_IsMoving`
            (:`T`
              (`self.IdleSwitch_CS`))))))
    (:`else`)))

(event `Update_Set_Stance`
  (bind _playerh_character (`self.PlayerH_Character`)
    (:`then`
      (bind _out_a (`/Game/GeneralBlueprints/Main/MacroLibrary/BPML_Object.MCL_DoOnly_IfDifferent(Byte)` (`/Game/GeneralBlueprints/Main/Characters/Player/BP_Char_Human.Current_Stance` _playerh_character) (`self.Player_Stance`))
        (:`true`
          (set `self.Player_Stance` _out_a)
          (`self.Switch_IsMoving`
            (:`T`
              (`self.IdleSwitch_CS`))))))
    (:`else`)))

(event `Update_Set)IsMoving`
  (bind _playerh_character (`self.PlayerH_Character`)
    (:`then`
      (bind _out_a (`/Game/GeneralBlueprints/Main/MacroLibrary/BPML_Object.MCL_DoOnly_IfDifferent(Bool)` (`/Game/GeneralBlueprints/Main/Characters/Player/BP_Char_Human.IsMoving` _playerh_character) (`self.IsMoving`))
        (:`true`
          (set `self.IsMoving` _out_a)
          (`self.IdleSwitch_CS`))))
    (:`else`)))

(fn `Calculate_SpeedIntensity_Scale`
  (params (FB_Input :type "Float (double-precision)") (RL_Input :type "Float (double-precision)"))
  (returns (ReturnValue :type "Float (double-precision)"))
  (bind (_default_maxspeed_value _coefmax_crouch_speed _coefmax_sprint_speed _coefmax_slowwalk_speed) (break `/Game/GeneralBlueprints/Miscellaneous/CharacterDefaults/Movement/ST_SpeedCoefs` (`self.Speed_Coef`)))
  (bind ((`CharacterMoveInput_RL_Scale_8_D12A3ED2458183AC5B155782F3C9088B` _charactermoveinput_rl_scale) (`CharacterMoveInput_Backward_Scale_10_2AA8B1A044701216F644BB962219ADEB` _charactermoveinput_backward_scale)) (break `/Game/GeneralBlueprints/Miscellaneous/CharacterDefaults/Movement/ST_CharacterInputParams` (`self.Input_Coef`)))
  (return (`KismetMathLibrary.NormalizeToRange` (`KismetMathLibrary.VSize` (`Actor.GetVelocity` (`self.PlayerH_Character`))) 0.0 (* (`KismetMathLibrary.SelectFloat` _charactermoveinput_backward_scale (`KismetMathLibrary.SelectFloat` _charactermoveinput_rl_scale 1.0 (and (!= (`local.RL_Input`) 0.0) (== (`local.FB_Input`) 0.0))) (< (`local.FB_Input`) 0.0)) (select `/Game/GeneralBlueprints/Miscellaneous/MovementEnums/E_Stance` (`self.Player_Stance`) :`NewEnumerator0` (select `/Game/GeneralBlueprints/Miscellaneous/MovementEnums/E_GaitTypes` (`self.Player_Gait`) :`NewEnumerator1` _default_maxspeed_value :`NewEnumerator0` (* _default_maxspeed_value _coefmax_slowwalk_speed) :`NewEnumerator2` (* _default_maxspeed_value _coefmax_sprint_speed)) :`NewEnumerator1` (* _default_maxspeed_value _coefmax_crouch_speed))))))

(fn `Component_Initialization`
  (`parent.Component_Initialization`)
  (bind _asbp_char_human (cast `/Game/GeneralBlueprints/Main/Characters/Player/BP_Char_Human` (`self.GetOwner`)))
  (bind _output_get (set `self.PlayerH_Character` _asbp_char_human))
  (bind (_movement_defaults_inputparams _movement_defaults_speedparams) (break `/Game/GeneralBlueprints/Miscellaneous/CharacterDefaults/Movement/ST_CharacterMovementParams` (`/Game/GeneralBlueprints/Main/Characters/Player/BP_Char_Human.Movement_Defaults` _output_get)))
  (set `self.Input_Coef` _movement_defaults_inputparams)
  (set `self.Speed_Coef` _movement_defaults_speedparams)
  (bind _playerh_character (`self.PlayerH_Character`)
    (:`then`
      (bind _asbp_default_player_controller (cast `/Game/GeneralBlueprints/Main/Control/PlayerControllers/BP_DefaultPlayerController` (`Pawn.GetController` _playerh_character)))
      (bind _asbp_default_player_cam_manager (cast `/Game/GeneralBlueprints/Main/Control/PlayerCameraManagers/BP_Default_PlayerCamManager` (`PlayerController.PlayerCameraManager` _asbp_default_player_controller)))
      (set `self.Camera_Manager` _asbp_default_player_cam_manager)
      (bind _returnvalue (`PlayerCameraManager.AddNewCameraModifier` (`self.Camera_Manager`) "/Game/GeneralBlueprints/Miscellaneous/CameraModifiers/Movement/BP_Velolcity_CamMod.BP_Velolcity_CamMod_C"))
      (bind _asbp_velolcity_cam_mod (cast `/Game/GeneralBlueprints/Miscellaneous/CameraModifiers/Movement/BP_Velolcity_CamMod` _returnvalue))
      (set `self.Velocity_CamMod` _asbp_velolcity_cam_mod)
      (`|ExecutionSequence`
        (:`then_0`
          (bind _playerh_character_2 (`self.PlayerH_Character`)
            (:`then`
              (add `/Game/GeneralBlueprints/Main/Characters/Player/BP_Char_Human.EventDisp_IsMoving_Changed` _playerh_character_2 (`|CreateDelegate` :!event `Update_Set)IsMoving`))
              (bind _playerh_character_3 (`self.PlayerH_Character`)
                (:`then`
                  (add `/Game/GeneralBlueprints/Main/Characters/Player/BP_Char_Human.EventDisp_PawnControl_Changed` _playerh_character_3 (`|CreateDelegate` :!event `Update_Set_ControlType`))
                  (bind _playerh_character_4 (`self.PlayerH_Character`)
                    (:`then`
                      (add `/Game/GeneralBlueprints/Main/Characters/Player/BP_Char_Human.EventDisp_GateType_Changed` _playerh_character_4 (`|CreateDelegate` :!event `Update_Set_Gait`))
                      (bind _playerh_character_5 (`self.PlayerH_Character`)
                        (:`then`
                          (add `/Game/GeneralBlueprints/Main/Characters/Player/BP_Char_Human.EventDisp_Stance_Changed` _playerh_character_5 (`|CreateDelegate` :!event `Update_Set_Stance`)))
                        (:`else`)))
                    (:`else`)))
                (:`else`)))
            (:`else`)))))
    (:`else`)))

(fn `IdleSwitch_CS`
  (`/Engine/EditorBlueprintResources/StandardMacros.IsValid` (`self.Camera_Manager`)
    (:`Is Valid`
      (`self.Switch_ShakeType`
        (:`Idle`
          (`self.Stop_Idle_CS` false))
        (:`Moving`
          (`self.Stop_Ambient_CS` false)))
      (`self.Switch_IsMoving`
        (:`T`
          (`self.PlayAmbien_CS`))
        (:`F`
          (`self.Play_Idle_CS`))))))

(fn `PawnControlSwitch_CS`
  (bind _playerh_character (`self.PlayerH_Character`)
    (:`then`
      (switch `/Game/GeneralBlueprints/Miscellaneous/MovementEnums/E_PawnControlTypes` (`/Game/GeneralBlueprints/Main/Characters/Player/BP_Char_Human.Current_PawnControlType` _playerh_character)))
    (:`else`)))

(fn `Play_Idle_CS`
  (`/Engine/EditorBlueprintResources/StandardMacros.IsValid` (`self.Camera_Manager`)
    (:`Is Valid`
      (set `self.ShakeType` "NewEnumerator0")
      (bind _returnvalue (`PlayerCameraManager.PlayCameraShake` :`self` (`self.Camera_Manager`) :`ShakeClass` (select `/Game/GeneralBlueprints/Miscellaneous/MovementEnums/E_Stance` (`self.Player_Stance`) :`NewEnumerator0` "/Game/GeneralBlueprints/Miscellaneous/CameraShake/Movement/Idle/Idle/BP_CamShake_IdleNoise_Stand.BP_CamShake_IdleNoise_Stand_C" :`NewEnumerator1` "/Game/GeneralBlueprints/Miscellaneous/CameraShake/Movement/Idle/Idle/BP_CamShake_IdleNoise_Crouch.BP_CamShake_IdleNoise_Crouch_C" :!type "CameraShake Class Reference") :`Scale` 2.0))
      (set `self.Idle_CS` _returnvalue))))

(fn `PlayAmbien_CS`
  (locals (Gait :type "/Game/GeneralBlueprints/Miscellaneous/MovementEnums/E_GaitTypes Enum" :default "NewEnumerator1"))
  (`/Engine/EditorBlueprintResources/StandardMacros.IsValid` (`self.Camera_Manager`)
    (:`Is Valid`
      (set `self.ShakeType` "NewEnumerator1")
      (bind _returnvalue (`PlayerCameraManager.PlayCameraShake` :`self` (`self.Camera_Manager`) :`ShakeClass` (select `/Game/GeneralBlueprints/Miscellaneous/MovementEnums/E_Stance` (`self.Player_Stance`) :`NewEnumerator0` (select `/Game/GeneralBlueprints/Miscellaneous/MovementEnums/E_GaitTypes` (`self.Player_Gait`) :`NewEnumerator1` "/Game/GeneralBlueprints/Miscellaneous/CameraShake/Movement/Moving/Running/BP_CamShake_Noise_Running.BP_CamShake_Noise_Running_C" :`NewEnumerator0` "/Game/GeneralBlueprints/Miscellaneous/CameraShake/Movement/Moving/Walking/BP_CamShake_Noise_Walking.BP_CamShake_Noise_Walking_C" :`NewEnumerator2` "/Game/GeneralBlueprints/Miscellaneous/CameraShake/Movement/Moving/Sprinting/BP_CamShake_Noise_Sprinting.BP_CamShake_Noise_Sprinting_C" :!type "CameraShake Class Reference") :`NewEnumerator1` "/Game/GeneralBlueprints/Miscellaneous/CameraShake/Movement/Moving/Crouching/BP_CamShake_Noise_Crouching.BP_CamShake_Noise_Crouching_C")))
      (set `self.AmbienNoise_CS` _returnvalue)
      (bind _returnvalue_2 (`PlayerCameraManager.PlayCameraShake` :`self` (`self.Camera_Manager`) :`ShakeClass` (select `/Game/GeneralBlueprints/Miscellaneous/MovementEnums/E_Stance` (`self.Player_Stance`) :`NewEnumerator0` (select `/Game/GeneralBlueprints/Miscellaneous/MovementEnums/E_GaitTypes` (`self.Player_Gait`) :`NewEnumerator1` "/Game/GeneralBlueprints/Miscellaneous/CameraShake/Movement/Moving/Running/BP_CamShake_ForwardPitch_Running.BP_CamShake_ForwardPitch_Running_C" :`NewEnumerator0` "/Game/GeneralBlueprints/Miscellaneous/CameraShake/Movement/Moving/Walking/BP_CamShake_ForwardPitch_Walking.BP_CamShake_ForwardPitch_Walking_C" :`NewEnumerator2` "/Game/GeneralBlueprints/Miscellaneous/CameraShake/Movement/Moving/Sprinting/BP_CamShake_ForwardPitch_Sprinting.BP_CamShake_ForwardPitch_Sprinting_C" :!type "CameraShake Class Reference") :`NewEnumerator1` "/Game/GeneralBlueprints/Miscellaneous/CameraShake/Movement/Moving/Crouching/BP_CameraShake_ForwardPitch_Crouching.BP_CameraShake_ForwardPitch_Crouching_C")))
      (set `self.AmbientForward_CS` _returnvalue_2)
      (bind _returnvalue_3 (`PlayerCameraManager.PlayCameraShake` :`self` (`self.Camera_Manager`) :`ShakeClass` (select `/Game/GeneralBlueprints/Miscellaneous/MovementEnums/E_Stance` (`self.Player_Stance`) :`NewEnumerator0` (select `/Game/GeneralBlueprints/Miscellaneous/MovementEnums/E_GaitTypes` (`self.Player_Gait`) :`NewEnumerator1` "/Game/GeneralBlueprints/Miscellaneous/CameraShake/Movement/Moving/Running/BP_CamShake_SidewaysRoll_Running.BP_CamShake_SidewaysRoll_Running_C" :`NewEnumerator0` "/Game/GeneralBlueprints/Miscellaneous/CameraShake/Movement/Moving/Walking/BP_CamShake_SidewaysRoll_Walking.BP_CamShake_SidewaysRoll_Walking_C" :`NewEnumerator2` "/Game/GeneralBlueprints/Miscellaneous/CameraShake/Movement/Moving/Sprinting/BP_CamShake_SidewaysRoll_Sprinting.BP_CamShake_SidewaysRoll_Sprinting_C" :!type "CameraShake Class Reference") :`NewEnumerator1` "/Game/GeneralBlueprints/Miscellaneous/CameraShake/Movement/Moving/Crouching/BP_CamShake_SidewaysRoll_Crouching.BP_CamShake_SidewaysRoll_Crouching_C") :`Scale` 0.001))
      (set `self.AmbientSide_CS` _returnvalue_3))))

(fn `Stop_Ambient_CS`
  (params (Immediately :type Boolean))
  (bind _camera_manager (`self.Camera_Manager`))
  (`PlayerCameraManager.StopAllInstancesOfCameraShake` _camera_manager "/Game/GeneralBlueprints/Miscellaneous/CameraShake/Movement/Moving/BP_CameraShake_AmbientNoise_Parent.BP_CameraShake_AmbientNoise_Parent_C" Immediately)
  (`PlayerCameraManager.StopAllInstancesOfCameraShake` _camera_manager "/Game/GeneralBlueprints/Miscellaneous/CameraShake/Movement/Moving/BP_CameraShake_AmbientForwardPitch_Parent.BP_CameraShake_AmbientForwardPitch_Parent_C" Immediately)
  (`PlayerCameraManager.StopAllInstancesOfCameraShake` _camera_manager "/Game/GeneralBlueprints/Miscellaneous/CameraShake/Movement/Moving/BP_CameraShake_AmbientSidewaysRoll_Parent.BP_CameraShake_AmbientSidewaysRoll_Parent_C" Immediately))

(fn `Stop_Idle_CS`
  (params (bImmediately :type Boolean))
  (`PlayerCameraManager.StopAllInstancesOfCameraShake` (`self.Camera_Manager`) "/Game/GeneralBlueprints/Miscellaneous/CameraShake/Movement/Idle/Idle/BP_CamShake_IdleNoiseParent.BP_CamShake_IdleNoiseParent_C" bImmediately))

(fn `Update_CameraShakes`
  (locals (Input_FB_Value :type "Float (double-precision)") (Input_RL_Value :type "Float (double-precision)"))
  (`/Engine/EditorBlueprintResources/StandardMacros.IsValid` (`self.Camera_Manager`)
    (:`Is Valid`
      (`self.Switch_IsMoving`
        (:`T`
          (bind _playerh_character (`self.PlayerH_Character`)
            (:`then`
              (bind _returnvalue (`self.Calculate_SpeedIntensity_Scale` (`/Game/GeneralBlueprints/Main/Characters/Player/BP_Char_Human.MoveFB` _playerh_character) (`/Game/GeneralBlueprints/Main/Characters/Player/BP_Char_Human.MoveRL` _playerh_character)))
              (`|ExecutionSequence`
                (:`then_0`
                  (bind _ambiennoise_cs (`self.AmbienNoise_CS`)
                    (:`then`
                      (set `CameraShake.ShakeScale` _returnvalue _ambiennoise_cs))
                    (:`else`)))
                (:`then_1`
                  (bind _ambientforward_cs (`self.AmbientForward_CS`)
                    (:`then`
                      (set `CameraShake.ShakeScale` _returnvalue _ambientforward_cs))
                    (:`else`)))
                (:`then_2`
                  (bind _ambientside_cs (`self.AmbientSide_CS`)
                    (:`then`
                      (set `CameraShake.ShakeScale` (* _returnvalue (`self.AmbientRoll_Scale`)) _ambientside_cs))
                    (:`else`)))))
            (:`else`)))))))

(fn `Update_VelocityModifier`
  (locals (Offset :type "Float (double-precision)"))
  (bind _offset (`local.Offset`))
  (if (and (`KismetSystemLibrary.IsValid` (`self.Velocity_CamMod`)) (`KismetSystemLibrary.IsValid` (`self.PlayerH_Character`)))
    (`self.Switch_IsMoving`
      (:`T`
        (set `local.Offset` (`self.CharacterRotation/VelocityDifference`))
        (set `/Game/GeneralBlueprints/Miscellaneous/CameraModifiers/Movement/BP_Velolcity_CamMod.AdditiveRotation` (`KismetMathLibrary.ClampAxes2D` (`KismetMathLibrary.Vector2DInterpTo` (`/Game/GeneralBlueprints/Miscellaneous/CameraModifiers/Movement/BP_Velolcity_CamMod.AdditiveRotation` (`self.Velocity_CamMod`)) (`KismetMathLibrary.MakeVector2D` (`self.Apply_SpeedCoef` (`self.Calculate_RollIntensity` _offset)) (`self.Apply_SpeedCoef` (`self.Calculate_PitchIntensity` _offset))) (`GameplayStatics.GetWorldDeltaSeconds`) 3.0) 0.0 20.0) (`self.Velocity_CamMod`)))
      (:`F`
        (if (not (`KismetMathLibrary.IsNearlyZero2D` (`/Game/GeneralBlueprints/Miscellaneous/CameraModifiers/Movement/BP_Velolcity_CamMod.AdditiveRotation` (`self.Velocity_CamMod`)) 0.001))
          (set `/Game/GeneralBlueprints/Miscellaneous/CameraModifiers/Movement/BP_Velolcity_CamMod.AdditiveRotation` (`KismetMathLibrary.Vector2DInterpTo` (`/Game/GeneralBlueprints/Miscellaneous/CameraModifiers/Movement/BP_Velolcity_CamMod.AdditiveRotation` (`self.Velocity_CamMod`)) (`KismetMathLibrary.MakeVector2D` 0.0) (`GameplayStatics.GetWorldDeltaSeconds`) 3.0) (`self.Velocity_CamMod`)))))))