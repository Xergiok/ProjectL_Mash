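; Floating interaction info icon that shows a textured or flipbook material on a plane, turned toward the player's view and scaled by distance.
; A Mode setting either nudges it inside screen margins, anchors it to its sphere Volume, or wanders it within that volume by random lerp or regenerated spline.
; An opacity timeline fades it in, while delayed, gate-cancellable deactivation fades it out and destroys it, removing it from the interaction component's InfoIcons.
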(event `self.ReceiveBeginPlay`
  ;[1 1 1] Create and set up material instance
  (bind _returnvalue (`KismetMaterialLibrary.CreateDynamicMaterialInstance` "/Game/Materials-Visual/ItemIcons/Materials/Mat_InfoIcon_Surf.Mat_InfoIcon_Surf"))
  (bind _output_get (set `self.MatInst_InfoIcon` _returnvalue))
  (`MaterialInstanceDynamic.SetTextureParameterValue` _output_get "Icon_Image" (`self.Icon_Texture`))
  (`PrimitiveComponent.SetMaterial` (`self.Plane`) 0 (`self.MatInst_InfoIcon`))
  ;[1 1 1] Starter opacity anim
  (`self.Set_Icon_Opacity` 0.0)
  (`KismetSystemLibrary.Delay` 0.5)
  (`TimelineComponent.PlayFromStart` (`self.Opacity_Timeline`))
  (`|ExecutionSequence`
    (:`then_0`
      (`/Engine/EditorBlueprintResources/StandardMacros.IsValid` (`self.Volume`)
        (:`Is Valid`
          (set `self.Scaled_Radius` (`SphereComponent.GetScaledSphereRadius` (`self.Volume`)))
          (switch `/Game/GeneralBlueprints/Main/Components/Player/Interaction/E_InfoIcon_Mode` (`self.Mode`)
            (:`NewEnumerator2`
              (set `self.Target_Location` (`self.RandomLocation_InPlane`))
              (`TimelineComponent.PlayFromStart` (`self.RandomLocation_InVolume_Timeline`)))
            (:`NewEnumerator3`
              (`/Engine/EditorBlueprintResources/StandardMacros.IsValid` (`self.SplineComponent`)
                (:`Is Not Valid`
                  (bind _returnvalue_2 (`AddComponent|NODE_AddSplineComponent-0`))
                  (bind _output_get_2 (set `self.SplineComponent` _returnvalue_2))
                  (`SplineComponent.SetDrawDebug` _output_get_2 true)
                  (`self.Setup_Spline`))))))))
    (:`then_1`
      ;[1 0 0.212] Comment
      (`/Game/GeneralBlueprints/Main/FunctionLibrary/BFL_ControlInput.BFL_Set_ActorActionInput` self true))))

(event `Key|One`
  (params (Key :type "Key Structure"))
  ;[1 0 0.212] Comment
  (:`Pressed`
    (bind _isa (`/Engine/EditorBlueprintResources/StandardMacros.FlipFlop`)
      (:`A`
        _)
      (:`B`
        _))
    (`self.Change_FlipBook_Animation` _isa)))

(event `self.ReceiveTick`
  (params (DeltaSeconds :type "Float (single-precision)"))
  (bind (_actorposition _controllerposition) (`self.Get_ControllerPosition`))
  (bind (_actorposition_2 _controllerposition_2) (`self.Get_ControllerPosition`))
  (bind _returnvalue (`KismetSystemLibrary.MakeLiteralDouble` (/ (`KismetMathLibrary.Vector_Distance` _actorposition _controllerposition) 500.0)))
  ;[1 1 1] Face to controller
  (bind _volume (`self.Volume`)
    (:`then`
      (`SceneComponent.K2_SetWorldRotation` (`self.RootComponent`) (`KismetMathLibrary.FindLookAtRotation` _actorposition_2 _controllerposition_2) false false)
      (`SceneComponent.K2_SetWorldRotation` _volume (`KismetMathLibrary.FindLookAtRotation` _actorposition_2 _controllerposition_2) false false)
      ;[1 1 1] Scaling from distance
      (`SceneComponent.SetRelativeScale3D` (`self.RootComponent`) (`KismetMathLibrary.MakeVector` _returnvalue _returnvalue _returnvalue))
      (`self.Update_Position`))
    (:`else`)))

(event `Change_FlipBook_Animation`
  (params (Enable :type Boolean))
  ;[1 0 0.212] Comment
  (if Enable
    (bind _returnvalue (`KismetMaterialLibrary.CreateDynamicMaterialInstance` "/Game/Materials-Visual/ItemIcons/Materials/Mat_InfoIcon_Surf_Flipbook.Mat_InfoIcon_Surf_Flipbook"))
    (bind _output_get (set `self.Flipbook_anim` _returnvalue))
    (`MaterialInstanceDynamic.SetTextureParameterValue` _output_get "FlipBook_Texture" "/Game/Materials-Visual/ItemIcons/Lamp_Flipbook.Lamp_Flipbook")
    (`PrimitiveComponent.SetMaterial` (`self.Plane`) 0 (`self.Flipbook_anim`))
    (else
      (`PrimitiveComponent.SetMaterial` (`self.Plane`) 0 (`self.MatInst_InfoIcon`)))))

(event `Play_Opacity_Animation`
  (params (InPlayRate :type "Float (double-precision)") (Reverse :type Boolean))
  ;[1 1 1] Event for Opacity anim
  (`TimelineComponent.SetPlayRate` (`self.Opacity_Timeline`) InPlayRate)
  (if Reverse
    (bind (_direction _opacity_value) (`Timeline|Opacity_Timeline` :!via `Reverse` :!label _label)
      (:`Update`
        (`self.Set_Icon_Opacity` _opacity_value))
      (:`Finished`
        (switch `ETimelineDirection` _direction
          (:`Backward`
            (`self.K2_DestroyActor`)))))
    (else
      (goto _label))))

(event `Activation`
  ;[1 1 1] Enable and disable from other bp
  (`|ExecutionSequence`
    (:`then_0`
      (goto _label_2 :!via `Close`))
    (:`then_1`
      (`self.Play_Opacity_Animation` 2.0))))

(event `Deactivation`
  ;[1 1 1] Enable and disable from other bp
  (`|ExecutionSequence`
    (:`then_0`
      (goto _label_2 :!via `Open`))
    (:`then_1`
      (`KismetSystemLibrary.Delay` 0.5)
      (`/Engine/EditorBlueprintResources/StandardMacros.Gate` true :!label _label_2
        (:`Exit`
          (`self.Play_Opacity_Animation` 2.0 true))))))

(event `self.ReceiveDestroyed`
  (bind _playercontroller (`self.PlayerController`))
  (bind (_isactive _interactioncomponent) (`/Game/GeneralBlueprints/Main/FunctionLibrary/BFL_Interaction_Use.BFL_Get_Actor_InteractionComponent` (`Controller.K2_GetPawn` _playercontroller)))
  ;[1 1 1] Clear ref in interaction bp
  (`/Engine/EditorBlueprintResources/StandardMacros.IsValid` _playercontroller
    (:`Is Valid`
      (if _isactive
        (`BlueprintMapLibrary.Map_Remove` (`/Game/GeneralBlueprints/Main/Components/BP_BaseInteraction_AComponent.InfoIcons` _interactioncomponent) (`self.GetOwner`))))))

(fn `Position_Fit`
  (params (Scale :type "Float (double-precision)") (Speed :type "Float (double-precision)"))
  (bind _returnvalue (`WidgetLayoutLibrary.GetViewportSize`))
  (bind _speed (`local.Speed`))
  (bind _speed_2 (`local.Speed`))
  (bind (_screenposition _returnvalue_2) (`GameplayStatics.ProjectWorldToScreen` (`self.PlayerController`) (`self.K2_GetActorLocation`)))
  (bind (_x _y) (`KismetMathLibrary.BreakVector2D` _returnvalue))
  (bind (_x_2 _y_2) (`KismetMathLibrary.BreakVector2D` (/ _returnvalue (`local.Scale`))))
  (bind (_x_3 _y_3) (`KismetMathLibrary.BreakVector2D` _screenposition))
  (bind _returnvalue_3 (> _y_3 (- _y _y_2)))
  (bind _returnvalue_4 (> _x_3 (- _x _x_2)))
  (if _returnvalue_2
    (if (or _returnvalue_4 (< _x_3 _x_2))
      (`self.K2_SetActorLocation` (+ (`self.K2_GetActorLocation`) (* (`KismetMathLibrary.GetRightVector` (`self.K2_GetActorRotation`)) (`KismetMathLibrary.SelectFloat` _speed_2 (* -1 _speed_2) _returnvalue_4))))
      (elif (or _returnvalue_3 (< _y_3 _y_2))
        (`self.K2_SetActorLocation` (+ (* (`KismetMathLibrary.GetUpVector` (`self.K2_GetActorRotation`)) (`KismetMathLibrary.SelectFloat` _speed (* -1 _speed) _returnvalue_3)) (`self.K2_GetActorLocation`)))))))

(fn `RandomLocation_InPlane`
  (returns (ReturnValue :type "Vector Structure"))
  (bind _returnvalue_roll (`KismetMathLibrary.BreakRotator` (`KismetMathLibrary.RandomRotator` true)))
  (bind _volume (`self.Volume`)
    (:`then`
      (bind (_returnvalue_roll_2 _returnvalue_pitch _returnvalue_yaw) (`KismetMathLibrary.BreakRotator` (`SceneComponent.K2_GetComponentRotation` _volume)))
      (return (+ (* (`KismetMathLibrary.GetRightVector` (`KismetMathLibrary.MakeRotator` _returnvalue_roll _returnvalue_pitch _returnvalue_yaw)) (`KismetMathLibrary.RandomFloatInRange` 0.01 (`self.Scaled_Radius`))) (`SceneComponent.K2_GetComponentLocation` _volume))))
    (:`else`)))

(fn `RandomLocation_InVolume`
  (returns (ReturnValue :type "Vector Structure"))
  (bind _volume (`self.Volume`)
    (:`then`
      (return (+ (* (`KismetMathLibrary.GetForwardVector` (`KismetMathLibrary.RandomRotator` false)) (`KismetMathLibrary.RandomFloatInRange` 0.01 (`self.Scaled_Radius`))) (`SceneComponent.K2_GetComponentLocation` _volume))))
    (:`else`)))

(fn `Set_Icon_Opacity`
  (params (Value :type "Float (double-precision)"))
  (`MaterialInstanceDynamic.SetScalarParameterValue` (`self.MatInst_InfoIcon`) "Opacity" Value))

(fn `Setup_Spline`
  (set `self.Target_Location` (`SceneComponent.K2_GetComponentLocation` (`self.Volume`)))
  (`self.Update_SplinePoints`)
  (`TimelineComponent.PlayFromStart` (`self.Spline_Timeline`)))

(fn `Update_Position`
  (switch `/Game/GeneralBlueprints/Main/Components/Player/Interaction/E_InfoIcon_Mode` (`self.Mode`)
    (:`NewEnumerator0`
      (`self.Position_Fit` 4.0 2.0))
    (:`NewEnumerator1`
      (bind _volume (`self.Volume`)
        (:`then`
          (`SceneComponent.K2_SetWorldLocation` (`self.RootComponent`) (`SceneComponent.K2_GetComponentLocation` _volume) false false))
        (:`else`)))))

(fn `Update_SplinePoints`
  (locals (Point :type Integer) (Size :type Integer :default 9) (`Period 100` :type "Float (double-precision)" :default 10.0))
  (bind _returnvalue (`SplineComponent.GetLocationAtSplinePoint` (`self.SplineComponent`) (`local.Point`) "Local"))
  (`SplineComponent.ClearSplinePoints` (`self.SplineComponent`) true)
  (for _index (range (+ (`local.Size`) 1))
    (set `local.Point` _index)
    (`SplineComponent.AddPoint` (`self.SplineComponent`) (make `SplinePoint` (`KismetMathLibrary.Conv_IntToDouble` (`local.Point`)) (`KismetMathLibrary.SelectVector` (`self.Target_Location`) (`self.RandomLocation_InVolume`) (== (`local.Point`) 0)) (`self.RandomLocation_InVolume`) (`self.RandomLocation_InVolume`)) true)
    ;[1 0 0.5857] debug
    (`KismetSystemLibrary.SphereTraceSingle` :`Start` _returnvalue :`End` _returnvalue :`Radius` 0.5 :`TraceChannel` "TraceTypeQuery1" :`bTraceComplex` true :`DrawDebugType` "ForDuration"))
  (set `self.Target_Location` (`SplineComponent.GetLocationAtSplinePoint` (`self.SplineComponent`) (+ (`local.Size`) 1) "Local"))
  (`TimelineComponent.SetPlayRate` (`self.Spline_Timeline`) (* (/ (`self.SplineSpeed`) (/ (`SplineComponent.GetSplineLength` (`self.SplineComponent`)) 40.0)) (/ (`self.Scaled_Radius`) 15.0))))

(fn `UserConstructionScript`
  (bind _returnvalue (`self.GetInstigator`))
  (`/Engine/EditorBlueprintResources/StandardMacros.IsValid` _returnvalue
    (:`Is Valid`
      (bind _asplayer_controller (cast `PlayerController` (`Pawn.GetController` _returnvalue)))
      (set `self.PlayerController` _asplayer_controller))))