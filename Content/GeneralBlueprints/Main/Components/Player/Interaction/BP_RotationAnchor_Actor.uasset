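; Temporary anchor actor for item examination, letting the player rotate an item with the mouse.
; Timelines move the item onto RotationRoot and back to its original transform, toggling player input and queuing briefly interrupted requests.
; Left-mouse drag rotates by simple or interpolated mode (NumPad 2), with speed scaled by cursor distance from screen center and pitch direction set by a trace.
; After return it self-destructs, re-enabling the instigator's interaction component.
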(event `self.ReceiveTick`
  (params (DeltaSeconds :type "Float (single-precision)"))
  ;[1 1 1] Checking if we can rotate actor
  (if (and (`KismetSystemLibrary.IsValid` (`self.Examine_Item`)) (not (`self.IsPlayingAnimation`)) (not (`self.Premature_ending`)))
    (`/Engine/EditorBlueprintResources/StandardMacros.Gate` true :!label _label
      (:`Exit`
        (`self.Add_Rotation` (`self.Select_Scale`) (stale `Key|LeftMouseButton` _reverse))))
    (else
      (`KismetSystemLibrary.PrintString` "Dont allowed" true true (struct :`G` 0.66 :`B` 1.0 :`A` 1.0) 0.0))))

(event `Key|LeftMouseButton`
  (params (Key :type "Key Structure"))
  (:`Pressed`
    (`KismetSystemLibrary.PrintString` "Inupt passed")
    (`self.Is_ClickedOnItem`)
    (bind _reverse (`self.ReverseRotation`))
    (goto _label :!via `Open`))
  (:`Released`
    (goto _label :!via `Close`)))

(event `Begin_Examine`
  (bind (_start_transform _end_transform) (`self.Select_ExamineTransform` true))
  (`|ExecutionSequence`
    (:`then_0`
      (goto _label :!via `Close`))
    (:`then_1`
      (if (`self.IsPlayingAnimation`)
        (`self.Re-call`)
        (else
          (set `self.Animation_Direction` "NewEnumerator1")
          (set `self.Premature_ending` false)
          (set `self.Origin_Transform` (`self.GetTransform` (`self.Examine_Item`)))
          (`/Game/GeneralBlueprints/Main/FunctionLibrary/BFL_ControlInput.BFL_Set_ControllerLookInput` false)
          (`/Game/GeneralBlueprints/Main/FunctionLibrary/BFL_ControlInput.BFL_Set_PlayerCharacterActionInput` false)
          (`/Game/GeneralBlueprints/Main/ItemSystem/BP_MasterItem.Set_CollisionProfile` (`self.Examine_Item`) true)
          (bind (_direction _lerpvalue) (`Timeline|Examine_Begin_Timeline` :!via `PlayFromStart`)
            (:`Update`
              (bind (_returnvalue_location _returnvalue_rotation) (`KismetMathLibrary.BreakTransform` (`KismetMathLibrary.TLerp` _start_transform _end_transform _lerpvalue)))
              (`self.K2_SetActorLocationAndRotation` (`self.Examine_Item`) _returnvalue_location _returnvalue_rotation false false))
            (:`Finished`
              (`SceneComponent.K2_AttachToComponent` (`Actor.RootComponent` (`self.Examine_Item`)) (`self.Rotation_Root`) "None" "SnapToTarget" "KeepWorld" "KeepWorld" true)
              (set `PlayerController.bShowMouseCursor` true (`self.PlayerController`))
              (set `self.Animation_Direction` "NewEnumerator0")
              (`self.EnableInput` (`self.PlayerController`))
              (if (`self.Premature_ending`)
                (`self.Finish_Examine`)))))))))

(event `Finish_Examine`
  (bind (_start_transform _end_transform) (`self.Select_ExamineTransform` false))
  (bind _examine_item (`self.Examine_Item`))
  (`|ExecutionSequence`
    (:`then_0`
      (goto _label :!via `Close`))
    (:`then_1`
      (if (`self.IsPlayingAnimation`)
        (`self.Re-call`)
        (else
          (set `self.Premature_ending` false)
          (`self.DisableInput` (`self.PlayerController`))
          (set `PlayerController.bShowMouseCursor` false (`self.PlayerController`))
          (`WidgetBlueprintLibrary.SetInputMode_GameOnly` (`self.PlayerController`))
          (set `self.Animation_Direction` "NewEnumerator2")
          (`/Engine/EditorBlueprintResources/StandardMacros.IsValid` _examine_item
            (:`Is Valid`
              (`SceneComponent.K2_DetachFromComponent` (`Actor.RootComponent` _examine_item) "KeepWorld" "KeepWorld" "KeepWorld" true)
              (bind (_direction _lerpvalue) (`Timeline|Exanine_Finished_Timeline` :!via `PlayFromStart`)
                (:`Update`
                  (bind (_returnvalue_location _returnvalue_rotation) (`KismetMathLibrary.BreakTransform` (`KismetMathLibrary.TLerp` _start_transform _end_transform _lerpvalue)))
                  (`self.K2_SetActorLocationAndRotation` (`self.Examine_Item`) _returnvalue_location _returnvalue_rotation false false))
                (:`Finished`
                  (`self.K2_SetActorTransform` (`self.Examine_Item`) (`self.Origin_Transform`) false false)
                  (bind _output_get (set `self.Relative_Rotation` (struct)))
                  (`SceneComponent.K2_SetRelativeRotation` (`self.Rotation_Root`) _output_get false false)
                  (set `self.Animation_Direction` "NewEnumerator0")
                  (if (`self.Premature_ending`)
                    (`self.Begin_Examine`)
                    (else
                      (`/Game/GeneralBlueprints/Main/FunctionLibrary/BFL_ControlInput.BFL_Set_ControllerLookInput` true)
                      (`/Game/GeneralBlueprints/Main/FunctionLibrary/BFL_ControlInput.BFL_Set_PlayerCharacterActionInput` true)
                      (`/Game/GeneralBlueprints/Main/ItemSystem/BP_MasterItem.Set_CollisionProfile` (`self.Examine_Item`) false)
                      (`self.K2_DestroyActor`))))))))))))

(event `self.ReceiveDestroyed`
  (bind _instigator (`self.Instigator`)
    (:`then`
      (bind _ascharacter (cast `Character` _instigator))
      (bind (_isactive _interactioncomponent) (`/Game/GeneralBlueprints/Main/FunctionLibrary/BFL_Interaction_Use.BFL_Get_Character_InteractionComponent` _ascharacter))
      (if _isactive
        (set `/Game/GeneralBlueprints/Main/Components/Player/Interaction/BP_Player_InteractionComponent.Examine_Actor` null _interactioncomponent)
        (`/Game/GeneralBlueprints/Main/Components/Player/Interaction/BP_Player_InteractionComponent.Enable_LOS` _interactioncomponent)))
    (:`else`)))

(event `Key|NumPadTwo`
  (params (Key :type "Key Structure"))
  ;[1 0 0.3584] Comment
  (:`Pressed`
    (bind _isa (`/Engine/EditorBlueprintResources/StandardMacros.FlipFlop`)
      (:`A`
        _)
      (:`B`
        _))
    (set `self.SimpleRotate_Option` _isa)))

(fn `Add_Rotation`
  (params (Scale :type "Float (double-precision)" :default 1.0) (Reverse :type Boolean))
  (bind _scale (`local.Scale`))
  (bind (_additive_rotation_x _additive_rotation_y) (`KismetMathLibrary.BreakVector2D` (`self.Additive_Rotation`)))
  (bind _scale_2 (`local.Scale`))
  (bind (_additive_rotation_x_2 _additive_rotation_y_2) (`KismetMathLibrary.BreakVector2D` (`self.Additive_Rotation`)))
  (bind _returnvalue (`KismetMathLibrary.SelectFloat` (* -1 _scale_2) _scale_2 (`local.Reverse`)))
  (if (`self.SimpleRotate_Option`)
    (`|ExecutionSequence`
      (:`then_0`
        (`SceneComponent.K2_SetWorldRotation` (`self.Rotation_Root`) (`self.Rotation_from_vector` (* (`self.GetInputAxisKeyValue`) (* (`local.Scale`) -2.0)) (`self.GetActorUpVector`)) false false))
      (:`then_1`
        (`SceneComponent.K2_SetWorldRotation` (`self.Rotation_Root`) (`self.Rotation_from_vector` (* (`self.GetInputAxisKeyValue`) (* (`local.Scale`) 2.0)) (`self.GetActorRightVector`)) false false)))
    (else
      (`|ExecutionSequence`
        (:`then_0`
          (`/Engine/EditorBlueprintResources/StandardMacros.CompareFloat` (`self.GetInputAxisKeyValue`)
            (:`>`
              (set `self.Additive_Rotation` (`KismetMathLibrary.MakeVector2D` (- _additive_rotation_x_2 _scale) _additive_rotation_y_2)))
            (:`<`
              (set `self.Additive_Rotation` (`KismetMathLibrary.MakeVector2D` (+ _additive_rotation_x_2 _scale) _additive_rotation_y_2)))))
        (:`then_1`
          (`/Engine/EditorBlueprintResources/StandardMacros.CompareFloat` (`self.GetInputAxisKeyValue`)
            (:`>`
              (set `self.Additive_Rotation` (`KismetMathLibrary.MakeVector2D` _additive_rotation_x_2 (- _additive_rotation_y_2 _returnvalue))))
            (:`<`
              (set `self.Additive_Rotation` (`KismetMathLibrary.MakeVector2D` _additive_rotation_x_2 (+ _additive_rotation_y_2 _returnvalue))))))
        (:`then_2`
          (bind _output_get (set `self.Relative_Rotation` (`KismetMathLibrary.RInterpTo` (`self.Relative_Rotation`) (`KismetMathLibrary.MakeRotator` 0.0 _additive_rotation_y _additive_rotation_x) (`GameplayStatics.GetWorldDeltaSeconds`) 5.0)))
          (`SceneComponent.K2_SetRelativeRotation` (`self.Rotation_Root`) _output_get false false))))))

(fn `ReverseRotation`
  (returns (Reverse :type Boolean))
  (bind _playercontroller (`self.PlayerController`))
  (bind (_locationx _locationy) (`PlayerController.GetMousePosition` _playercontroller))
  (bind (_worldposition _worlddirection) (`GameplayStatics.DeprojectScreenToWorld` _playercontroller (`KismetMathLibrary.MakeVector2D` _locationx _locationy)))
  (bind (_outhit _returnvalue) (`KismetSystemLibrary.LineTraceSingleForObjects` _worldposition (+ _worldposition (* _worlddirection 500.0)) (`|MakeArray` "ObjectTypeQuery7" :!type "EObjectTypeQuery Enum")))
  (if _returnvalue
    (return (< (`KismetMathLibrary.DegAcos` (`KismetMathLibrary.Dot_VectorVector` (`KismetMathLibrary.Normal` (`KismetMathLibrary.GetForwardVector` (`SceneComponent.K2_GetComponentRotation` (`self.Rotation_Root`)))) (`KismetMathLibrary.Normal` (- (`.Location` (`GameplayStatics.BreakHitResult` _outhit)) (`self.K2_GetActorLocation`))))) 90.0))))

(fn `Select_Scale`
  (returns (ReturnValue :type "Float (double-precision)"))
  (bind (_locationx _locationy) (`PlayerController.GetMousePosition` (`self.PlayerController`)))
  (return (`KismetMathLibrary.MapRangeClamped` (`KismetMathLibrary.VSize2D` (- (/ (`WidgetLayoutLibrary.GetViewportSize`) 2.0) (`KismetMathLibrary.MakeVector2D` _locationx _locationy))) 0.0 300.0 2.0 1.0)))

(fn `UserConstructionScript`
  (`/Engine/EditorBlueprintResources/StandardMacros.IsValid` (`self.Examine_Item`)
    (:`Is Valid`
      (bind _asbp_default_player_controller (cast `/Game/GeneralBlueprints/Main/Control/PlayerControllers/BP_DefaultPlayerController` (`self.GetOwner`)))
      (set `self.PlayerController` _asbp_default_player_controller)
      ;[1 0 0.3584] Comment
      (`KismetSystemLibrary.PrintString` "To change rotation mode press num 2" true true (struct :`G` 1.0 :`B` 0.009062 :`A` 1.0) 5.0))))