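; Player interaction component for BP_Char_Human that handles picking up, using, dropping and examining world items.
; Main action sphere-traces to pick up or interact through interfaces; side action uses the held item or toggles examine.
; A hand-slot map tracks held items, storing two-handed ones under both keys, while character dispatchers stow or drop the right-hand item.
; Examine spawns an actor at the camera manager's InspectLocation and suspends line-of-sight detection.
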(event `self.ReceiveBeginPlay`
  (`parent.ReceiveBeginPlay`)
  (bind _asbp_char_human (cast `/Game/GeneralBlueprints/Main/Characters/Player/BP_Char_Human` (`self.GetOwner`)))
  (set `self.Player` _asbp_char_human)
  (bind _player (`self.Player`)
    (:`then`
      (add `/Game/GeneralBlueprints/Main/Characters/Player/BP_Char_Human.EventDisp_AddItem` _player (delegate `CustomEvent_0`))
      (bind _player_2 (`self.Player`)
        (:`then`
          (add `/Game/GeneralBlueprints/Main/Characters/Player/BP_Char_Human.EventDisp_DropItem` _player_2 (delegate `CustomEvent_1`)))
        (:`else`)))
    (:`else`)))

(event `self.ReceiveEndPlay`
  (params (EndPlayReason :type "EEndPlayReason Enum" :default "Destroyed"))
  (clear `self.OnComponentDeactivated`))

(event `CustomEvent_0`
  (`self.Add Held Item To Inventory` "NewEnumerator1"))

(event `CustomEvent_1`
  (`self.Drop Held Item` "NewEnumerator1"))

(event `self.ReceiveTick`
  (params (DeltaSeconds :type "Float (single-precision)"))
  (`self.Switch_IsExamineItem`
    (:`T`
      (`self.Item At Sight Lost` (`self.Last Item At Sight`))
      (set `self.Last Item At Sight` null))
    (:`F`
      (`self.Check Line Of Sight Intersection`))))

(event `/Game/GeneralBlueprints/Main/Interfaces/Components/BPI_BaseInteraction.Main_Action`
  (bind (_interaction_param_x _interaction_param_y) (`KismetMathLibrary.BreakVector2D` (`self.Interaction_Param`)))
  (`self.Switch_IsExamineItem`
    (:`F`
      (bind (_returnvalue _last_hit_actor) (`/Game/GeneralBlueprints/Main/FunctionLibrary/BFL_Camera.BFL_Simple_SphereTrace` (`self.Get_OwnerController`) _interaction_param_x _interaction_param_y))
      (if _returnvalue
        (`/Engine/EditorBlueprintResources/StandardMacros.IsValid` _last_hit_actor
          (:`Is Valid`
            (`self.Switch_ItemInterfaces` _last_hit_actor
              (:`Pickable`
                (bind _aspickable_item (cast `/Game/GeneralBlueprints/Main/ItemSystem/Pickable/Pickable_Item` _last_hit_actor))
                (`self.Hold_Switch` _aspickable_item true))
              (:`Interactable`
                (message `/Game/GeneralBlueprints/Main/Interfaces/Items/BPI_Interactable.Interact` _last_hit_actor (`self.GetOwner`))))))))))

(event `/Game/GeneralBlueprints/Main/Interfaces/Components/BPI_BaseInteraction.Side_Action`
  (bind (_interaction_param_x _interaction_param_y) (`KismetMathLibrary.BreakVector2D` (`self.Interaction_Param`)))
  (`self.Switch_IsHoldingItem` "NewEnumerator2"
    (:`true`
      (message `/Game/GeneralBlueprints/Main/Interfaces/Items/BPI_Usable.Use` (`.Item` (`self.Get_SlotItem` "NewEnumerator0")) (`self.GetOwner`)))
    (:`false`
      (`self.Switch_IsExamineItem`
        (:`T`
          (`self.Stop_Examine`))
        (:`F`
          (bind (_returnvalue _last_hit_actor) (`/Game/GeneralBlueprints/Main/FunctionLibrary/BFL_Camera.BFL_Simple_SphereTrace` (`self.Get_OwnerController`) _interaction_param_x _interaction_param_y))
          (if _returnvalue
            (`self.Start_Examine` _last_hit_actor)))))))

(event `self.Item At Sight Gained`
  (params (`Last Item At Sight` :type "Actor Object Reference"))
  (`parent.Item At Sight Gained` `Last Item At Sight`))

(event `self.Item At Sight Lost`
  (params (`Last Item At Sight` :type "Actor Object Reference"))
  (`parent.Item At Sight Lost` `Last Item At Sight`))

(event `Add Held Item To Inventory`
  (params (Slot :type "/Game/GeneralBlueprints/Miscellaneous/Inventory/E_HandSlots Enum" :default "NewEnumerator0"))
  (bind (_exist _item) (`self.Get_SlotItem` Slot))
  (if _exist
    (bind _player (`self.Player`)
      (:`then`
        (message `/Game/GeneralBlueprints/Main/Interfaces/Items/BPI_Pickable.Add To Inventory` _item _player))
      (:`else`))))

(event `Drop Held Item`
  (params (Slot :type "/Game/GeneralBlueprints/Miscellaneous/Inventory/E_HandSlots Enum" :default "NewEnumerator0"))
  (bind (_exist _item) (`self.Get_SlotItem` Slot))
  (if _exist
    (`self.Hold_Switch` _item)))

(event `Inspect_Item`
  (params (Slot :type "/Game/GeneralBlueprints/Miscellaneous/Inventory/E_HandSlots Enum" :default "NewEnumerator0") (Slot2 :type "/Game/GeneralBlueprints/Miscellaneous/Inventory/E_HandSlots Enum" :default "NewEnumerator0"))
  (bind (_exist _item) (`self.Get_SlotItem` Slot2))
  (if _exist
    (message `/Game/GeneralBlueprints/Main/Interfaces/Items/BPI_Inspectable.Inspect` _item (`self.GetOwner`))))

(fn `Component_Initialization`
  (`parent.Component_Initialization`))

(fn `Get_SlotItem`
  (params (Slot :type "/Game/GeneralBlueprints/Miscellaneous/Inventory/E_HandSlots Enum" :default "NewEnumerator0"))
  (returns (Exist :type Boolean) (Item :type "/Game/GeneralBlueprints/Main/ItemSystem/Pickable/Pickable_Item Object Reference"))
  (locals (RightHand :type "EHand Enum" :default "VR_RightHand") (LeftHand :type "EHand Enum" :default "VR_LeftHand"))
  (bind (_both_ _value) (`self.Is_BothHands`))
  (bind (_value_2 _returnvalue) (`BlueprintMapLibrary.Map_Find` (`self.HandSlots`) (select `/Game/GeneralBlueprints/Miscellaneous/Inventory/E_HandSlots` (`local.Slot`) :`NewEnumerator0` "VR_LeftHand" :`NewEnumerator1` (`local.RightHand`) :`NewEnumerator2` (`local.LeftHand`) :`NewEnumerator3` "VR_LeftHand")))
  (switch `/Game/GeneralBlueprints/Miscellaneous/Inventory/E_HandSlots` Slot
    (:`NewEnumerator0`
      (return (`self.Is_HandsEmpty`) null))
    (:`NewEnumerator1`
      _)
    (:`NewEnumerator2`
      _)
    (:`NewEnumerator3`
      (return _both_ _value)))
  (return _returnvalue _value_2))

(fn `Get_ValidSlots`
  (returns (Keys :type "Array of EHand Enum"))
  (bind _keys (`BlueprintMapLibrary.Map_Keys` (`self.HandSlots`)))
  (return _keys))

(fn `Hold_Switch`
  (params (Item :type "/Game/GeneralBlueprints/Main/ItemSystem/Pickable/Pickable_Item Object Reference") (Hold :type Boolean))
  (locals (DesiredSlot :type "/Game/GeneralBlueprints/Miscellaneous/Inventory/E_HandSlots Enum"))
  (bind _returnvalue (`self.GetOwner`))
  (bind ((`SlotPriority_37_BA3499684EAE1C3FD85AB2A7E7E13969` _slotpriority)) (break `/Game/GeneralBlueprints/Miscellaneous/Inventory/InventoryStructure/ST_ItemSignature` (`/Game/GeneralBlueprints/Main/ItemSystem/BP_MasterItem.ItemSignature` Item)))
  (bind (_exist _item) (`self.Get_SlotItem` (`local.DesiredSlot`)))
  (bind (_exist_2 _item_2) (`self.Get_SlotItem` (`local.DesiredSlot`)))
  (`/Engine/EditorBlueprintResources/StandardMacros.IsValid` Item
    (:`Is Valid`
      (if (`|EnumInequality` _slotpriority "NewEnumerator0")
        (set `local.DesiredSlot` _slotpriority)
        (if (`local.Hold`)
          (`self.Switch_IsHoldingItem` (`local.DesiredSlot`)
            (:`false`
              (bind _success (`self.Set_Slots` (`local.DesiredSlot`) (`local.Item`)))
              (if _success
                (`KismetSystemLibrary.PrintString` (`KismetStringLibrary.Conv_BoolToString` _exist))
                (message `/Game/GeneralBlueprints/Main/Interfaces/Items/BPI_Pickable.Pick Up` _item _returnvalue (`self.Select_SocketName` _returnvalue (`local.DesiredSlot`))))))
          (else
            (`self.Switch_IsHoldingItem` (`local.DesiredSlot`)
              (:`true`
                (if (== _item_2 (`local.Item`))
                  (message `/Game/GeneralBlueprints/Main/Interfaces/Items/BPI_Pickable.Throw` _item_2)
                  (`self.Remove_Slot` (`local.DesiredSlot`))
                  (`self.Remove_Slot` (`local.DesiredSlot`)))))))))))

(fn `Is_BothHands`
  (returns (`Both?` :type Boolean) (Value :type "/Game/GeneralBlueprints/Main/ItemSystem/Pickable/Pickable_Item Object Reference"))
  (bind _handslots (`self.HandSlots`))
  (bind (_value _returnvalue) (`BlueprintMapLibrary.Map_Find` _handslots "VR_LeftHand"))
  (bind (_value_2 _returnvalue_2) (`BlueprintMapLibrary.Map_Find` _handslots "VR_RightHand"))
  (if _returnvalue_2
    (if _returnvalue
      (return (== _value_2 _value) _value_2))))

(fn `Is_HandsEmpty`
  (returns (ReturnValue :type Boolean))
  (return (== (`BlueprintMapLibrary.Map_Length` (`self.HandSlots`)) 0)))

(fn `Remove_Slot`
  (params (Slot :type "/Game/GeneralBlueprints/Miscellaneous/Inventory/E_HandSlots Enum" :default "NewEnumerator0"))
  (locals (RightHand :type "EHand Enum" :default "VR_RightHand") (LeftHand :type "EHand Enum"))
  (switch `/Game/GeneralBlueprints/Miscellaneous/Inventory/E_HandSlots` Slot
    (:`NewEnumerator1`
      (`BlueprintMapLibrary.Map_Remove` (`self.HandSlots`) (select `/Game/GeneralBlueprints/Miscellaneous/Inventory/E_HandSlots` (`local.Slot`) :`NewEnumerator0` "VR_LeftHand" :`NewEnumerator1` (`local.RightHand`) :`NewEnumerator2` (`local.LeftHand`) :`NewEnumerator3` "VR_LeftHand") :!label _label))
    (:`NewEnumerator2`
      (goto _label))
    (:`NewEnumerator3`
      (`BlueprintMapLibrary.Map_Clear` (`self.HandSlots`)))))

(fn `Select_SocketName`
  (params (Actor :type "Actor Object Reference") (Index :type "/Game/GeneralBlueprints/Miscellaneous/Inventory/E_HandSlots Enum" :default "NewEnumerator0"))
  (returns (ReturnValue :type Name))
  (bind _asbp_char_human (cast `/Game/GeneralBlueprints/Main/Characters/Player/BP_Char_Human` Actor)
    (:`then`
      (bind (_character_sockets_pelvisbone _character_sockets_headsocket _character_sockets_righthandsocket _character_sockets_lefthandsocket) (break `/Game/GeneralBlueprints/Miscellaneous/CharacterDefaults/Sockets/ST_CharacterSockets` (`/Game/GeneralBlueprints/Main/Characters/Player/BP_Char_Human.Character_Sockets` _asbp_char_human)))
      (return (select `/Game/GeneralBlueprints/Miscellaneous/Inventory/E_HandSlots` Index :`NewEnumerator1` _character_sockets_righthandsocket :`NewEnumerator2` _character_sockets_lefthandsocket :`NewEnumerator3` _character_sockets_righthandsocket)))
    (:`CastFailed`
      (return "None"))))

(fn `Set_Slots`
  (params (Slot :type "/Game/GeneralBlueprints/Miscellaneous/Inventory/E_HandSlots Enum" :default "NewEnumerator0") (Item :type "/Game/GeneralBlueprints/Main/ItemSystem/Pickable/Pickable_Item Object Reference"))
  (returns (Success :type Boolean))
  (locals (RightHand :type "EHand Enum" :default "VR_RightHand") (LeftHand :type "EHand Enum"))
  (if (`|EnumEquality` Slot "NewEnumerator0")
    (`BlueprintMapLibrary.Map_Clear` (`self.HandSlots`) :!label _label)
    (return true)
    (else
      (`/Engine/EditorBlueprintResources/StandardMacros.IsValid` (`local.Item`)
        (:`Is Valid`
          (switch `/Game/GeneralBlueprints/Miscellaneous/Inventory/E_HandSlots` (`local.Slot`)
            (:`NewEnumerator0`
              (goto _label))
            (:`NewEnumerator1`
              (`BlueprintMapLibrary.Map_Add` (`self.HandSlots`) (select `/Game/GeneralBlueprints/Miscellaneous/Inventory/E_HandSlots` (`local.Slot`) :`NewEnumerator0` "VR_LeftHand" :`NewEnumerator1` (`local.RightHand`) :`NewEnumerator2` (`local.LeftHand`) :`NewEnumerator3` "VR_LeftHand") (`local.Item`) :!label _label_2)
              (return true))
            (:`NewEnumerator2`
              (goto _label_2))
            (:`NewEnumerator3`
              (if (`self.Is_HandsEmpty`)
                (`BlueprintMapLibrary.Map_Clear` (`self.HandSlots`))
                (`BlueprintMapLibrary.Map_Add` (`self.HandSlots`) "VR_RightHand" (`local.Item`))
                (`BlueprintMapLibrary.Map_Add` (`self.HandSlots`) "VR_LeftHand" (`local.Item`))
                (return true)))))
        (:`Is Not Valid`
          (return false))))))

(fn `Start_Examine`
  (params (Actor :type "Actor Object Reference"))
  (locals (Item :type "/Game/GeneralBlueprints/Main/ItemSystem/BP_MasterItem Object Reference") (Inspect_Location :type "SceneComponent Object Reference"))
  (if (`KismetSystemLibrary.DoesImplementInterface` Actor "/Game/GeneralBlueprints/Main/Interfaces/Items/BPI_Examine.BPI_Examine_C")
    (bind _asbp_master_item (cast `/Game/GeneralBlueprints/Main/ItemSystem/BP_MasterItem` Actor))
    (set `local.Item` _asbp_master_item)
    (set `local.Inspect_Location` (`/Game/GeneralBlueprints/Main/Controllers/PlayerCameraManagers/BP_Default_PlayerCamManager.Inspect_Location` (cast `/Game/GeneralBlueprints/Main/Controllers/PlayerCameraManagers/BP_Default_PlayerCamManager` (`PlayerController.PlayerCameraManager` (`self.Get_OwnerController`)) :!pure true)))
    (bind _returnvalue (`|SpawnActorFromClass` "/Game/GeneralBlueprints/Main/Components/Player/Interaction/BP_Examine_Actor.BP_Examine_Actor_C" (`SceneComponent.K2_GetComponentToWorld` (`local.Inspect_Location`)) "Undefined" "OverrideRootScale" (`self.Get_OwnerController`) (`local.Item`) null))
    (bind _output_get (set `self.Examine_Actor` _returnvalue))
    (`Actor.K2_AttachToComponent` _output_get (`local.Inspect_Location`) "None" "SnapToTarget" "SnapToTarget" "SnapToTarget" true)
    (`/Game/GeneralBlueprints/Main/Components/Player/Interaction/BP_Examine_Actor.Begin_Examine` (`self.Examine_Actor`))))

(fn `Stop_Examine`
  (bind _examine_actor (`self.Examine_Actor`))
  (`/Engine/EditorBlueprintResources/StandardMacros.IsValid` _examine_actor
    (:`Is Valid`
      (`/Game/GeneralBlueprints/Main/Components/Player/Interaction/BP_Examine_Actor.Finish_Examine` _examine_actor)
      (set `self.Examine_Actor` null))))