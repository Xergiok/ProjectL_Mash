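; Player mental health component that tracks a clamped Sanity value and a three-tier MentalLevel derived from it.
; On BeginPlay it binds to the owning Pawn's any-damage event, but the handler is empty.
; SetSanity subtracts its input from Sanity, then sets the level by full sanity or a halfway threshold; its only call in the event graph is unreachable.
; Component initialization only calls the parent.
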(event `self.ReceiveBeginPlay`
  (bind _aspawn (cast `Pawn` (`self.GetOwner`)))
  (add `Actor.OnTakeAnyDamage` _aspawn (delegate `Recieve_MentalDamage`)))

(event `Recieve_MentalDamage`
  (params (DamagedActor :type "Actor Object Reference") (Damage :type "Float (double-precision)") (DamageType :type "DamageType Object Reference") (InstigatedBy :type "Controller Object Reference") (DamageCauser :type "Actor Object Reference")))

(fn `Component_Initialization`
  (`parent.Component_Initialization`))

(fn `Set_Sanity`
  (params (Value :type "Float (double-precision)"))
  (bind _output_get (set `self.Sanity` (`KismetMathLibrary.FClamp` (- (`self.Sanity`) Value))))
  (if (== _output_get 1.0)
    (set `self.Mental_Level` "NewEnumerator0")
    (elif (`KismetMathLibrary.InRange_FloatFloat` _output_get 0.5)
      (set `self.Mental_Level` "NewEnumerator1")
      (else
        (set `self.Mental_Level` "NewEnumerator2")))))