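; Player inventory component, named as old, that plays animations in sync on the current item's skeletal mesh and the owning character.
; Parallel events handle anim sequences, played as dynamic slot montages, and montages, each caching its latest request in a struct.
; Requests either play immediately or, if queued while a montage is playing, start a looping per-frame timer.
; That timer polls the player's anim instance and replays the cached request once it is free.
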(event `Component Initialization_1`)

(event `Sync_AnimSequence_Play`
  (params (Stop_existing :type Boolean) (Queued_playback :type Boolean) (Item_anim :type "AnimSequence Object Reference") (Character_anim :type "AnimSequence Object Reference") (InPlayRate :type "Float (double-precision)" :default 1.0) (DynamicSlot :type Name) (Reverse :type Boolean))
  (bind (_last_seq_prop_itemanim _last_seq_prop_characteranim _last_seq_prop_playrate _last_seq_prop_dynslotname _last_seq_prop_reverse) (break `/Game/GeneralBlueprints/Miscellaneous/Inventory/ItemAnims/ST_Sync_AnimSeq_Prop` (`self.Last_Seq_Prop`)))
  (bind _returnvalue (`KismetMathLibrary.SelectFloat` 1.0 0.0 _last_seq_prop_reverse))
  ;[1 1 1] An event that triggers the playing of animations synchronously for the item and the character that owns it
  (`/Engine/EditorBlueprintResources/StandardMacros.IsValid` (`self.Player`)
    (:`Is Valid`
      (set `self.Last_Seq_Prop` (make `/Game/GeneralBlueprints/Miscellaneous/Inventory/ItemAnims/ST_Sync_AnimSeq_Prop` Item_anim Character_anim InPlayRate DynamicSlot Reverse))
      (if Stop_existing
        (`|ExecutionSequence` :!label _label
          (:`then_0`
            (if (`SkeletalMeshComponent.HasValidAnimationInstance` (`/Game/GeneralBlueprints/Main/Storage/BP_Parent_Storage_Actor.Item_SKMesh` (`self.Current_Item`)))
              (`AnimInstance.PlaySlotAnimationAsDynamicMontage` (`self.Get_ItemAnimInstance`) _last_seq_prop_itemanim _last_seq_prop_dynslotname 0.2 0.2 _last_seq_prop_playrate 1 -1.0 _returnvalue)))
          (:`then_1`
            (`AnimInstance.PlaySlotAnimationAsDynamicMontage` (`self.Get_PlayerAnimInstance`) _last_seq_prop_characteranim _last_seq_prop_dynslotname 0.2 0.2 _last_seq_prop_playrate 1 -1.0 _returnvalue)))
        (elif Queued_playback
          (`self.AnyMontageIsPlaying?`
            (:`true`
              (bind _returnvalue_2 (`KismetSystemLibrary.K2_SetTimerDelegate` (delegate `SequenceQueue`) (`GameplayStatics.GetWorldDeltaSeconds`) true))
              (set `self.AnimQueueTimer` _returnvalue_2))
            (:`false`
              (goto _label))))))))

(event `SequenceQueue`
  (bind (_last_seq_prop_itemanim _last_seq_prop_characteranim _last_seq_prop_playrate _last_seq_prop_dynslotname _last_seq_prop_reverse) (break `/Game/GeneralBlueprints/Miscellaneous/Inventory/ItemAnims/ST_Sync_AnimSeq_Prop` (`self.Last_Seq_Prop`)))
  ;[1 1 1] An event that triggers the playing of animations synchronously for the item and the character that owns it
  (if (not (`AnimInstance.Montage_IsPlaying` (`self.Get_PlayerAnimInstance`) null))
    (`self.Sync_AnimSequence_Play` false false _last_seq_prop_itemanim _last_seq_prop_characteranim _last_seq_prop_playrate _last_seq_prop_dynslotname _last_seq_prop_reverse)
    (`KismetSystemLibrary.K2_ClearAndInvalidateTimerHandle` (`self.AnimQueueTimer`))))

(event `Sync_AnimMontage_Play`
  (params (Stop_existing :type Boolean) (Queued_playback :type Boolean) (Item_Montage :type "AnimMontage Object Reference") (Character_Montage :type "AnimMontage Object Reference") (InPlayRate :type "Float (double-precision)" :default 1.0) (Reverse :type Boolean))
  (bind (_last_mont_prop_itemmontage _last_mont_prop_charactermontage _last_mont_prop_playrate _last_mont_prop_reverse) (break `/Game/GeneralBlueprints/Miscellaneous/Inventory/ItemAnims/ST_Item_Montage_Prop` (`self.Last_Mont_Prop`)))
  (bind _returnvalue (`KismetMathLibrary.SelectFloat` 1.0 0.0 _last_mont_prop_reverse))
  ;[1 1 1] An event that triggers the playing of animations synchronously for the item and the character that owns it
  (`/Engine/EditorBlueprintResources/StandardMacros.IsValid` (`self.Player`)
    (:`Is Valid`
      (set `self.Last_Mont_Prop` (make `/Game/GeneralBlueprints/Miscellaneous/Inventory/ItemAnims/ST_Item_Montage_Prop` Item_Montage Character_Montage InPlayRate Reverse))
      (if Stop_existing
        (`|ExecutionSequence` :!label _label_2
          (:`then_0`
            (if (`SkeletalMeshComponent.HasValidAnimationInstance` (`/Game/GeneralBlueprints/Main/Storage/BP_Parent_Storage_Actor.Item_SKMesh` (`self.Current_Item`)))
              (`AnimInstance.Montage_Play` (`self.Get_ItemAnimInstance`) _last_mont_prop_itemmontage _last_mont_prop_playrate "Duration" _returnvalue true)))
          (:`then_1`
            (`AnimInstance.Montage_Play` (`self.Get_PlayerAnimInstance`) _last_mont_prop_charactermontage _last_mont_prop_playrate "Duration" _returnvalue true)))
        (elif Queued_playback
          (`self.AnyMontageIsPlaying?`
            (:`true`
              (bind _returnvalue_2 (`KismetSystemLibrary.K2_SetTimerDelegate` (delegate `MontageQueue`) (`GameplayStatics.GetWorldDeltaSeconds`) true))
              (set `self.AnimQueueTimer` _returnvalue_2))
            (:`false`
              (goto _label_2))))))))

(event `MontageQueue`
  (bind (_last_mont_prop_itemmontage _last_mont_prop_charactermontage _last_mont_prop_playrate _last_mont_prop_reverse) (break `/Game/GeneralBlueprints/Miscellaneous/Inventory/ItemAnims/ST_Item_Montage_Prop` (`self.Last_Mont_Prop`)))
  ;[1 1 1] An event that triggers the playing of animations synchronously for the item and the character that owns it
  (if (not (`AnimInstance.Montage_IsPlaying` (`self.Get_PlayerAnimInstance`) null))
    (`self.Sync_AnimMontage_Play` true false _last_mont_prop_itemmontage _last_mont_prop_charactermontage _last_mont_prop_playrate _last_mont_prop_reverse)
    (`KismetSystemLibrary.K2_ClearAndInvalidateTimerHandle` (`self.AnimQueueTimer`))))