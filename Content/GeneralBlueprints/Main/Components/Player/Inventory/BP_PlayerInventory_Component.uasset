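; Player inventory storage component that toggles the inventory display on the owning human character's event and manages moving items out to the hand.
; It shows either a viewport widget or a widget component, the latter opening only within a camera pitch limit and applying camera boundaries.
; Adding or removing items refreshes the open view.
; Removing a single-quantity entry spawns a pickable to hold, while larger stacks just decrement.
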(event `self.ReceiveBeginPlay`
  (`parent.ReceiveBeginPlay`))

(fn `Add Item To Storage`
  (params (`Item To Add` :type "/Game/GeneralBlueprints/Miscellaneous/Inventory/InventoryStructure/ST_InventorySlot Structure"))
  (returns (Success :type Boolean))
  (locals (`Is Successful` :type Boolean))
  (bind _alternative_inventory_widget (`self.Alternative Inventory Widget`))
  (bind _success (`parent.Add Item To Storage` `Item To Add`))
  (set `local.Is Successful` _success)
  (`self.Switch_IsOpened`
    (:`T`
      (if (`self.Alternative Inventory`)
        (`/Game/GeneralBlueprints/Widget/InventoryUI/WB_AlternativeInventoryWindow.Init Indexes` _alternative_inventory_widget)
        (`/Game/GeneralBlueprints/Widget/InventoryUI/WB_AlternativeInventoryWindow.ShowAltInventory` _alternative_inventory_widget)
        (else
          (`/Game/GeneralBlueprints/Widget/InventoryUI/WB_InvenoryWindow.Show Inventory` (`/Game/GeneralBlueprints/Main/Components/Player/Inventory/BP_Inventory_WidgetComponent.InventoryWindow` (`self.WidgetComp`))))))
    (:`F`
      _))
  (return (`local.Is Successful`)))

(fn `Component_Initialization`
  (`parent.Component_Initialization`)
  (bind _asbp_char_human (cast `/Game/GeneralBlueprints/Main/Characters/Player/BP_Char_Human` (`self.GetOwner`)))
  (add `/Game/GeneralBlueprints/Main/Characters/Player/BP_Char_Human.EventDisp_ToggleInventory` _asbp_char_human (`|CreateDelegate` :!event `Toggle`)))

(fn `Get_HeldItem`
  (returns (Exist :type Boolean) (Held_Item :type "/Game/GeneralBlueprints/Main/ItemSystem/Pickable/Pickable_Item Object Reference"))
  (bind _ascharacter (cast `Character` (`self.GetOwner`)))
  (bind (_exist _held_item) (`/Game/GeneralBlueprints/Main/FunctionLibrary/BFL_Interaction_Use.BFL_Get_HeldItem` _ascharacter))
  (return _exist _held_item))

(fn `Remove Item From Storage`
  (params (`Item Index` :type Integer) (Force :type Boolean))
  (returns (Success :type Boolean))
  (locals (`Item to remove` :type "/Game/GeneralBlueprints/Main/ItemSystem/Pickable/Pickable_Item Object Reference"))
  (bind (_output_itemstructure _output_quantity) (break `/Game/GeneralBlueprints/Miscellaneous/Inventory/InventoryStructure/ST_InventorySlot` (`|GetArrayItem` (`self.Items`) `Item Index`)))
  (bind _output (`|GetArrayItem` (`self.Items`) (`local.Item Index`)))
  (if (> _output_quantity 1)
    (`KismetArrayLibrary.Array_Set` (`self.Items`) (`local.Item Index`) (make `/Game/GeneralBlueprints/Miscellaneous/Inventory/InventoryStructure/ST_InventorySlot` _output_itemstructure (- _output_quantity 1)))
    (`self.Switch_IsOpened` :!label _label
      (:`T`
        (if (`self.Alternative Inventory`)
          (`/Game/GeneralBlueprints/Widget/InventoryUI/WB_AlternativeInventoryWindow.Update Indexes` (`self.Alternative Inventory Widget`) true)
          (else
            (`/Game/GeneralBlueprints/Widget/InventoryUI/WB_InvenoryWindow.Show Inventory` (`/Game/GeneralBlueprints/Main/Components/Player/Inventory/BP_Inventory_WidgetComponent.InventoryWindow` (`self.WidgetComp`)))
            (return false))))
      (:`F`
        (return false)))
    (else
      (`self.Switch_IsHoldingItem`
        (:`T`
          (if (`local.Force`)
            (message `/Game/GeneralBlueprints/Main/Interfaces/Components/BPI_PlayerInteraction.Hold_Switch_BPIF` (`self.GetOwner`) (`.Held_Item` (`self.Get_HeldItem`)) false)
            (bind _returnvalue (`|SpawnActorFromClass` (`.Class_26_E006C6FB4E2DC58CD00E21BEACA06322` (break `/Game/GeneralBlueprints/Miscellaneous/Inventory/InventoryStructure/ST_ItemSignature` (break `/Game/GeneralBlueprints/Miscellaneous/Inventory/InventoryStructure/ST_InventorySlot` _output))) (`KismetMathLibrary.MakeTransform` (0.0 0.0 0.0)) "Undefined" "OverrideRootScale" null (`.Quantity_5_715DEC3F4D3BC6156DE64DAEE147E216` (break `/Game/GeneralBlueprints/Miscellaneous/Inventory/InventoryStructure/ST_InventorySlot` _output)) null :!label _label_2))
            (bind _aspickable_item (cast `/Game/GeneralBlueprints/Main/ItemSystem/Pickable/Pickable_Item` _returnvalue))
            (bind _output_get (set `local.Item to remove` _aspickable_item))
            (`/Game/GeneralBlueprints/Main/ItemSystem/BP_MasterItem.Set_CollisionProfile` _output_get true)
            (`KismetArrayLibrary.Array_Remove` (`self.Items`) (`local.Item Index`))
            (message `/Game/GeneralBlueprints/Main/Interfaces/Components/BPI_PlayerInteraction.Hold_Switch_BPIF` (`self.GetOwner`) (`local.Item to remove`) true)
            (goto _label)))
        (:`F`
          (goto _label_2))))))

(fn `Replase_Items`
  (params (Item_to_add :type "/Game/GeneralBlueprints/Main/ItemSystem/Pickable/Pickable_Item Object Reference") (Item_to_remove_index :type Integer))
  (returns (Success :type Boolean))
  (`/Engine/EditorBlueprintResources/StandardMacros.IsValid` Item_to_add
    (:`Is Valid`
      (message `/Game/GeneralBlueprints/Main/Interfaces/Items/BPI_Pickable.Add To Inventory` (`local.Item_to_add`) (`self.GetOwner`)))
    (:`Is Not Valid`
      (`self.Switch_IsHoldingItem`
        (:`T`
          (return false))
        (:`F`
          _))))
  (if (and (`KismetArrayLibrary.Array_IsValidIndex` (`self.Items`)) (>= (`local.Item_to_remove_index`) 0))
    (bind _success (`self.Remove Item From Storage` (`local.Item_to_remove_index`) true))
    (return _success)))

(fn `Set_Inventory_Boundaries`
  (params (Opened :type Boolean))
  (bind _playercameramanager (`PlayerController.PlayerCameraManager` (`GameplayStatics.GetPlayerController` 0)))
  (if Opened
    (bind _asbp_default_player_cam_manager (cast `/Game/GeneralBlueprints/Main/Control/PlayerCameraManagers/BP_Default_PlayerCamManager` _playercameramanager))
    (`/Game/GeneralBlueprints/Main/Control/PlayerCameraManagers/BP_Default_PlayerCamManager.Set_Boundaries` _asbp_default_player_cam_manager (`self.Inventory_Boundaries`) false)
    (`/Game/GeneralBlueprints/Main/Control/PlayerCameraManagers/BP_Default_PlayerCamManager.Should_UpdateBoundaries` _asbp_default_player_cam_manager true)
    (else
      (bind _asbp_default_player_cam_manager_2 (cast `/Game/GeneralBlueprints/Main/Control/PlayerCameraManagers/BP_Default_PlayerCamManager` _playercameramanager))
      (`/Game/GeneralBlueprints/Main/Control/PlayerCameraManagers/BP_Default_PlayerCamManager.Boundaries_NormalMode` _asbp_default_player_cam_manager_2 false)
      (`/Game/GeneralBlueprints/Main/Control/PlayerCameraManagers/BP_Default_PlayerCamManager.Should_UpdateBoundaries` _asbp_default_player_cam_manager_2 false))))

(fn `Set_WidgetComp`
  (params (WidgetComponent :type "WidgetComponent Object Reference"))
  (`/Engine/EditorBlueprintResources/StandardMacros.IsValid` WidgetComponent
    (:`Is Valid`
      (bind _asbp_inventory_widget_component (cast `/Game/GeneralBlueprints/Main/Components/Player/Inventory/BP_Inventory_WidgetComponent` WidgetComponent))
      (set `self.WidgetComp` _asbp_inventory_widget_component))))

(fn `Toggle`
  (bind _widgetcomp (`self.WidgetComp`))
  (bind _inventory_boundaries_pitch_rangeminmax (break `/Game/GeneralBlueprints/Miscellaneous/CharacterDefaults/Camera/ST_CameraBoundaries` (`self.Inventory_Boundaries`)))
  (bind (_returnvalue_roll _returnvalue_pitch) (`KismetMathLibrary.BreakRotator` (`PlayerCameraManager.GetCameraRotation` (`GameplayStatics.GetPlayerCameraManager` 0))))
  (if (`self.Alternative Inventory`)
    (`self.Switch_IsOpened`
      (:`T`
        (`Widget.RemoveFromParent` (`self.Alternative Inventory Widget`))
        (set `self.Opened` false))
      (:`F`
        (bind _returnvalue (`|CreateWidget` "/Game/GeneralBlueprints/Widget/InventoryUI/WB_AlternativeInventoryWindow.WB_AlternativeInventoryWindow_C"))
        (bind _output_get (set `self.Alternative Inventory Widget` _returnvalue))
        (set `/Game/GeneralBlueprints/Widget/InventoryUI/WB_AlternativeInventoryWindow.Inventory_Storage` self _output_get)
        (`UserWidget.AddToViewport` (`self.Alternative Inventory Widget`) 0)
        (`/Game/GeneralBlueprints/Widget/InventoryUI/WB_AlternativeInventoryWindow.ShowAltInventory` (`self.Alternative Inventory Widget`))
        (set `self.Opened` true)))
    (else
      (`self.Switch_IsOpened`
        (:`T`
          (`SceneComponent.SetVisibility` _widgetcomp false false)
          (`self.Set_Inventory_Boundaries` false)
          (set `self.Opened` (not (`self.Opened`)) :!label _label))
        (:`F`
          (if (<= _returnvalue_pitch (`.Y` (`KismetMathLibrary.BreakVector2D` _inventory_boundaries_pitch_rangeminmax)))
            (`SceneComponent.SetVisibility` _widgetcomp true false)
            (`/Game/GeneralBlueprints/Widget/InventoryUI/WB_InvenoryWindow.Show Inventory` (`/Game/GeneralBlueprints/Main/Components/Player/Inventory/BP_Inventory_WidgetComponent.InventoryWindow` (`self.WidgetComp`)))
            (`self.Set_Inventory_Boundaries` true)
            (goto _label)))))))