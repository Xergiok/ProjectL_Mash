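; BP_Inventory_WidgetComponent is a widget component that connects a player inventory component to its inventory window widget.
; On BeginPlay it sizes the storage to three rows of MaxItemsInRow, then passes the storage and row width to the WB_InvenoryWindow it hosts.
; A setter accepts only a valid BP_PlayerInventory_Component as that storage.
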(event `self.ReceiveBeginPlay`
  (set `/Game/GeneralBlueprints/Main/Components/Player/Inventory/BP_PlayerInventory_Component.Capacity` (* (`self.Max Items In Row`) 3) (`self.StorageComp`))
  (bind _asinventorywindow (cast `/Game/GeneralBlueprints/Widget/InventoryUI/WB_InvenoryWindow` (`self.GetUserWidgetObject`)))
  (bind _output_get (set `self.InventoryWindow` _asinventorywindow))
  (set `/Game/GeneralBlueprints/Widget/InventoryUI/WB_InvenoryWindow.Inventory_Storage` (`self.StorageComp`) _output_get)
  (set `/Game/GeneralBlueprints/Widget/InventoryUI/WB_InvenoryWindow.Max Items In Row` (`self.Max Items In Row`) _output_get))

(fn `Set_StorageComp`
  (params (Inventory :type "/Game/GeneralBlueprints/Main/Components/Player/Inventory/BP_PlayerInventory_Component Object Reference"))
  (`/Engine/EditorBlueprintResources/StandardMacros.IsValid` Inventory
    (:`Is Valid`
      (bind _asbp_player_inventory_component (cast `/Game/GeneralBlueprints/Main/Components/Player/Inventory/BP_PlayerInventory_Component` Inventory))
      (set `self.StorageComp` _asbp_player_inventory_component))))