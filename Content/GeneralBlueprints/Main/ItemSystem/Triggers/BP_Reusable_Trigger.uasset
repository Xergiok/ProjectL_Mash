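; Reusable trigger in the item system that shows its link to ActorToInteract as a debug visual.
; After the parent construction script, it flushes persistent debug lines and draws a long-lived pink arrow from itself to that actor.
; Debug also has an unused SmallArrow mode that adds an arrow component rotated along the direction from the actor to the trigger.
; No trigger logic appears here.
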(fn `UserConstructionScript`
  (`parent.UserConstructionScript`)
  (`|ExecutionSequence`
    (:`then_0`
      (`KismetSystemLibrary.FlushPersistentDebugLines`)
      (if false
        (bind _returnvalue (`AddComponent|NODE_AddArrowComponent-0`))
        (`ArrowComponent.SetArrowColor` _returnvalue (struct :`R` 1.0 :`B` 0.806269 :`A` 1.0))
        (bind _actor_to_interact (`self.Actor to interact`)
          (:`then`
            (`SceneComponent.K2_SetWorldRotation` _returnvalue (`KismetMathLibrary.FindLookAtRotation` (`self.K2_GetActorLocation` _actor_to_interact) (`self.K2_GetActorLocation`)) false false))
          (:`else`))
        (else
          (bind _actor_to_interact_2 (`self.Actor to interact`)
            (:`then`
              (`KismetSystemLibrary.DrawDebugArrow` (`self.K2_GetActorLocation`) (`self.K2_GetActorLocation` _actor_to_interact_2) 10.0 (struct :`R` 0.887923 :`B` 0.619479 :`A` 1.0) 999999.0 2.0))
            (:`else`)))))))