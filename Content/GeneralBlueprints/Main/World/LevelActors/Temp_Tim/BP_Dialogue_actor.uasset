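; Dialogue actor whose camera-facing bubble offers up to four unused replies, one gated on HasGun, and destroys itself when none remain.
; MainAction registers it as speaker in the GameInstance and swaps player input for dialogue keys, routed back as interface messages.
; A first press expands a reply; repeating confirms, another cancels.
; A timer animation defaults to the first option; StressedMode locks the first press and auto-confirms after a delay.
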(event `self.ReceiveBeginPlay`
  (`Widget.SetVisibility` (`WidgetComponent.GetUserWidgetObject` (`self.options_act`)) "Hidden"))

(event `self.ReceiveTick`
  (params (DeltaSeconds :type "Float (single-precision)"))
  (bind (_location _rotation) (`/Game/GeneralBlueprints/Main/FunctionLibrary/BFL_Camera.BFL_Get_CurrentCamera_Location/Rotation` 0))
  (bind _options_act (`self.options_act`))
  ;[1 1 1] widget rotation
  (`SceneComponent.K2_SetRelativeLocationAndRotation` _options_act (`KismetMathLibrary.GreaterGreater_VectorRotator` (0.0 100.0 90.0) _rotation) (`KismetMathLibrary.FindLookAtRotation` (`SceneComponent.K2_GetComponentLocation` _options_act) _location) false false))

(event `InputAction|Dialogue1`
  (params (Key :type "Key Structure"))
  ;[1 1 1] dialogue choice (bind 1-4) + cancel
  (:`Pressed`
    (bind _asbp_game_inst_variable_storage (cast `/Game/GeneralBlueprints/Main/GameInstance/BP_GameInst_VariableStorage` (`GameplayStatics.GetGameInstance`)))
    (if (`/Game/GeneralBlueprints/Main/GameInstance/BP_GameInst_VariableStorage.isSpeaking` _asbp_game_inst_variable_storage)
      (bind _asbp_game_inst_variable_storage_2 (cast `/Game/GeneralBlueprints/Main/GameInstance/BP_GameInst_VariableStorage` (`GameplayStatics.GetGameInstance`)))
      (message `/Game/GeneralBlueprints/Main/Interfaces/BPI_DialogueChoice.case1` (`/Game/GeneralBlueprints/Main/GameInstance/BP_GameInst_VariableStorage.whoHeIsSpeakingTo` _asbp_game_inst_variable_storage_2)))))

(event `InputAction|Dialogue2`
  (params (Key :type "Key Structure"))
  ;[1 1 1] dialogue choice (bind 1-4) + cancel
  (:`Pressed`
    (bind _asbp_game_inst_variable_storage (cast `/Game/GeneralBlueprints/Main/GameInstance/BP_GameInst_VariableStorage` (`GameplayStatics.GetGameInstance`)))
    (if (`/Game/GeneralBlueprints/Main/GameInstance/BP_GameInst_VariableStorage.isSpeaking` _asbp_game_inst_variable_storage)
      (bind _asbp_game_inst_variable_storage_2 (cast `/Game/GeneralBlueprints/Main/GameInstance/BP_GameInst_VariableStorage` (`GameplayStatics.GetGameInstance`)))
      (message `/Game/GeneralBlueprints/Main/Interfaces/BPI_DialogueChoice.case2` (`/Game/GeneralBlueprints/Main/GameInstance/BP_GameInst_VariableStorage.whoHeIsSpeakingTo` _asbp_game_inst_variable_storage_2)))))

(event `InputAction|Dialogue3`
  (params (Key :type "Key Structure"))
  ;[1 1 1] dialogue choice (bind 1-4) + cancel
  (:`Pressed`
    (bind _asbp_game_inst_variable_storage (cast `/Game/GeneralBlueprints/Main/GameInstance/BP_GameInst_VariableStorage` (`GameplayStatics.GetGameInstance`)))
    (if (`/Game/GeneralBlueprints/Main/GameInstance/BP_GameInst_VariableStorage.isSpeaking` _asbp_game_inst_variable_storage)
      (bind _asbp_game_inst_variable_storage_2 (cast `/Game/GeneralBlueprints/Main/GameInstance/BP_GameInst_VariableStorage` (`GameplayStatics.GetGameInstance`)))
      (message `/Game/GeneralBlueprints/Main/Interfaces/BPI_DialogueChoice.case3` (`/Game/GeneralBlueprints/Main/GameInstance/BP_GameInst_VariableStorage.whoHeIsSpeakingTo` _asbp_game_inst_variable_storage_2)))))

(event `InputAction|Dialogue4`
  (params (Key :type "Key Structure"))
  ;[1 1 1] dialogue choice (bind 1-4) + cancel
  (:`Pressed`
    (bind _asbp_game_inst_variable_storage (cast `/Game/GeneralBlueprints/Main/GameInstance/BP_GameInst_VariableStorage` (`GameplayStatics.GetGameInstance`)))
    (if (`/Game/GeneralBlueprints/Main/GameInstance/BP_GameInst_VariableStorage.isSpeaking` _asbp_game_inst_variable_storage)
      (bind _asbp_game_inst_variable_storage_2 (cast `/Game/GeneralBlueprints/Main/GameInstance/BP_GameInst_VariableStorage` (`GameplayStatics.GetGameInstance`)))
      (message `/Game/GeneralBlueprints/Main/Interfaces/BPI_DialogueChoice.case4` (`/Game/GeneralBlueprints/Main/GameInstance/BP_GameInst_VariableStorage.whoHeIsSpeakingTo` _asbp_game_inst_variable_storage_2)))))

(event `InputAction|CancelDialogue`
  (params (Key :type "Key Structure"))
  ;[1 1 1] dialogue choice (bind 1-4) + cancel
  (:`Pressed`
    (bind _asbp_game_inst_variable_storage (cast `/Game/GeneralBlueprints/Main/GameInstance/BP_GameInst_VariableStorage` (`GameplayStatics.GetGameInstance`)))
    (if (`/Game/GeneralBlueprints/Main/GameInstance/BP_GameInst_VariableStorage.isSpeaking` _asbp_game_inst_variable_storage)
      (bind _asbp_game_inst_variable_storage_2 (cast `/Game/GeneralBlueprints/Main/GameInstance/BP_GameInst_VariableStorage` (`GameplayStatics.GetGameInstance`)))
      (message `/Game/GeneralBlueprints/Main/Interfaces/BPI_DialogueChoice.dialogueCanceling` (`/Game/GeneralBlueprints/Main/GameInstance/BP_GameInst_VariableStorage.whoHeIsSpeakingTo` _asbp_game_inst_variable_storage_2)))))

(event `/Game/GeneralBlueprints/Main/Interfaces/BPI_DialogueChoice.dialogueCanceling`
  ;[1 1 1] dialogue canceling can be done via pressing a button of other choice or pressing a specific button (Q)
  (if (`self.hasExpandedSpeechBubbleAndWaitingForConfirmation`)
    (`KismetSystemLibrary.PrintString` "canceling")
    ;[1 1 1] animations and decisions
    (bind _asumg_options (cast `/Game/GeneralBlueprints/Widget/Dialogue/UMG_options` (`WidgetComponent.GetUserWidgetObject` (`self.options_act`)) :!label _label))
    (`UserWidget.PlayAnimation` _asumg_options (`self.buffer_anim`) 0.0 1 "Reverse" (`self.amination_speed`) false)
    (`self.reversing_content_animation` (`self.border_buffer`))
    (set `self.hasExpandedSpeechBubbleAndWaitingForConfirmation` false)
    (set `self.whatWasChosen` 0)))

(event `/Game/GeneralBlueprints/Main/Interfaces/BPI_DialogueChoice.case1`
  (bind _whatwaschosen (`self.whatWasChosen`))
  (bind _returnvalue (`WidgetComponent.GetUserWidgetObject` (`self.empty_widget`)))
  ;[1 1 1] animations and decisions
  (if (`self.1st_option_valid`)
    (`KismetSystemLibrary.PrintString` "1")
    (if (`self.hasExpandedSpeechBubbleAndWaitingForConfirmation`)
      (bind _asbp_game_inst_variable_storage (cast `/Game/GeneralBlueprints/Main/GameInstance/BP_GameInst_VariableStorage` (`GameplayStatics.GetGameInstance`)))
      (if (`/Game/GeneralBlueprints/Main/GameInstance/BP_GameInst_VariableStorage.stressed_mode` _asbp_game_inst_variable_storage)
        (`KismetSystemLibrary.PrintString` "can't change nor confirm variant, too stressed" :!label _label_2)
        (elif (== (`self.whatWasChosen`) 1)
          (`KismetSystemLibrary.PrintString` "chose variant 1" :!label _label_3)
          (bind _asumg_options (cast `/Game/GeneralBlueprints/Widget/Dialogue/UMG_options` (`WidgetComponent.GetUserWidgetObject` (`self.options_act`))))
          (`self.validating_options` (`/Game/GeneralBlueprints/Widget/Dialogue/UMG_options.Border_1` _asumg_options))
          (bind _asbp_game_inst_variable_storage_2 (cast `/Game/GeneralBlueprints/Main/GameInstance/BP_GameInst_VariableStorage` (`GameplayStatics.GetGameInstance`) :!label _label_4))
          (set `/Game/GeneralBlueprints/Main/GameInstance/BP_GameInst_VariableStorage.isSpeaking` false _asbp_game_inst_variable_storage_2)
          ;[1 1 1] swiftly reversing the animation that just played
          (bind _asumg_options_2 (cast `/Game/GeneralBlueprints/Widget/Dialogue/UMG_options` (`WidgetComponent.GetUserWidgetObject` (`self.options_act`))))
          (`UserWidget.PlayAnimation` _asumg_options_2 (`self.buffer_anim`) 0.0 1 "Reverse" 20.0 false)
          (set `self.hasExpandedSpeechBubbleAndWaitingForConfirmation` false)
          (set `self.whatWasChosen` 0)
          (`Widget.SetVisibility` (`WidgetComponent.GetUserWidgetObject` (`self.options_act`)) "Hidden")
          (bind _asumg_options_3 (cast `/Game/GeneralBlueprints/Widget/Dialogue/UMG_options` (`WidgetComponent.GetUserWidgetObject` (`self.options_act`))))
          (`ContentWidget.SetContent` (`/Game/GeneralBlueprints/Widget/Dialogue/UMG_options.Border_1` _asumg_options_3) _returnvalue)
          (`ContentWidget.SetContent` (`/Game/GeneralBlueprints/Widget/Dialogue/UMG_options.Border_2` _asumg_options_3) _returnvalue)
          (`ContentWidget.SetContent` (`/Game/GeneralBlueprints/Widget/Dialogue/UMG_options.Border_3` _asumg_options_3) _returnvalue)
          (`ContentWidget.SetContent` (`/Game/GeneralBlueprints/Widget/Dialogue/UMG_options.Border_4` _asumg_options_3) _returnvalue)
          (`KismetSystemLibrary.PrintString` "finish speaking")
          (`self.Switch_DialogInput` false)
          (else
            (goto _label))))
      (else
        (bind _asumg_options_4 (cast `/Game/GeneralBlueprints/Widget/Dialogue/UMG_options` (`WidgetComponent.GetUserWidgetObject` (`self.options_act`))))
        (bind _choose1 (`/Game/GeneralBlueprints/Widget/Dialogue/UMG_options.Choose1` _asumg_options_4))
        (`UserWidget.PlayAnimation` _asumg_options_4 _choose1 0.0 1 "Forward" (`self.amination_speed`) false)
        (set `self.buffer_anim` _choose1)
        (bind _border_1 (`/Game/GeneralBlueprints/Widget/Dialogue/UMG_options.Border_1` _asumg_options_4))
        (`self.playing_content_animation` _border_1)
        (set `self.border_buffer` _border_1)
        (set `self.hasExpandedSpeechBubbleAndWaitingForConfirmation` true)
        (set `self.whatWasChosen` 1)
        (bind _asbp_game_inst_variable_storage_3 (cast `/Game/GeneralBlueprints/Main/GameInstance/BP_GameInst_VariableStorage` (`GameplayStatics.GetGameInstance`)))
        (if (`/Game/GeneralBlueprints/Main/GameInstance/BP_GameInst_VariableStorage.stressed_mode` _asbp_game_inst_variable_storage_3)
          (bind _asumg_options_5 (cast `/Game/GeneralBlueprints/Widget/Dialogue/UMG_options` (`WidgetComponent.GetUserWidgetObject` (`self.options_act`)) :!label _label_5))
          (`UserWidget.StopAnimation` _asumg_options_5 (`/Game/GeneralBlueprints/Widget/Dialogue/UMG_options.time` _asumg_options_5))
          (`UserWidget.PlayAnimation` _asumg_options_5 (`/Game/GeneralBlueprints/Widget/Dialogue/UMG_options.stressed_time` _asumg_options_5) 0.0 1 "Forward" 1.0 false)
          (`KismetSystemLibrary.Delay` 5.0)
          (if (== _whatwaschosen 1)
            (goto _label_3)
            (elif (== _whatwaschosen 2)
              (`KismetSystemLibrary.PrintString` "chose variant 2" :!label _label_6)
              (bind _asumg_options_6 (cast `/Game/GeneralBlueprints/Widget/Dialogue/UMG_options` (`WidgetComponent.GetUserWidgetObject` (`self.options_act`))))
              (`self.validating_options` (`/Game/GeneralBlueprints/Widget/Dialogue/UMG_options.Border_2` _asumg_options_6))
              (goto _label_4)
              (elif (== _whatwaschosen 3)
                (`KismetSystemLibrary.PrintString` "chose variant 3" :!label _label_7)
                (bind _asumg_options_7 (cast `/Game/GeneralBlueprints/Widget/Dialogue/UMG_options` (`WidgetComponent.GetUserWidgetObject` (`self.options_act`))))
                (`self.validating_options` (`/Game/GeneralBlueprints/Widget/Dialogue/UMG_options.Border_3` _asumg_options_7))
                (goto _label_4)
                (elif (== _whatwaschosen 4)
                  (`KismetSystemLibrary.PrintString` "chose variant 4" :!label _label_8)
                  (bind _asumg_options_8 (cast `/Game/GeneralBlueprints/Widget/Dialogue/UMG_options` (`WidgetComponent.GetUserWidgetObject` (`self.options_act`))))
                  (`self.validating_options` (`/Game/GeneralBlueprints/Widget/Dialogue/UMG_options.Border_4` _asumg_options_8))
                  (goto _label_4)
                  (else
                    (`KismetSystemLibrary.PrintString` "something is clearly fucking wrong" true true (struct :`R` 0.963607 :`B` 1.0 :`A` 1.0))))))))))))

(event `/Game/GeneralBlueprints/Main/Interfaces/BPI_DialogueChoice.case2`
  (bind _amination_speed (`self.amination_speed`))
  ;[1 1 1] animations and decisions
  (if (`self.2nd_option_valid`)
    (`KismetSystemLibrary.PrintString` "2")
    (if (`self.hasExpandedSpeechBubbleAndWaitingForConfirmation`)
      (bind _asbp_game_inst_variable_storage (cast `/Game/GeneralBlueprints/Main/GameInstance/BP_GameInst_VariableStorage` (`GameplayStatics.GetGameInstance`)))
      (if (`/Game/GeneralBlueprints/Main/GameInstance/BP_GameInst_VariableStorage.stressed_mode` _asbp_game_inst_variable_storage)
        (goto _label_2)
        (elif (== (`self.whatWasChosen`) 2)
          (goto _label_6)
          (else
            (bind _asumg_options (cast `/Game/GeneralBlueprints/Widget/Dialogue/UMG_options` (`WidgetComponent.GetUserWidgetObject` (`self.options_act`))))
            (`UserWidget.PlayAnimation` _asumg_options (`self.buffer_anim`) 0.0 1 "Reverse" _amination_speed false)
            (`self.reversing_content_animation` (`self.border_buffer`))
            (set `self.hasExpandedSpeechBubbleAndWaitingForConfirmation` false)
            (set `self.whatWasChosen` 0))))
      (else
        (bind _asumg_options_2 (cast `/Game/GeneralBlueprints/Widget/Dialogue/UMG_options` (`WidgetComponent.GetUserWidgetObject` (`self.options_act`))))
        (bind _choose2 (`/Game/GeneralBlueprints/Widget/Dialogue/UMG_options.Choose2` _asumg_options_2))
        (`UserWidget.PlayAnimation` _asumg_options_2 _choose2 0.0 1 "Forward" _amination_speed false)
        (set `self.buffer_anim` _choose2)
        (bind _border_2 (`/Game/GeneralBlueprints/Widget/Dialogue/UMG_options.Border_2` _asumg_options_2))
        (`self.playing_content_animation` _border_2)
        (set `self.border_buffer` _border_2)
        (set `self.hasExpandedSpeechBubbleAndWaitingForConfirmation` true)
        (set `self.whatWasChosen` 2)
        (bind _asbp_game_inst_variable_storage_2 (cast `/Game/GeneralBlueprints/Main/GameInstance/BP_GameInst_VariableStorage` (`GameplayStatics.GetGameInstance`)))
        (if (`/Game/GeneralBlueprints/Main/GameInstance/BP_GameInst_VariableStorage.stressed_mode` _asbp_game_inst_variable_storage_2)
          (goto _label_5))))))

(event `/Game/GeneralBlueprints/Main/Interfaces/Components/BPI_BaseInteraction.Main_Action`
  (bind _returnvalue (`KismetArrayLibrary.Array_IsValidIndex` (`self.interactTarget`) 3))
  (bind _returnvalue_2 (`KismetArrayLibrary.Array_IsValidIndex` (`self.interactTarget`)))
  (bind _returnvalue_3 (`KismetArrayLibrary.Array_IsValidIndex` (`self.interactTarget`) 1))
  (bind _returnvalue_4 (`KismetArrayLibrary.Array_IsValidIndex` (`self.interactTarget`) 2))
  (`self.Switch_DialogInput` true)
  (bind _asbp_game_inst_variable_storage (cast `/Game/GeneralBlueprints/Main/GameInstance/BP_GameInst_VariableStorage` (`GameplayStatics.GetGameInstance`)))
  (if (not (`/Game/GeneralBlueprints/Main/GameInstance/BP_GameInst_VariableStorage.isSpeaking` _asbp_game_inst_variable_storage))
    (`Widget.SetVisibility` (`WidgetComponent.GetUserWidgetObject` (`self.options_act`)) "Visible")
    (bind _asbp_game_inst_variable_storage_2 (cast `/Game/GeneralBlueprints/Main/GameInstance/BP_GameInst_VariableStorage` (`GameplayStatics.GetGameInstance`)))
    (set `/Game/GeneralBlueprints/Main/GameInstance/BP_GameInst_VariableStorage.isSpeaking` true _asbp_game_inst_variable_storage_2)
    (set `/Game/GeneralBlueprints/Main/GameInstance/BP_GameInst_VariableStorage.whoHeIsSpeakingTo` self _asbp_game_inst_variable_storage_2)
    ;[1 1 1] checking triggers and adding variants to array
    (bind _asbp_game_inst_variable_storage_3 (cast `/Game/GeneralBlueprints/Main/GameInstance/BP_GameInst_VariableStorage` (`GameplayStatics.GetGameInstance`)))
    (if (`/Game/GeneralBlueprints/Main/GameInstance/BP_GameInst_VariableStorage.hasGun` _asbp_game_inst_variable_storage_3)
      (if (not (`self.usedDiop_3`))
        (`KismetArrayLibrary.Array_Add` (`self.interactTarget`) (`self.diop3`))))
    (if (not (`self.usedDiop`))
      (`KismetArrayLibrary.Array_Add` (`self.interactTarget`) (`self.diop`)))
    (if (not (`self.usedDiop_1`))
      (`KismetArrayLibrary.Array_Add` (`self.interactTarget`) (`self.diop1`)))
    (if (not (`self.usedDiop_2`))
      (`KismetArrayLibrary.Array_Add` (`self.interactTarget`) (`self.diop2`)))
    ;[1 1 1] avoiding errors, validating dialogue choises
    (set `self.1st_option_valid` _returnvalue_2)
    (if _returnvalue_2
      (bind _asumg_options (cast `/Game/GeneralBlueprints/Widget/Dialogue/UMG_options` (`WidgetComponent.GetUserWidgetObject` (`self.options_act`))))
      (`ContentWidget.SetContent` (`/Game/GeneralBlueprints/Widget/Dialogue/UMG_options.Border_1` _asumg_options) (`WidgetComponent.GetUserWidgetObject` (`|GetArrayItem` (`self.interactTarget`))))
      (if _returnvalue_3
        (`ContentWidget.SetContent` (`/Game/GeneralBlueprints/Widget/Dialogue/UMG_options.Border_2` _asumg_options) (`WidgetComponent.GetUserWidgetObject` (`|GetArrayItem` (`self.interactTarget`) 1)))
        (if _returnvalue_4
          (`ContentWidget.SetContent` (`/Game/GeneralBlueprints/Widget/Dialogue/UMG_options.Border_3` _asumg_options) (`WidgetComponent.GetUserWidgetObject` (`|GetArrayItem` (`self.interactTarget`) 2)))
          (if _returnvalue
            (`ContentWidget.SetContent` (`/Game/GeneralBlueprints/Widget/Dialogue/UMG_options.Border_4` _asumg_options) (`WidgetComponent.GetUserWidgetObject` (`|GetArrayItem` (`self.interactTarget`) 3))))))
      (set `self.2nd_option_valid` _returnvalue_3)
      (set `self.3rd_option_valid` _returnvalue_4)
      (set `self.4th_option_valid` _returnvalue)
      (set `self.interactTarget` (`self.EMPTY_ARRAY_LUL`))
      ;[1 1 1] if none was chosen, first option is selected automatically
      (bind _asumg_options_2 (cast `/Game/GeneralBlueprints/Widget/Dialogue/UMG_options` (`WidgetComponent.GetUserWidgetObject` (`self.options_act`))))
      (`|PlayAnimation` _asumg_options_2 (`/Game/GeneralBlueprints/Widget/Dialogue/UMG_options.time` _asumg_options_2)
        (:`Finished`
          (bind _asbp_game_inst_variable_storage_4 (cast `/Game/GeneralBlueprints/Main/GameInstance/BP_GameInst_VariableStorage` (`GameplayStatics.GetGameInstance`)))
          (if (and (`/Game/GeneralBlueprints/Main/GameInstance/BP_GameInst_VariableStorage.stressed_mode` _asbp_game_inst_variable_storage_4) (`self.hasExpandedSpeechBubbleAndWaitingForConfirmation`))
            _
            (elif (`/Game/GeneralBlueprints/Main/GameInstance/BP_GameInst_VariableStorage.isSpeaking` _asbp_game_inst_variable_storage_4)
              (`KismetSystemLibrary.PrintString` "timeout")
              (goto _label_3)))))
      (else
        (`KismetSystemLibrary.PrintString` "BOOOOOOM!!!")
        (bind _asbp_game_inst_variable_storage_5 (cast `/Game/GeneralBlueprints/Main/GameInstance/BP_GameInst_VariableStorage` (`GameplayStatics.GetGameInstance`)))
        (set `/Game/GeneralBlueprints/Main/GameInstance/BP_GameInst_VariableStorage.isSpeaking` false _asbp_game_inst_variable_storage_5)
        ;;[1 1 1] if nothing left to talk about
        (`self.K2_DestroyActor`)
        (`self.Switch_DialogInput` false)))))

(event `/Game/GeneralBlueprints/Main/Interfaces/BPI_DialogueChoice.case3`
  (bind _amination_speed (`self.amination_speed`))
  ;[1 1 1] animations and decisions
  (if (`self.3rd_option_valid`)
    (`KismetSystemLibrary.PrintString` "3")
    (if (`self.hasExpandedSpeechBubbleAndWaitingForConfirmation`)
      (bind _asbp_game_inst_variable_storage (cast `/Game/GeneralBlueprints/Main/GameInstance/BP_GameInst_VariableStorage` (`GameplayStatics.GetGameInstance`)))
      (if (`/Game/GeneralBlueprints/Main/GameInstance/BP_GameInst_VariableStorage.stressed_mode` _asbp_game_inst_variable_storage)
        (goto _label_2)
        (elif (== (`self.whatWasChosen`) 3)
          (goto _label_7)
          (else
            (bind _asumg_options (cast `/Game/GeneralBlueprints/Widget/Dialogue/UMG_options` (`WidgetComponent.GetUserWidgetObject` (`self.options_act`))))
            (`UserWidget.PlayAnimation` _asumg_options (`self.buffer_anim`) 0.0 1 "Reverse" _amination_speed false)
            (`self.reversing_content_animation` (`self.border_buffer`))
            (set `self.hasExpandedSpeechBubbleAndWaitingForConfirmation` false)
            (set `self.whatWasChosen` 0))))
      (else
        (bind _asumg_options_2 (cast `/Game/GeneralBlueprints/Widget/Dialogue/UMG_options` (`WidgetComponent.GetUserWidgetObject` (`self.options_act`))))
        (bind _choose3 (`/Game/GeneralBlueprints/Widget/Dialogue/UMG_options.Choose3` _asumg_options_2))
        (`UserWidget.PlayAnimation` _asumg_options_2 _choose3 0.0 1 "Forward" _amination_speed false)
        (set `self.buffer_anim` _choose3)
        (bind _border_3 (`/Game/GeneralBlueprints/Widget/Dialogue/UMG_options.Border_3` _asumg_options_2))
        (`self.playing_content_animation` _border_3)
        (set `self.border_buffer` _border_3)
        (set `self.hasExpandedSpeechBubbleAndWaitingForConfirmation` true)
        (set `self.whatWasChosen` 3)
        (bind _asbp_game_inst_variable_storage_2 (cast `/Game/GeneralBlueprints/Main/GameInstance/BP_GameInst_VariableStorage` (`GameplayStatics.GetGameInstance`)))
        (if (`/Game/GeneralBlueprints/Main/GameInstance/BP_GameInst_VariableStorage.stressed_mode` _asbp_game_inst_variable_storage_2)
          (goto _label_5))))))

(event `/Game/GeneralBlueprints/Main/Interfaces/BPI_DialogueChoice.case4`
  (bind _amination_speed (`self.amination_speed`))
  ;[1 1 1] animations and decisions
  (if (`self.4th_option_valid`)
    (`KismetSystemLibrary.PrintString` "4")
    (if (`self.hasExpandedSpeechBubbleAndWaitingForConfirmation`)
      (bind _asbp_game_inst_variable_storage (cast `/Game/GeneralBlueprints/Main/GameInstance/BP_GameInst_VariableStorage` (`GameplayStatics.GetGameInstance`)))
      (if (`/Game/GeneralBlueprints/Main/GameInstance/BP_GameInst_VariableStorage.stressed_mode` _asbp_game_inst_variable_storage)
        (goto _label_2)
        (elif (== (`self.whatWasChosen`) 4)
          (goto _label_8)
          (else
            (bind _asumg_options (cast `/Game/GeneralBlueprints/Widget/Dialogue/UMG_options` (`WidgetComponent.GetUserWidgetObject` (`self.options_act`))))
            (`UserWidget.PlayAnimation` _asumg_options (`self.buffer_anim`) 0.0 1 "Reverse" _amination_speed false)
            (`self.reversing_content_animation` (`self.border_buffer`))
            (set `self.hasExpandedSpeechBubbleAndWaitingForConfirmation` false)
            (set `self.whatWasChosen` 0))))
      (else
        (bind _asumg_options_2 (cast `/Game/GeneralBlueprints/Widget/Dialogue/UMG_options` (`WidgetComponent.GetUserWidgetObject` (`self.options_act`))))
        (bind _choose4 (`/Game/GeneralBlueprints/Widget/Dialogue/UMG_options.Choose4` _asumg_options_2))
        (`UserWidget.PlayAnimation` _asumg_options_2 _choose4 0.0 1 "Forward" _amination_speed false)
        (set `self.buffer_anim` _choose4)
        (bind _border_4 (`/Game/GeneralBlueprints/Widget/Dialogue/UMG_options.Border_4` _asumg_options_2))
        (`self.playing_content_animation` _border_4)
        (set `self.border_buffer` _border_4)
        (set `self.hasExpandedSpeechBubbleAndWaitingForConfirmation` true)
        (set `self.whatWasChosen` 4)
        (bind _asbp_game_inst_variable_storage_2 (cast `/Game/GeneralBlueprints/Main/GameInstance/BP_GameInst_VariableStorage` (`GameplayStatics.GetGameInstance`)))
        (if (`/Game/GeneralBlueprints/Main/GameInstance/BP_GameInst_VariableStorage.stressed_mode` _asbp_game_inst_variable_storage_2)
          (goto _label_5))))))

(fn `playing_content_animation`
  (params (border_type :type "Border Object Reference"))
  (bind _returnvalue (`ContentWidget.GetContent` border_type))
  (bind _amination_speed (`self.amination_speed`))
  (bind _returnvalue_2 (`WidgetComponent.GetUserWidgetObject` (`self.diop2`)))
  (bind _returnvalue_3 (`WidgetComponent.GetUserWidgetObject` (`self.diop3`)))
  (bind _returnvalue_4 (`WidgetComponent.GetUserWidgetObject` (`self.diop1`)))
  (bind _returnvalue_5 (`WidgetComponent.GetUserWidgetObject` (`self.diop`)))
  (if (== _returnvalue _returnvalue_5)
    (bind _asumg_dial_option_1 (cast `/Game/GeneralBlueprints/Widget/Dialogue/UMG_dialOption1` _returnvalue_5))
    (`UserWidget.PlayAnimation` _asumg_dial_option_1 (`/Game/GeneralBlueprints/Widget/Dialogue/UMG_dialOption1.Expand1` _asumg_dial_option_1) 0.0 1 "Forward" _amination_speed false)
    (elif (== _returnvalue _returnvalue_4)
      (bind _asumg_dial_option_2 (cast `/Game/GeneralBlueprints/Widget/Dialogue/UMG_dialOption2` _returnvalue_4))
      (`UserWidget.PlayAnimation` _asumg_dial_option_2 (`/Game/GeneralBlueprints/Widget/Dialogue/UMG_dialOption2.Expand2` _asumg_dial_option_2) 0.0 1 "Forward" _amination_speed false)
      (elif (== _returnvalue _returnvalue_2)
        (bind _asumg_dial_option_3 (cast `/Game/GeneralBlueprints/Widget/Dialogue/UMG_dialOption3` _returnvalue_2))
        (`UserWidget.PlayAnimation` _asumg_dial_option_3 (`/Game/GeneralBlueprints/Widget/Dialogue/UMG_dialOption3.Expand3` _asumg_dial_option_3) 0.0 1 "Forward" _amination_speed false)
        (elif (== _returnvalue _returnvalue_3)
          (bind _asumg_dial_option_special (cast `/Game/GeneralBlueprints/Widget/Dialogue/UMG_dialOptionSpecial` _returnvalue_3))
          (`UserWidget.PlayAnimation` _asumg_dial_option_special (`/Game/GeneralBlueprints/Widget/Dialogue/UMG_dialOptionSpecial.ExpandSpecial` _asumg_dial_option_special) 0.0 1 "Forward" _amination_speed false)
          (else
            (`KismetSystemLibrary.PrintString` "someone forgot to add an exeption")))))))

(fn `reversing_content_animation`
  (params (buffer_border :type "Border Object Reference"))
  (bind _returnvalue (`ContentWidget.GetContent` buffer_border))
  (bind _amination_speed (`self.amination_speed`))
  (bind _returnvalue_2 (`WidgetComponent.GetUserWidgetObject` (`self.diop2`)))
  (bind _returnvalue_3 (`WidgetComponent.GetUserWidgetObject` (`self.diop3`)))
  (bind _returnvalue_4 (`WidgetComponent.GetUserWidgetObject` (`self.diop1`)))
  (bind _returnvalue_5 (`WidgetComponent.GetUserWidgetObject` (`self.diop`)))
  (if (== _returnvalue _returnvalue_5)
    (bind _asumg_dial_option_1 (cast `/Game/GeneralBlueprints/Widget/Dialogue/UMG_dialOption1` _returnvalue_5))
    (`UserWidget.PlayAnimation` _asumg_dial_option_1 (`/Game/GeneralBlueprints/Widget/Dialogue/UMG_dialOption1.Expand1` _asumg_dial_option_1) 0.0 1 "Reverse" _amination_speed false)
    (elif (== _returnvalue _returnvalue_4)
      (bind _asumg_dial_option_2 (cast `/Game/GeneralBlueprints/Widget/Dialogue/UMG_dialOption2` _returnvalue_4))
      (`UserWidget.PlayAnimation` _asumg_dial_option_2 (`/Game/GeneralBlueprints/Widget/Dialogue/UMG_dialOption2.Expand2` _asumg_dial_option_2) 0.0 1 "Reverse" _amination_speed false)
      (elif (== _returnvalue _returnvalue_2)
        (bind _asumg_dial_option_3 (cast `/Game/GeneralBlueprints/Widget/Dialogue/UMG_dialOption3` _returnvalue_2))
        (`UserWidget.PlayAnimation` _asumg_dial_option_3 (`/Game/GeneralBlueprints/Widget/Dialogue/UMG_dialOption3.Expand3` _asumg_dial_option_3) 0.0 1 "Reverse" _amination_speed false)
        (elif (== _returnvalue _returnvalue_3)
          (bind _asumg_dial_option_special (cast `/Game/GeneralBlueprints/Widget/Dialogue/UMG_dialOptionSpecial` _returnvalue_3))
          (`UserWidget.PlayAnimation` _asumg_dial_option_special (`/Game/GeneralBlueprints/Widget/Dialogue/UMG_dialOptionSpecial.ExpandSpecial` _asumg_dial_option_special) 0.0 1 "Reverse" _amination_speed false)
          (else
            (`KismetSystemLibrary.PrintString` "someone still hasn't added an exeption")))))))

(fn `Switch_DialogInput`
  (params (Enable :type Boolean))
  (`/Game/GeneralBlueprints/Main/FunctionLibrary/BFL_ControlInput.BFL_Set_ActorActionInput` self Enable)
  (`/Game/GeneralBlueprints/Main/FunctionLibrary/BFL_ControlInput.BFL_Set_PlayerCharacterActionInput` (not Enable)))

(fn `UserConstructionScript`)

(fn `validating_options`
  (params (border_type :type "Border Object Reference"))
  (bind _returnvalue (`ContentWidget.GetContent` border_type))
  (set `self.usedDiop` (or (== _returnvalue (`WidgetComponent.GetUserWidgetObject` (`self.diop`))) (`self.usedDiop`)))
  (set `self.usedDiop_1` (or (== _returnvalue (`WidgetComponent.GetUserWidgetObject` (`self.diop1`))) (`self.usedDiop_1`)))
  (set `self.usedDiop_2` (or (== _returnvalue (`WidgetComponent.GetUserWidgetObject` (`self.diop2`))) (`self.usedDiop_2`)))
  (set `self.usedDiop_3` (or (== _returnvalue (`WidgetComponent.GetUserWidgetObject` (`self.diop3`))) (`self.usedDiop_3`))))