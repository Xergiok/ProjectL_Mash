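; BP_toggle_stressed_mode is a level actor that switches the game's stressed mode on and off.
; Its MainAction event flips the StressedMode flag on BP_GameInst_VariableStorage, the game instance that holds the state.
; The actor's PointLight then turns red when stressed mode is on and white when it is off.
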(event `/Game/GeneralBlueprints/Main/Interfaces/BPI_Interaction.Main_Action`
  (bind _pointlight (`self.PointLight`))
  (bind _asbp_game_inst_variable_storage (cast `/Game/GeneralBlueprints/Main/GameInstance/BP_GameInst_VariableStorage` (`GameplayStatics.GetGameInstance`)))
  (bind _output_get (set `/Game/GeneralBlueprints/Main/GameInstance/BP_GameInst_VariableStorage.stressed_mode` (not (`/Game/GeneralBlueprints/Main/GameInstance/BP_GameInst_VariableStorage.stressed_mode` _asbp_game_inst_variable_storage)) _asbp_game_inst_variable_storage))
  (if _output_get
    (`LightComponent.SetLightColor` _pointlight (make `LinearColor` 1.0 0.0 0.0 1.0) true)
    (else
      (`LightComponent.SetLightColor` _pointlight (make `LinearColor` 1.0 1.0 1.0 1.0) true))))

(fn `UserConstructionScript`)