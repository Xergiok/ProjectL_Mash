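; BP_MasterItem is an item actor, evidently a base class, that can sit in the scene or be attached.
; On construction it fills ItemSignature from DT_ItemsTable, using its own class display name as the row key, and resets mesh scale.
; SetCollisionProfile toggles physics and swaps between attached and scene collision profiles.
; An interface function exposes IconVolume and InfoIconMode as the anchor and mode for an info icon.
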(fn `Get_Anchor_BPIF`
  (returns (Mode :type "/Game/DarkTaleDemo/Core/Main/Components/Player/Interaction/EInfoIconMode Enum") (Anchor :type "SphereComponent Object Reference"))
  (bind _icon_volume (`self.Icon_Volume`)
    (:`then`
      (return (`self.InfoIcon_Mode`) _icon_volume))
    (:`else`)))

(fn `Set_CollisionProfile`
  (params (Attached :type Boolean))
  (`PrimitiveComponent.SetSimulatePhysics` (`self.StaticMesh`) (not Attached))
  (`PrimitiveComponent.SetCollisionProfileName` (`self.StaticMesh`) (select `bool` (`local.Attached`) :`false` (`self.Scene_CollisionProfile`) :`true` (`self.Attached_CollisionProfile`)) true))

(fn `UserConstructionScript`
  (bind _returnvalue (`|GetDataTableRow` "/Game/DarkTaleDemo/Core/Miscellaneous/Inventory/InventoryStructure/DT_ItemsTable.DT_ItemsTable" (`KismetStringLibrary.Conv_StringToName` (`KismetSystemLibrary.GetClassDisplayName` (`GameplayStatics.GetObjectClass` self))))
    (:`then`
      (set `self.ItemSignature` _returnvalue)
      (`SceneComponent.SetRelativeScale3D` (`self.StaticMesh`) (`KismetMathLibrary.MakeVector` 1.0 1.0 1.0)))))