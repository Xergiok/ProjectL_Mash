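; BP_Item_Pickable is an item actor that players can pick up, throw or store in their inventory.
; PickUp attaches it to a socket on the player's skeletal mesh; Throw detaches it and applies an impulse along the player controller's forward vector, each switching the collision profile.
; AddtoInventory sends an inventory slot to the player through an interface, then clears the hold and destroys the actor if accepted.
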(event `/Game/DarkTaleDemo/Core/Main/Interfaces/Items/BPI_Pickable.Add To Inventory`
  (params (Player :type "Actor Object Reference"))
  (bind (_itemsignature_name _itemsignature_description _itemsignature_isstackable _itemsignature_isconsumable _itemsignature_maxstacksize _itemsignature_thumbnail _itemsignature_slotpriority _itemsignature_class) (break `/Game/DarkTaleDemo/Core/Miscellaneous/Inventory/InventoryStructure/SItemSignature` (`self.ItemSignature`)))
  ;[1 1 1] Add to iventory
  (bind _success (message `/Game/DarkTaleDemo/Core/Main/Interfaces/Components/BPI_InventoryOwner.Add_Item_To_Inventory_BPIF` Player (make `/Game/DarkTaleDemo/Core/Miscellaneous/Inventory/InventoryStructure/SInventorySlot` (`self.ItemSignature`) (`self.Quanity`))))
  (if _success
    (message `/Game/DarkTaleDemo/Core/Main/Interfaces/Components/BPI_PlayerInteraction.Hold_Switch_BPIF` Player self false)
    (`self.K2_DestroyActor`)
    (`KismetSystemLibrary.PrintString` (`KismetStringLibrary.Concat_StrStr` "Added " (`KismetSystemLibrary.GetClassDisplayName` _itemsignature_class)))))

(event `self.ReceiveBeginPlay`
  (`self.Set_CollisionProfile` false))

(event `/Game/DarkTaleDemo/Core/Main/Interfaces/Items/BPI_Pickable.Throw`
  (`SceneComponent.K2_DetachFromComponent` (`self.RootComponent`) "KeepWorld" "KeepWorld" "KeepWorld" false)
  (set `self.Attached` false)
  (`self.Set_CollisionProfile` false)
  (`PrimitiveComponent.AddImpulse` (`self.StaticMesh`) (* (`self.GetActorForwardVector` (`GameplayStatics.GetPlayerController` 0)) 100.0) "None" true))

(event `/Game/DarkTaleDemo/Core/Main/Interfaces/Items/BPI_Pickable.Pick Up`
  (params (Player :type "Actor Object Reference") (SocketName :type Name))
  (`self.Set_CollisionProfile` true)
  (bind _returnvalue (`SceneComponent.K2_AttachToComponent` (`self.RootComponent`) (`self.GetComponentByClass` Player "/Script/Engine.SkeletalMeshComponent") SocketName "SnapToTarget" "SnapToTarget" "KeepWorld" true))
  (set `self.Attached` _returnvalue))

(fn `UserConstructionScript`
  (`parent.UserConstructionScript`))