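; BP_Item_DoorBasic is an interactable door item that can be locked behind a required key.
; On interact, a locked door compares the class of the item in one of the character's interaction slots to RequiredKey, staying unlocked after a match.
; An unlocked door toggles Opened and snaps its root yaw 90 degrees either way, with debug prints.
; Focus adds a concentration camera modifier to the instigator's camera; losing focus disables it.
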(event `/Game/DarkTaleDemo/Core/Main/Interfaces/Items/BPI_Interactable.Interact`
  (params (Instigator :type "Actor Object Reference"))
  (bind _rootcomponent (`self.RootComponent`))
  (bind (_isactive _interactioncomponent) (`/Game/DarkTaleDemo/Core/Main/FunctionLibrary/BPFL_Interaction_Use.Get_Character_InteractionComponent_BPFL` (cast `Character` Instigator :!pure true)))
  (bind (_returnvalue_roll _returnvalue_pitch _returnvalue_yaw) (`KismetMathLibrary.BreakRotator` (`SceneComponent.K2_GetComponentRotation` _rootcomponent)))
  (bind (_exist _item) (`/Game/DarkTaleDemo/Core/Main/Components/Player/Interaction/BP_CharInteraction_AC.Get_SlotItem` _interactioncomponent "NewEnumerator1"))
  (if (`self.Locked`)
    (if _isactive
      (if _exist
        (bind _unlocked (`self.Unlock` (`GameplayStatics.GetObjectClass` _item)))
        (if _unlocked
          (`KismetSystemLibrary.PrintString` "door unlocked")
          (if (`self.Opened`) :!label _label
            (`KismetSystemLibrary.PrintString` "door closed")
            (else
              (`KismetSystemLibrary.PrintString` "door opened")))
          (bind _output_get (set `self.Opened` (not (`self.Opened`))))
          (`SceneComponent.K2_SetWorldRotation` _rootcomponent (`KismetMathLibrary.MakeRotator` _returnvalue_roll _returnvalue_pitch (`KismetMathLibrary.SelectFloat` (+ _returnvalue_yaw 90.0) (+ _returnvalue_yaw -90.0) _output_get)) false false)
          (else
            (`KismetSystemLibrary.PrintString` "wrong key")))
        (else
          (`KismetSystemLibrary.PrintString` "Door is locked, you need a key"))))
    (else
      (goto _label))))

(event `/Game/DarkTaleDemo/Core/Main/Interfaces/Items/BPI_Focusable.FocusedInto_BPIF`
  (params (Instigator :type "Actor Object Reference"))
  (`/Engine/EditorBlueprintResources/StandardMacros.IsValid` Instigator
    (:`Is Valid`
      (bind _camera_manager (`/Game/DarkTaleDemo/Core/Main/MacroLibrary/BPML_MasterItem.Get_CameraManager_BPML` (`self.GetInstigatorController` Instigator)))
      (bind _returnvalue (`PlayerCameraManager.AddNewCameraModifier` _camera_manager "/Game/DarkTaleDemo/Core/Miscellaneous/CameraModifiers/Items/CMD_Concentration.CMD_Concentration_C")))))

(event `/Game/DarkTaleDemo/Core/Main/Interfaces/Items/BPI_Focusable.FucusedOut_BPIF`
  (params (Instigator :type "Actor Object Reference"))
  (`/Engine/EditorBlueprintResources/StandardMacros.IsValid` Instigator
    (:`Is Valid`
      (`CameraModifier.DisableModifier` (stale `/Game/DarkTaleDemo/Core/Main/Interfaces/Items/BPI_Focusable.FocusedInto_BPIF` _returnvalue) false))))

(event `CustomEvent_0`)

(fn `Unlock`
  (params (Key :type "Actor Class Reference"))
  (returns (Unlocked :type Boolean))
  (if (== Key (`self.Required Key`))
    (set `self.Locked` false)
    (return true)
    (else
      (return false))))

(fn `UserConstructionScript`
  (`parent.UserConstructionScript`))