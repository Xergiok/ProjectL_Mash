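; BP_Main_Bullet is a base-style weapon bullet actor that limits its lifetime on BeginPlay.
; Its Hit event is empty; the impact effect, physics impulse, conditional destroy and damage-interface call sit in disconnected nodes.
; That unwired damage path uses a bone-name hitbox helper to double head damage and spawns floating debug text.
; Its own damage-interface functions are stubs returning failure and zero amplitude.
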(event `self.ReceiveBeginPlay`
  (`self.SetLifeSpan` 30.0))

(event `self.ReceiveHit`
  (params (MyComp :type "PrimitiveComponent Object Reference") (Other :type "Actor Object Reference") (OtherComp :type "PrimitiveComponent Object Reference") (bSelfMoved :type Boolean) (HitLocation :type "Vector Structure") (HitNormal :type "Vector Structure") (NormalImpulse :type "Vector Structure") (Hit :type "HitResult Structure (by ref)")))

(fn `Debug_FloatDamageText`
  (params (SpawnTransform_Location :type "Vector Structure") (Value :type Text))
  (`|SpawnActorFromClass` "/Game/DarkTaleDemo/Core/Widget/debug/BP_FloatingText.BP_FloatingText_C" (`KismetMathLibrary.MakeTransform` SpawnTransform_Location) "Undefined" "OverrideRootScale" null Value null))

(fn `Process_AnyDamage_BPIF`
  (params (Scale :type "Float (double-precision)") (Reciever :type "Actor Object Reference") (Instigator :type "Controller Object Reference") (Causer :type "Actor Object Reference"))
  (returns (Successfully :type Boolean) (Amplitude :type "Float (double-precision)") (Form :type "/Game/DarkTaleDemo/Core/Main/Components/DamageSystem/EDamageForm Enum"))
  (return false 0.0 "NewEnumerator0"))

(fn `Process_PointDamage_BPIF`
  (params (Scale :type "Float (double-precision)") (Reciever :type "Actor Object Reference") (Instigator :type "Controller Object Reference") (Causer :type "Actor Object Reference") (Location :type "Vector Structure") (Direction :type "Vector Structure") (Component :type "PrimitiveComponent Object Reference") (Bone :type Name))
  (returns (Successfully :type Boolean) (Amplitude :type "Float (double-precision)") (Form :type "/Game/DarkTaleDemo/Core/Main/Components/DamageSystem/EDamageForm Enum"))
  (return false 0.0 "NewEnumerator0"))

(fn `Process_RadialDamage_BPIF`
  (params (Scale :type "Float (double-precision)") (Reciever :type "Actor Object Reference") (Instigator :type "Controller Object Reference") (Causer :type "Actor Object Reference") (Origin :type "Vector Structure") (HitInfo :type "HitResult Structure"))
  (returns (Successfully :type Boolean) (Amplitude :type "Float (double-precision)") (Form :type "/Game/DarkTaleDemo/Core/Main/Components/DamageSystem/EDamageForm Enum"))
  (return false 0.0 "NewEnumerator0"))

(fn `Select_Hitbox`
  (params (Bone_Name :type Name))
  (returns (ReturnValue :type "/Game/DarkTaleDemo/Core/Miscellaneous/Bones/Hitbox/EHitboxNPC Enum"))
  (return (select `bool` (or (== Bone_Name "neck_01") (== Bone_Name "head")) :`false` "NewEnumerator0" :`true` "NewEnumerator1" :!type "/Game/DarkTaleDemo/Core/Miscellaneous/Bones/Hitbox/EHitboxNPC Enum")))

(fn `UserConstructionScript`)