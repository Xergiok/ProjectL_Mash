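; Revolver weapon Blueprint that extends a parent weapon with part-by-part reloading and a hand-rotated cylinder ("Baraban").
; Partial reload plays opening and idle sequences, then enables gated mouse-wheel input that drives cylinder rotation through a timeline.
; Inserting a bullet plays its own animation, briefly locking rotation, and an ordered bullet list drives shell/bullet mesh swaps.
; Random shot animations and the reload-end sequence are present but unconnected.
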(event `self.ReceiveBeginPlay`
  ;[1 1 1] Here we do store bullets in the array,
  ; for revolver logic.
  (`parent.ReceiveBeginPlay`)
  (set `self.Bullet_List` (`|MakeArray` (`self.4`) (`self.5`) (`self.1`) (`self.2`) (`self.0`) (`self.3`)))
  (set `self.Use_Part_Reload` true)
  (set `self.UseCustomFireAnim` false))

(event `self.Refresh_PhysModel`
  ;[1 1 1] Here we do store bullets in the array,
  ; for revolver logic.
  (for (_array_element _array_index) (`self.Bullet_List`)
    (if (>= _array_index 0)
      (`StaticMeshComponent.SetStaticMesh` _array_element "/Game/Temp/PackAnimatedRevolver/staticmeshes/static_shell.static_shell")
      (else
        (`StaticMeshComponent.SetStaticMesh` _array_element "/Game/Temp/PackAnimatedRevolver/staticmeshes/static_bullet.static_bullet") ; if we have enough bullets in barrel\nwe should show the bullet mesh.
      ))))

(event `self.Custom_FireAnim`)

(event `self.Part_Reload`
  (`self.Play Sequence` true false null null 1.0 1 "None" "/Game/DarkTaleDemo/Characters/TestChar/Anims/States/Weapon/Pistol/AS_TestChar_Revolver_Reload_Begin.AS_TestChar_Revolver_Reload_Begin" "/Game/Temp/PackAnimatedRevolver/anims/revolver/sequences/w_revolver_reload_start.w_revolver_reload_start")
  (`KismetSystemLibrary.Delay` 2.53)
  (`self.Play Sequence` true false null null 0.0 1 "None" "/Game/Temp/PackAnimatedRevolver/anims/revolver/sequences/AA_W_Revolver_Reload_Idle.AA_W_Revolver_Reload_Idle")
  (set `self.CanRotateBaraban` true)
  (set `self.AdditiveBarRot` 0.0))

(event `InputAxis|MouseWheelControl`
  (params (AxisValue :type "Float (single-precision)"))
  (if (and (!= AxisValue 0.0) (`self.CanRotateBaraban`) (`self.Reloading?`))
    (`/Engine/EditorBlueprintResources/StandardMacros.Gate` false :!label _label
      (:`Exit`
        (`|ExecutionSequence`
          (:`then_0`
            (bind _output_get (set `self.MouseWheel_Axis` (`KismetMathLibrary.FClamp` AxisValue -1.0)))
            (set `self.AdditiveBarRot` (+ _output_get (`self.AdditiveBarRot`)))
            (`TimelineComponent.PlayFromStart` (`self.BarabanRot_Timeline`))
            (goto _label :!via `Close`))
          (:`then_1`
            (`KismetSystemLibrary.Delay` 0.2)
            (goto _label :!via `Open`)))))))

(event `self.Put_One_Bullet`
  (`/Engine/EditorBlueprintResources/StandardMacros.Gate` false :!label _label_2
    (:`Exit`
      (`/Game/DarkTaleDemo/Core/Main/MacroLibrary/BPML_FireWeapon.CheckAmmo_BPML`
        (:`Magazine full`)
        (:`Has some ammo in the magazine`
          _)
        (:`Empty magazine (has ammo)`
          _))
      (`|ExecutionSequence`
        (:`then_0`
          (set `self.CanRotateBaraban` false)
          (`self.Play Sequence` true false null null 1.0 1 "None" "/Game/DarkTaleDemo/Characters/TestChar/Anims/States/Weapon/Pistol/AS_TestChar_Revolver_Reload_a1b.AS_TestChar_Revolver_Reload_a1b" "/Game/Temp/PackAnimatedRevolver/anims/revolver/sequences/w_revolver_reload_a1b.w_revolver_reload_a1b")
          (goto _label_2 :!via `Close`))
        (:`then_1`
          (`KismetSystemLibrary.Delay` 1.2)
          (set `self.CanRotateBaraban` true)
          (`/Game/DarkTaleDemo/Core/Main/MacroLibrary/BPML_FireWeapon.CheckAmmo_BPML`))))))

(fn `UserConstructionScript`
  (set `self.MuzzleSocket` "SKT_Muzzle")
  (`parent.UserConstructionScript`))