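; BP_Item_FlashlightBasic is a flashlight item whose spotlight toggles on and off when used.
; The Use event flips the LightOn flag and calls ChangeLight, which sets the SpotLight intensity to the Intensity variable or zero.
; BeginPlay runs the parent logic, then applies the initial light state.
; The construction script runs the parent's version, then shrinks the static mesh with a uniform relative scale.
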(event `self.ReceiveBeginPlay`
  (`parent.ReceiveBeginPlay`)
  (`self.Change Light`))

(event `Change Light`
  (bind _spotlight (`self.SpotLight`))
  (if (`self.Light On`)
    (`LightComponent.SetIntensity` _spotlight (`self.Intensity`))
    (else
      (`LightComponent.SetIntensity` _spotlight 0.0))))

(event `/Game/DarkTaleDemo/Core/Main/Interfaces/Items/BPI_Usable.Use`
  (params (Insigator :type "Actor Object Reference"))
  (if (`self.Light On`)
    (set `self.Light On` false)
    (else
      (set `self.Light On` true)))
  (`self.Change Light`))

(fn `UserConstructionScript`
  (`parent.UserConstructionScript`)
  (`SceneComponent.SetRelativeScale3D` (`self.StaticMesh`) (`KismetMathLibrary.MakeVector` 0.2 0.2 0.2)))