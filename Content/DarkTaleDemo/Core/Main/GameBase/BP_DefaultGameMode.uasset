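; Default game mode for the DarkTale demo, acting as a holder of player references and input-mode settings.
; On BeginPlay it casts and caches the player character (BP_HumanChar), its PC_Default controller and its ABP_General_HumanCharacter anim instance.
; A separate UpdatePlayerSettings function, not called within this Blueprint, copies the crouch, walk and sprint hold settings from the input settings struct onto the cached character.
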(event `self.ReceiveBeginPlay`
  (`self.Add_Maintain_References`))

(fn `Add_Maintain_References`
  (`|ExecutionSequence`
    (:`then_0`
      (bind _asbp_human_char (cast `/Game/DarkTaleDemo/Core/Main/Characters/Player/BP_HumanChar` (`GameplayStatics.GetPlayerCharacter` 0)))
      (set `self.PlayerCharacter` _asbp_human_char))
    (:`then_1`
      (bind _aspc_default (cast `/Game/DarkTaleDemo/Core/Main/Control/PlayerControllers/PC_Default` (`GameplayStatics.GetPlayerController` 0)))
      (set `self.PlayerController` _aspc_default))
    (:`then_2`
      (bind _playercharacter (`self.PlayerCharacter`)
        (:`then`
          (bind _asabp_general_human_character (cast `/Game/DarkTaleDemo/Characters/TestChar/Anims/AnimBP/ABP_General_HumanCharacter` (`SkeletalMeshComponent.GetAnimInstance` (`self.GetComponentByClass` _playercharacter "/Script/Engine.SkeletalMeshComponent"))))
          (set `self.Player Animation` _asabp_general_human_character))
        (:`else`)))))

(fn `Update_PlayerSettings`
  (`|ExecutionSequence`
    (:`then_0`
      (set `/Game/DarkTaleDemo/Core/Main/Characters/Player/BP_HumanChar.crouch_settings_hold` (`.InputSettings_Crouch_Hold_3_59ED9E7F4470D4E8892935B6FA4A0FC3` (break `/Game/DarkTaleDemo/Core/Miscellaneous/KeySettings/SKeypressSettings` (`self.ST_Input_Settings`))) (`self.PlayerCharacter`)))
    (:`then_1`
      (set `/Game/DarkTaleDemo/Core/Main/Characters/Player/BP_HumanChar.walk_settings_hold` (`.InputSettings_Walk_Hold_4_C5E9AA7142969297911FE49B5829AC61` (break `/Game/DarkTaleDemo/Core/Miscellaneous/KeySettings/SKeypressSettings` (`self.ST_Input_Settings`))) (`self.PlayerCharacter`)))
    (:`then_2`
      (set `/Game/DarkTaleDemo/Core/Main/Characters/Player/BP_HumanChar.sprint_settings_hold` (`.InputSettings_Sprint_Hold_5_26A9FF3E489CB4926C0588AF4987C67E` (break `/Game/DarkTaleDemo/Core/Miscellaneous/KeySettings/SKeypressSettings` (`self.ST_Input_Settings`))) (`self.PlayerCharacter`)))))

(fn `UserConstructionScript`)