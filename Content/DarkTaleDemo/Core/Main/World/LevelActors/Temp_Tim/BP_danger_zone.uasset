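; BP_danger_zone is a level trigger volume that marks when the player is inside a dangerous area.
; Box begin and end overlap events set the IsInDangerZone flag on the player controller to true and false.
; A helper function filters overlapping actors to player-controlled pawns and returns their PC_Default controller.
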(event `self.Box.OnComponentBeginOverlap`
  (params (OverlappedComponent :type "PrimitiveComponent Object Reference") (OtherActor :type "Actor Object Reference") (OtherComp :type "PrimitiveComponent Object Reference") (OtherBodyIndex :type Integer) (bFromSweep :type Boolean) (SweepResult :type "HitResult Structure (by ref)"))
  (bind _asbp_default_player_controller (`self.Check_PlayerController` OtherActor))
  (set `/Game/DarkTaleDemo/Core/Main/Control/PlayerControllers/PC_Default.is_in_danger_zone` true _asbp_default_player_controller))

(event `self.Box.OnComponentEndOverlap`
  (params (OverlappedComponent :type "PrimitiveComponent Object Reference") (OtherActor :type "Actor Object Reference") (OtherComp :type "PrimitiveComponent Object Reference") (OtherBodyIndex :type Integer))
  (bind _asbp_default_player_controller (`self.Check_PlayerController` OtherActor))
  (set `/Game/DarkTaleDemo/Core/Main/Control/PlayerControllers/PC_Default.is_in_danger_zone` false _asbp_default_player_controller))

(fn `UserConstructionScript`)