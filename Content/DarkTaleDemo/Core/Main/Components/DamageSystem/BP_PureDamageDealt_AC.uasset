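; BP_PureDamageDealt_AC is a damage-system actor component that deals pure damage to a given actor.
; ApplyPureDamageFC loops over damage types from a selection macro, calling ApplyDamage for each with the component owner as causer.
; A debug macro receives calculated and applied amounts.
; CalculateBaseDamage returns zero here, and the radial and point damage nodes in the event graph never run.
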(fn `Apply_PureDamageFC`
  (params (DamagedActor :type "Actor Object Reference") (EventInstigator :type "Controller Object Reference"))
  (bind _basedamage (`self.Calculate_BaseDamage`))
  (bind _array_element (`/Game/DarkTaleDemo/Core/Main/MacroLibrary/BPML_BaseDamageDealt_AComponent.DamageTypeSelection_BPML`)
    (:`LoopBody`
      (bind _returnvalue (`GameplayStatics.ApplyDamage` (`local.DamagedActor`) _basedamage (`local.EventInstigator`) (`self.GetOwner`) _array_element))
      (`/Game/DarkTaleDemo/Core/Main/MacroLibrary/BPML_BaseDamageDealt_AComponent.DamageDealtDebug_BPML` _basedamage _returnvalue _array_element))))

(fn `Calculate_BaseDamage`
  (returns (BaseDamage :type "Float (double-precision)"))
  (return 0.0))

(fn `Component_Initialization`
  (`parent.Component_Initialization`))