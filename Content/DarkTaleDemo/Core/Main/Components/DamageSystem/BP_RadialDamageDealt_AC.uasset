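; Actor component in the DarkTale demo damage system that deals radial damage with falloff around a given origin.
; ApplyRadialDamageFC loops through damage types from a selection macro, applying damage for each with the owner as causer, honoring ignored actors and a prevention channel.
; DamageRange supplies minimum and base damage, DamageRadius the inner and outer radii.
; Each application feeds a debug macro, which receives base damage as both calculated and applied values.
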(fn `Apply_RadialDamageFC`
  (params (InstigatedByController :type "Controller Object Reference") (Origin :type "Vector Structure (by ref)"))
  (bind _basedamage (`self.Calculate_BaseDamage`))
  (bind _damagerange_x (`KismetMathLibrary.BreakVector2D` (`self.DamageRange`)))
  (bind (_damageradius_x _damageradius_y) (`KismetMathLibrary.BreakVector2D` (`self.DamageRadius`)))
  (bind _array_element (`/Game/DarkTaleDemo/Core/Main/MacroLibrary/BPML_BaseDamageDealt_AComponent.DamageTypeSelection_BPML`)
    (:`LoopBody`
      (`GameplayStatics.ApplyRadialDamageWithFalloff` _basedamage _damagerange_x (`local.Origin`) _damageradius_x _damageradius_y (`self.DamageFalloff`) _array_element (`self.IgnoredActors`) (`self.GetOwner`) (`local.InstigatedByController`) (`self.DamagePreventionChannel`))
      (`/Game/DarkTaleDemo/Core/Main/MacroLibrary/BPML_BaseDamageDealt_AComponent.DamageDealtDebug_BPML` _basedamage _basedamage _array_element))))

(fn `Calculate_BaseDamage`
  (returns (BaseDamage :type "Float (double-precision)"))
  (bind (_damagerange_x _damagerange_y) (`KismetMathLibrary.BreakVector2D` (`self.DamageRange`)))
  (return _damagerange_y))