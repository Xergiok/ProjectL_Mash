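; BP_PointDamageDealt_AC is a damage-system component that deals point damage from its owning actor to a given target.
; It loops over damage types supplied by a selection macro, applying point damage for each with the passed hit direction, hit info and instigator.
; Base damage is always the Y value of DamageRange, with no randomization, and a debug macro receives the calculated and applied amounts per type.
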(fn `Apply_PointDamageFC`
  (params (DamagedActor :type "Actor Object Reference") (EventInstigator :type "Controller Object Reference") (HitFromDirection :type "Vector Structure (by ref)") (HitInfo :type "HitResult Structure (by ref)"))
  (bind _basedamage (`self.Calculate_BaseDamage`))
  (bind _array_element (`/Game/DarkTaleDemo/Core/Main/MacroLibrary/BPML_BaseDamageDealt_AComponent.DamageTypeSelection_BPML`)
    (:`LoopBody`
      (bind _returnvalue (`GameplayStatics.ApplyPointDamage` (`local.DamagedActor`) _basedamage (`local.HitFromDirection`) (`local.HitInfo`) (`local.EventInstigator`) (`self.GetOwner`) _array_element))
      (`/Game/DarkTaleDemo/Core/Main/MacroLibrary/BPML_BaseDamageDealt_AComponent.DamageDealtDebug_BPML` _basedamage _returnvalue _array_element))))

(fn `Calculate_BaseDamage`
  (returns (BaseDamage :type "Float (double-precision)"))
  (bind (_damagerange_x _damagerange_y) (`KismetMathLibrary.BreakVector2D` (`self.DamageRange`)))
  (return _damagerange_y))