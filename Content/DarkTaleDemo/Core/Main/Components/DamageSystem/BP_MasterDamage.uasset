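; BP_MasterDamage is a damage-processing Blueprint in the DamageSystem, apparently the base that specific damage kinds build on.
; Its any-damage handler reports success and returns Scale times DamageMultiplyer, clamped to 0–1, as the amplitude.
; Point and radial handlers are defaults that report failure with zero amplitude, and all three return the same damage form.
; A getter exposes the multiplier.
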(fn `Process_AnyDamage_BPIF`
  (params (Scale :type "Float (double-precision)") (Reciever :type "Actor Object Reference") (Instigator :type "Controller Object Reference") (Causer :type "Actor Object Reference"))
  (returns (Successfully :type Boolean) (Amplitude :type "Float (double-precision)") (Form :type "/Game/DarkTaleDemo/Core/Main/Components/DamageSystem/EDamageForm Enum"))
  (return true (`KismetMathLibrary.FClamp` (* Scale (`self.Damage_Multiplyer`))) "NewEnumerator0"))

(fn `Process_PointDamage_BPIF`
  (params (Scale :type "Float (double-precision)") (Reciever :type "Actor Object Reference") (Instigator :type "Controller Object Reference") (Causer :type "Actor Object Reference") (Location :type "Vector Structure") (Direction :type "Vector Structure") (Component :type "PrimitiveComponent Object Reference") (Bone :type Name))
  (returns (Successfully :type Boolean) (Amplitude :type "Float (double-precision)") (Form :type "/Game/DarkTaleDemo/Core/Main/Components/DamageSystem/EDamageForm Enum"))
  (return false 0.0 "NewEnumerator0"))

(fn `Process_RadialDamage_BPIF`
  (params (Scale :type "Float (double-precision)") (Reciever :type "Actor Object Reference") (Instigator :type "Controller Object Reference") (Causer :type "Actor Object Reference") (Origin :type "Vector Structure") (HitInfo :type "HitResult Structure"))
  (returns (Successfully :type Boolean) (Amplitude :type "Float (double-precision)") (Form :type "/Game/DarkTaleDemo/Core/Main/Components/DamageSystem/EDamageForm Enum"))
  (return false 0.0 "NewEnumerator0"))

(fn `Select_DamageMultiplyer`
  (returns (Damage_Multiplyer :type "Float (double-precision)"))
  (return (`self.Damage_Multiplyer`)))