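; Base damage reaction component that tracks a clamped damage/heal scale for its owning actor and raises damaged, healed, level-change, full and null events.
; It binds enabled any, point and radial damage events, filters allowed damage types, and delegates amount and Loss/Heal form to each type through an interface.
; The scale selects a level from threshold-sorted map keys, with edge values forcing full or null, and debug prints report changes.
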(event `self.ReceiveBeginPlay`
  (`self.Component_Initialization`))

(event `Apply_AnyDamage`
  (params (DamagedActor :type "Actor Object Reference") (Damage :type "Float (double-precision)") (DamageType :type "DamageType Object Reference") (InstigatedBy :type "Controller Object Reference") (DamageCauser :type "Actor Object Reference"))
  (`self.DamageType_Filter` DamageType
    (:`T`
      (bind (_successfully _amplitude _form) (message `/Game/DarkTaleDemo/Core/Main/Interfaces/Components/BPI_DamageReaction.Process_AnyDamage_BPIF` DamageType Damage DamagedActor InstigatedBy DamageCauser))
      (if _successfully
        (`self.Calculate_Damage` _amplitude _form)))))

(event `Apply_PointDamage`
  (params (DamagedActor :type "Actor Object Reference") (Damage :type "Float (double-precision)") (InstigatedBy :type "Controller Object Reference") (HitLocation :type "Vector Structure") (FHitComponent :type "PrimitiveComponent Object Reference") (BoneName :type Name) (ShotFromDirection :type "Vector Structure") (DamageType :type "DamageType Object Reference") (DamageCauser :type "Actor Object Reference"))
  (`self.DamageType_Filter` DamageType
    (:`T`
      (bind (_successfully _amplitude _form) (message `/Game/DarkTaleDemo/Core/Main/Interfaces/Components/BPI_DamageReaction.Process_PointDamage_BPIF` DamageType Damage DamagedActor InstigatedBy DamageCauser HitLocation ShotFromDirection FHitComponent BoneName))
      (if _successfully
        (`self.Calculate_Damage` _amplitude _form)))))

(event `Apply_RadialDamage`
  (params (DamagedActor :type "Actor Object Reference") (Damage :type "Float (double-precision)") (DamageType :type "DamageType Object Reference") (Origin :type "Vector Structure") (HitInfo :type "HitResult Structure") (InstigatedBy :type "Controller Object Reference") (DamageCauser :type "Actor Object Reference"))
  (`self.DamageType_Filter` DamageType
    (:`T`
      (bind (_successfully _amplitude _form) (message `/Game/DarkTaleDemo/Core/Main/Interfaces/Components/BPI_DamageReaction.Process_RadialDamage_BPIF` DamageType Damage DamagedActor InstigatedBy DamageCauser Origin HitInfo))
      (if _successfully
        (`self.Calculate_Damage` _amplitude _form)))))

(fn `Calculate_Damage`
  (params (Decrement :type "Float (double-precision)") (Form :type "/Game/DarkTaleDemo/Core/Main/Components/DamageSystem/EDamageForm Enum" :default "NewEnumerator0"))
  (`self.Value_Check` Decrement)
  (`self.Heal_Check` Form)
  (bind _result (`self.Damage_Deduction` Decrement Form))
  (`self.Value_Check` _result)
  (`self.Edge_Check ` (`self.Scale_value`)
    (:`Continue`
      (`self.Set_Damage_value`)
      (`self.Search_Level`))))

(fn `Component_Initialization`
  (`parent.Component_Initialization`)
  (`|ExecutionSequence`
    (:`then_0`
      (`|ExecutionSequence`
        (:`then_0`
          (if (`self.Sensible_to_AnyDamage`)
            (add `Actor.OnTakeAnyDamage` (`self.GetOwner`) (`|CreateDelegate` :!event `Apply_AnyDamage`))))
        (:`then_1`
          (if (`self.Sensible_to_PointDamage`)
            (add `Actor.OnTakePointDamage` (`self.GetOwner`) (`|CreateDelegate` :!event `Apply_PointDamage`))))
        (:`then_2`
          (if (`self.Sensible_to_RadialDamage`)
            (add `Actor.OnTakeRadialDamage` (`self.GetOwner`) (`|CreateDelegate` :!event `Apply_RadialDamage`))))))
    (:`then_1`
      (`self.Sort_List`)
      (`self.Set_Damage_value`)
      (`self.Search_Level`))))

(fn `Damage_Deduction`
  (params (Decrement :type "Float (double-precision)") (Form :type "/Game/DarkTaleDemo/Core/Main/Components/DamageSystem/EDamageForm Enum" :default "NewEnumerator0"))
  (returns (Result :type "Float (double-precision)"))
  (`|ExecutionSequence`
    (:`then_0`
      (set `self.Scale_value` (`KismetMathLibrary.FClamp` (- (`self.Scale_value`) (select `/Game/DarkTaleDemo/Core/Main/Components/DamageSystem/EDamageForm` Form :`NewEnumerator0` Decrement :`NewEnumerator1` (* -1 Decrement))) 0.0 (`self.Max_Scale_value`))))
    (:`then_1`
      (switch `/Game/DarkTaleDemo/Core/Main/Components/DamageSystem/EDamageForm` (`local.Form`)
        (:`NewEnumerator0`
          (`self.ED_Damaged`))
        (:`NewEnumerator1`
          (`self.ED_Healed`))))
    (:`then_2`
      (`|ExecutionSequence`
        (:`then_0`
          (`KismetSystemLibrary.PrintString` (`KismetStringLibrary.Concat_StrStr` "Damaged actor: " (`KismetSystemLibrary.GetDisplayName` (`self.GetOwner`)) " --- " (`|GetEnumeratorNameAsString` Form) " damage applied: " (`KismetStringLibrary.Conv_DoubleToString` Decrement)) true true (struct :`R` 0.633645 :`G` 1.0 :`A` 1.0) 5.0))
        (:`then_1`
          (return (`self.Scale_value`)))))))

(fn `IF_Beth`)

(fn `IF_Full`
  (`self.ED_Full`))

(fn `IF_Null`
  (`self.ED_Null`))

(fn `Search_Level`
  (locals (LastIndex :type Integer))
  (bind (_value _returnvalue) (`BlueprintMapLibrary.Map_Find` (`self.Damage_Levels`) (`|GetArrayItem` (`self.Float_Keys`) (- (`local.LastIndex`) 1))))
  (for (_array_element _array_index) (`self.Float_Keys`)
    (set `local.LastIndex` _array_index)
    (if (not (>= (`self.Scale_value`) _array_element))
      (break)))
  (if _returnvalue
    (`self.Set_NewDamageLevel` _value)))

(fn `Select_Value`
  (returns (ReturnValue :type "Float (double-precision)"))
  (return (`|EaseFunction` "EaseInOut" (`self.Scale_value`) 0.0 (`self.Max_Scale_value`))))

(fn `Set_Damage_value`
  (set `self.Damage_value` (`KismetMathLibrary.SelectFloat` (`self.Scale_value`) (`self.Select_Value`) (`self.Linear_Falloff`))))

(fn `Set_NewDamageLevel`
  (params (New_Level :type "/Game/DarkTaleDemo/Core/Main/Components/DamageSystem/EDefaultDamageLevels Enum" :default "NewEnumerator14"))
  (bind _out_a (`/Game/DarkTaleDemo/Core/Main/MacroLibrary/BPML_Object.DoOnly_IfDifferent(Byte)_BPML` New_Level (`self.Current_Level`))
    (:`true`
      (bind _output_get (set `self.Current_Level` _out_a))
      (`|ExecutionSequence`
        (:`then_0`
          (`self.ED_LevelChanged`)
          (`|ExecutionSequence`
            (:`then_0`
              (`KismetSystemLibrary.PrintString` (`KismetStringLibrary.Concat_StrStr` "Damaged actor: " (`KismetSystemLibrary.GetDisplayName` (`self.GetOwner`)) " new lvl: " (`KismetStringLibrary.Conv_DoubleToString` (`self.Scale_value`)) " - " (`|GetEnumeratorNameAsString` (`self.Current_Level`))) true true (struct :`R` 0.633645 :`G` 1.0 :`A` 1.0) 5.0))))
        (:`then_1`
          (`self.Switch_DefaultLevels` _output_get
            (:`Full`
              (`self.IF_Full`))
            (:`Null`
              (`self.IF_Null`))
            (:`Beth`
              (`self.IF_Beth`))))))))

(fn `Sort_List`
  (locals (Bufer :type "Array of Float (double-precision)"))
  (bind (_indexofminvalue _minvalue) (`KismetMathLibrary.MinOfFloatArray` (`local.Bufer`)))
  (bind _keys (`BlueprintMapLibrary.Map_Keys` (`self.Damage_Levels`)))
  (bind _output_get (set `local.Bufer` _keys))
  (while (> (`KismetArrayLibrary.Array_Length` _output_get) 0)
    (`KismetArrayLibrary.Array_Add` (`self.Float_Keys`) _minvalue)
    (`KismetArrayLibrary.Array_Remove` (`local.Bufer`) _indexofminvalue)))