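; BP_BaseStorage_AC is a base storage component holding an array of item stacks limited by a slot Capacity.
; Adding a stackable item tops up the first partial stack of the same class, recursing through AddItemToStorage with any overflow, otherwise creating a new slot.
; A full storage returns false, even after partially filling a stack.
; Removal takes one unit or deletes the slot, and a helper branches on the Opened state.
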(event `self.ReceiveBeginPlay`
  (`parent.ReceiveBeginPlay`))

(fn `Add Item To Storage`
  (params (`Item To Add` :type "/Game/DarkTaleDemo/Core/Miscellaneous/Inventory/InventoryStructure/SInventorySlot Structure"))
  (returns (Success :type Boolean))
  (bind _item_to_add_itemstructure (break `/Game/DarkTaleDemo/Core/Miscellaneous/Inventory/InventoryStructure/SInventorySlot` (`local.Item To Add`)))
  (if (`.IsStackable_5_B52D73584D8F68DCB2276DAA60B13975` (break `/Game/DarkTaleDemo/Core/Miscellaneous/Inventory/InventoryStructure/SItemSignature` (break `/Game/DarkTaleDemo/Core/Miscellaneous/Inventory/InventoryStructure/SInventorySlot` `Item To Add`)))
    (bind _stack_index (`self.Has Partial Stack` _item_to_add_itemstructure)
      (:`True`
        (bind _success (`self.Add To Stack` (`local.Item To Add`) _stack_index))
        (return _success))
      (:`False`
        _)))
  (bind _success_2 (`self.Create Stack` (`local.Item To Add`)))
  (return _success_2))

(fn `Add To Stack`
  (params (`To Add` :type "/Game/DarkTaleDemo/Core/Miscellaneous/Inventory/InventoryStructure/SInventorySlot Structure") (`Slot Index` :type Integer))
  (returns (Success :type Boolean))
  (locals (`Current Quantity` :type Integer))
  (bind _items (`self.Items`))
  (bind _slot_index (`local.Slot Index`))
  (bind (_to_add_itemstructure _to_add_quantity) (break `/Game/DarkTaleDemo/Core/Miscellaneous/Inventory/InventoryStructure/SInventorySlot` (`local.To Add`)))
  (bind _to_add_itemstructure_2 (break `/Game/DarkTaleDemo/Core/Miscellaneous/Inventory/InventoryStructure/SInventorySlot` (`local.To Add`)))
  (bind (_to_add_itemstructure_3 _to_add_quantity_2) (break `/Game/DarkTaleDemo/Core/Miscellaneous/Inventory/InventoryStructure/SInventorySlot` (`local.To Add`)))
  (bind (_name _description _isstackable _isconsumable _maxstacksize) (break `/Game/DarkTaleDemo/Core/Miscellaneous/Inventory/InventoryStructure/SItemSignature` _to_add_itemstructure_2))
  (bind _output (`|GetArrayItem` (`self.Items`) `Slot Index`))
  (bind (_output_itemstructure _output_quantity) (break `/Game/DarkTaleDemo/Core/Miscellaneous/Inventory/InventoryStructure/SInventorySlot` (`|GetArrayItem` _items _slot_index)))
  (bind _output_get (set `local.Current Quantity` (`.Quantity_5_715DEC3F4D3BC6156DE64DAEE147E216` (break `/Game/DarkTaleDemo/Core/Miscellaneous/Inventory/InventoryStructure/SInventorySlot` _output))))
  (if (> (+ `To Add_Quantity_5_715DEC3F4D3BC6156DE64DAEE147E216` _output_get) (`.MaxStackSize_18_707460814B45CCD43FF1AE893C5FC2C3` (break `/Game/DarkTaleDemo/Core/Miscellaneous/Inventory/InventoryStructure/SItemSignature` (break `/Game/DarkTaleDemo/Core/Miscellaneous/Inventory/InventoryStructure/SInventorySlot` _output))))
    (`KismetArrayLibrary.Array_Set` (`self.Items`) (`local.Slot Index`) (make `/Game/DarkTaleDemo/Core/Miscellaneous/Inventory/InventoryStructure/SInventorySlot` _to_add_itemstructure_2 _maxstacksize))
    (bind _success (`self.Add Item To Storage` (make `/Game/DarkTaleDemo/Core/Miscellaneous/Inventory/InventoryStructure/SInventorySlot` _to_add_itemstructure_3 (- _to_add_quantity_2 (- _maxstacksize (`local.Current Quantity`))))))
    (return _success)
    (else
      (`KismetArrayLibrary.Array_Set` _items _slot_index (make `/Game/DarkTaleDemo/Core/Miscellaneous/Inventory/InventoryStructure/SInventorySlot` _output_itemstructure (+ _output_quantity _to_add_quantity)))
      (return true))))

(fn `Create Stack`
  (params (`To Add` :type "/Game/DarkTaleDemo/Core/Miscellaneous/Inventory/InventoryStructure/SInventorySlot Structure"))
  (returns (Success :type Boolean))
  (if (> (`self.Capacity`) (`KismetArrayLibrary.Array_Length` (`self.Items`)))
    (`KismetArrayLibrary.Array_Add` (`self.Items`) (`local.To Add`))
    (return true)
    (else
      (return false))))

(fn `Remove Item From Storage`
  (params (`Item Index` :type Integer) (Force :type Boolean))
  (returns (Success :type Boolean))
  (bind (_output_itemstructure _output_quantity) (break `/Game/DarkTaleDemo/Core/Miscellaneous/Inventory/InventoryStructure/SInventorySlot` (`|GetArrayItem` (`self.Items`) `Item Index`)))
  (if (> _output_quantity 1)
    (`KismetArrayLibrary.Array_Set` (`self.Items`) (`local.Item Index`) (make `/Game/DarkTaleDemo/Core/Miscellaneous/Inventory/InventoryStructure/SInventorySlot` _output_itemstructure (- _output_quantity 1)))
    (else
      (`KismetArrayLibrary.Array_Remove` (`self.Items`) (`local.Item Index`))))
  (return true))