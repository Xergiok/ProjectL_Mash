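; Base interaction component that lets a pawn detect, highlight and interact with items in view.
; On tick, a locally controlled pawn sphere-traces forward for items, sending focus in/out messages as the sighted item changes.
; Sighted items get a BP_InfoIcon, cached per actor for reactivation, anchored through BPI_Icon and textured by the interface the actor implements.
; The side action runs a separate sphere trace and sends Interact; the main action is empty.
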(event `self.ReceiveBeginPlay`
  (`parent.ReceiveBeginPlay`))

(event `self.ReceiveTick`
  (params (DeltaSeconds :type "Float (single-precision)"))
  (`self.Check Line Of Sight Intersection`))

(event `/Game/DarkTaleDemo/Core/Main/Interfaces/Components/BPI_BaseInteraction.Side_Action_BPIF`
  (bind (_interaction_param_x _interaction_param_y) (`KismetMathLibrary.BreakVector2D` (`self.Interaction_Param`)))
  (bind (_returnvalue _last_hit_actor) (`/Game/DarkTaleDemo/Core/Main/FunctionLibrary/BPFL_Camera.Simple_SphereTrace_BPFL` (`self.Get_OwnerController`) _interaction_param_x _interaction_param_y))
  (if _returnvalue
    (message `/Game/DarkTaleDemo/Core/Main/Interfaces/Items/BPI_Interactable.Interact` _last_hit_actor (`self.GetOwner`))))

(event `/Game/DarkTaleDemo/Core/Main/Interfaces/Components/BPI_BaseInteraction.Main_Action_BPIF`)

(event `Item At Sight Gained`
  (params (`Last Item At Sight` :type "Actor Object Reference"))
  (`self.Add_InfoIcon` `Last Item At Sight`)
  (message `/Game/DarkTaleDemo/Core/Main/Interfaces/Items/BPI_Focusable.FocusedInto_BPIF` `Last Item At Sight` (`self.GetOwner`)))

(event `Item At Sight Lost`
  (params (`Last Item At Sight` :type "Actor Object Reference"))
  (`self.Remove_InfoIcon` `Last Item At Sight`)
  (message `/Game/DarkTaleDemo/Core/Main/Interfaces/Items/BPI_Focusable.FucusedOut_BPIF` `Last Item At Sight` (`self.GetOwner`)))

(fn `Add_InfoIcon`
  (params (Actor :type "Actor Object Reference"))
  (returns (Success :type Boolean))
  (locals (Anchor :type "SphereComponent Object Reference") (Mode :type "/Game/DarkTaleDemo/Core/Main/Components/Player/Interaction/EInfoIconMode Enum" :default "NewEnumerator0"))
  (bind _actor (`local.Actor`))
  (bind (_value _returnvalue) (`BlueprintMapLibrary.Map_Find` (`self.InfoIcons`) (`local.Actor`)))
  (`/Engine/EditorBlueprintResources/StandardMacros.IsValid` Actor
    (:`Is Valid`
      (if _returnvalue
        (`/Engine/EditorBlueprintResources/StandardMacros.IsValid` _value
          (:`Is Valid`
            (`/Game/DarkTaleDemo/Core/Main/Components/Player/Interaction/BP_InfoIcon.Activation` _value)
            (return true)))
        (elif (`KismetSystemLibrary.DoesImplementInterface` _actor "/Game/DarkTaleDemo/Core/Main/Interfaces/Items/BPI_Icon.BPI_Icon_C")
          (bind (_mode _anchor) (message `/Game/DarkTaleDemo/Core/Main/Interfaces/Items/BPI_Icon.Get_Anchor_BPIF` _actor))
          (set `local.Anchor` _anchor)
          (set `local.Mode` _mode)
          (bind _anchor_2 (`local.Anchor`)
            (:`then`
              (bind _returnvalue_2 (`SceneComponent.K2_GetComponentLocation` _anchor_2))
              (bind _returnvalue_3 (`|SpawnActorFromClass` "/Game/DarkTaleDemo/Core/Main/Components/Player/Interaction/BP_InfoIcon.BP_InfoIcon_C" (`KismetMathLibrary.MakeTransform` (select `/Game/DarkTaleDemo/Core/Main/Components/Player/Interaction/EInfoIconMode` (`local.Mode`) :`NewEnumerator0` (`Actor.K2_GetActorLocation` (`local.Actor`)) :`NewEnumerator1` _returnvalue_2 :`NewEnumerator2` _returnvalue_2 :`NewEnumerator3` _returnvalue_2)) "Undefined" "OverrideRootScale" (`local.Actor`) (`.Texture` (`self.Select_Texture` (`local.Actor`))) (`local.Anchor`) (`local.Mode`) (cast `Pawn` (`self.GetOwner`) :!pure true)))
              (`BlueprintMapLibrary.Map_Add` (`self.InfoIcons`) (`local.Actor`) _returnvalue_3)
              (return true))
            (:`else`)))))))

(fn `Check Line Of Sight Intersection`
  (locals (`Hit Item` :type "Actor Object Reference"))
  (bind (_los_param_x _los_param_y) (`KismetMathLibrary.BreakVector2D` (`self.LOS_Param`)))
  (bind (_start _end) (`self.ForwardTrace` _los_param_x))
  (bind _aspawn (cast `Pawn` (`self.GetOwner`)))
  (if (`Pawn.IsLocallyControlled` _aspawn)
    (bind (_outhit _returnvalue) (`KismetSystemLibrary.SphereTraceSingleForObjects` _start _end _los_param_y (`|MakeArray` "ObjectTypeQuery7" :!type "EObjectTypeQuery Enum") true (`|MakeArray` (`self.GetOwner`))))
    (if _returnvalue
      (bind (_bblockinghit _binitialoverlap _time _distance _location _impactpoint _normal _impactnormal _physmat _hitactor) (`GameplayStatics.BreakHitResult` _outhit))
      (`/Engine/EditorBlueprintResources/StandardMacros.IsValid` _hitactor
        (:`Is Valid`
          (set `local.Hit Item` _hitactor)
          (`self.IsSeeingItem`
            (:`T`
              (bind (_out_a _out_b) (`/Game/DarkTaleDemo/Core/Main/MacroLibrary/BPML_Object.DoOnly_IfDifferent(Object)_BPML` (`local.Hit Item`) (`self.Last Item At Sight`))
                (:`true`
                  (`self.Item At Sight Lost` _out_b))))
            (:`F`
              _))
          (bind _output_get (set `self.Last Item At Sight` (`local.Hit Item`)))
          (`self.Item At Sight Gained` _output_get)))
      (else
        (`self.IsSeeingItem`
          (:`T`
            (`self.Item At Sight Lost` (`self.Last Item At Sight`))
            (set `self.Last Item At Sight` null)))))))

(fn `Component_Initialization`
  (`parent.Component_Initialization`))

(fn `Remove_InfoIcon`
  (params (Actor :type "Actor Object Reference"))
  (bind (_value _returnvalue) (`BlueprintMapLibrary.Map_Find` (`self.InfoIcons`) Actor))
  (`/Engine/EditorBlueprintResources/StandardMacros.IsValid` Actor
    (:`Is Valid`
      (if _returnvalue
        (`/Game/DarkTaleDemo/Core/Main/Components/Player/Interaction/BP_InfoIcon.Deactivation ` _value)))))

(fn `Select_Texture`
  (params (Actor :type "Actor Object Reference"))
  (returns (Interface :type "Interface Class Reference") (Texture :type "Texture2D Object Reference"))
  (locals (Selected_Interface :type "Interface Class Reference"))
  (bind (_value _returnvalue) (`BlueprintMapLibrary.Map_Find` (`self.Interface_Selection`) (`local.Selected_Interface`)))
  (`/Engine/EditorBlueprintResources/StandardMacros.IsValid` Actor
    (:`Is Valid`
      (if (!= (`BlueprintMapLibrary.Map_Length` (`self.Interface_Selection`)) 0)
        (bind _keys (`BlueprintMapLibrary.Map_Keys` (`self.Interface_Selection`)))
        (for _array_element _keys
          (if (`KismetSystemLibrary.DoesImplementInterface` (`local.Actor`) _array_element)
            (set `local.Selected_Interface` _array_element)
            (if _returnvalue
              (`|ExecutionSequence`
                (:`then_0`
                  (break))
                (:`then_1`
                  (return (`local.Selected_Interface`) _value))))))))))

(fn `Simple_SphereTrace`
  (params (Length :type "Float (double-precision)") (Radius :type "Float (double-precision)") (DrawDebugType :type "EDrawDebugTrace Enum" :default "None"))
  (returns (ReturnValue :type Boolean) (Last_Hit_Actor :type "Actor Object Reference") (Last_Hit_ActorComp :type "PrimitiveComponent Object Reference"))
  (bind (_start _end) (`self.ForwardTrace` (`local.Length`)))
  (if (and (> Length 0.0) (> Radius 0.0))
    (bind (_outhit _returnvalue) (`KismetSystemLibrary.SphereTraceSingle` _start _end (`local.Radius`) "TraceTypeQuery1" true (`|MakeArray` (`self.GetOwner`)) (`local.DrawDebugType`)))
    (if _returnvalue
      (bind (_bblockinghit _binitialoverlap _time _distance _location _impactpoint _normal _impactnormal _physmat _hitactor _hitcomponent) (`GameplayStatics.BreakHitResult` _outhit))
      (`/Engine/EditorBlueprintResources/StandardMacros.IsValid` _hitactor
        (:`Is Valid`
          (`/Engine/EditorBlueprintResources/StandardMacros.IsValid` _hitcomponent
            (:`Is Valid`
              (return true _hitactor _hitcomponent))
            (:`Is Not Valid`
              _)))
        (:`Is Not Valid`
          _)))
    (return false null null)))