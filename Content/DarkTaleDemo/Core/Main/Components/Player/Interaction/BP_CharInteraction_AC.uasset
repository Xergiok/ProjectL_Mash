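; Player interaction component for BP_HumanChar that handles picking up, holding, using, stowing, dropping and examining items.
; Side action and examine sphere-trace for targets, picking up or interacting by interface, or spawning a camera-attached icon anchor for inspection.
; A hand-slot map tracks held items; main action uses or double-clicks to inventory, double-click concentration drops.
; Gate macros toggle each action and the per-tick line-of-sight check.
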(event `self.ReceiveBeginPlay`
  (`parent.ReceiveBeginPlay`)
  (`self.Component_Initialization`))

(event `self.ReceiveEndPlay`
  (params (EndPlayReason :type "EEndPlayReason Enum" :default "Destroyed"))
  (clear `self.OnComponentDeactivated`))

(event `Enable_LOS`
  ;[1 1 1] Perfoming LOS - line of sight intersection, every tick
  (`|ExecutionSequence`
    (:`then_0`
      (goto _label :!via `Open`))
    (:`then_1`
      (goto _label_2 :!via `Close`))))

(event `Disable_LOS`
  ;[1 1 1] Perfoming LOS - line of sight intersection, every tick
  (`|ExecutionSequence`
    (:`then_0`
      (goto _label :!via `Close`))
    (:`then_1`
      (goto _label_2 :!via `Open`))))

(event `self.ReceiveTick`
  (params (DeltaSeconds :type "Float (single-precision)"))
  ;[1 1 1] Perfoming LOS - line of sight intersection, every tick
  (`|ExecutionSequence`
    (:`then_0`
      (`/Engine/EditorBlueprintResources/StandardMacros.Gate` false :!label _label
        (:`Exit`
          (`self.Check Line Of Sight Intersection`))))
    (:`then_1`
      (`/Engine/EditorBlueprintResources/StandardMacros.Gate` true :!label _label_2
        (:`Exit`
          (`self.Item At Sight Lost` (`self.Last Item At Sight`))
          (set `self.Last Item At Sight` null))))))

(event `/Game/DarkTaleDemo/Core/Main/Interfaces/Components/BPI_BaseInteraction.Main_Action_BPIF`
  (bind (_exist _item) (`self.Get_SlotItem` "NewEnumerator1"))
  (`|ExecutionSequence`
    (:`then_0`
      (`/Engine/EditorBlueprintResources/StandardMacros.Gate` false :!label _label_3
        (:`Exit`
          (`self.Switch_IsExamineItem`
            (:`F`
              (`self.Switch_IsHoldingItem` "NewEnumerator1"
                (:`T`
                  (`self.DoubleClick` 0.3
                    (:`Double`
                      (`self.Add_Slot_to_Inventory` "NewEnumerator1"))
                    (:`Single`
                      (if _exist
                        (`/Engine/EditorBlueprintResources/StandardMacros.IsValid` _item
                          (:`Is Valid`
                            (message `/Game/DarkTaleDemo/Core/Main/Interfaces/Items/BPI_Usable.Use` _item (`self.GetOwner`))))))))))))))
    (:`then_1`
      (`/Engine/EditorBlueprintResources/StandardMacros.Gate` true :!label _label_4))))

(event `Disable_MainAction`
  (`|ExecutionSequence`
    (:`then_0`
      (goto _label_3 :!via `Close`))
    (:`then_1`
      (goto _label_4 :!via `Open`))))

(event `Enable_MainAction`
  (`|ExecutionSequence`
    (:`then_0`
      (goto _label_3 :!via `Open`))
    (:`then_1`
      (goto _label_4 :!via `Close`))))

(event `/Game/DarkTaleDemo/Core/Main/Interfaces/Components/BPI_BaseInteraction.Side_Action_BPIF`
  (bind (_interaction_param_x _interaction_param_y) (`KismetMathLibrary.BreakVector2D` (`self.Interaction_Param`)))
  (`|ExecutionSequence`
    (:`then_0`
      (`/Engine/EditorBlueprintResources/StandardMacros.Gate` false :!label _label_5
        (:`Exit`
          (bind (_returnvalue _last_hit_actor) (`/Game/DarkTaleDemo/Core/Main/FunctionLibrary/BPFL_Camera.Simple_SphereTrace_BPFL` (`self.Get_OwnerController`) _interaction_param_x _interaction_param_y))
          (if _returnvalue
            (`/Engine/EditorBlueprintResources/StandardMacros.IsValid` _last_hit_actor
              (:`Is Valid`
                (`self.Switch_ItemInterfaces` _last_hit_actor
                  (:`Pickable`
                    (bind _asbp_item_pickable (cast `/Game/DarkTaleDemo/Core/Main/ItemSystem/Pickable/BP_Item_Pickable` _last_hit_actor))
                    (`self.Hold_Switch` _asbp_item_pickable true))
                  (:`Interactable`
                    (message `/Game/DarkTaleDemo/Core/Main/Interfaces/Items/BPI_Interactable.Interact` _last_hit_actor (`self.GetOwner`))))))))))
    (:`then_1`
      (`/Engine/EditorBlueprintResources/StandardMacros.Gate` true :!label _label_6))))

(event `Enable_SideAction`
  (`|ExecutionSequence`
    (:`then_0`
      (goto _label_5 :!via `Open`))
    (:`then_1`
      (goto _label_6 :!via `Close`))))

(event `Disable_SideAction`
  (`|ExecutionSequence`
    (:`then_0`
      (goto _label_5 :!via `Close`))
    (:`then_1`
      (goto _label_6 :!via `Open`))))

(event `/Game/DarkTaleDemo/Core/Main/Interfaces/Components/BPI_BaseInteraction.Concentration_BPIF`
  (`|ExecutionSequence`
    (:`then_0`
      (`/Engine/EditorBlueprintResources/StandardMacros.Gate` false :!label _label_7
        (:`Exit`
          (`self.Switch_IsHoldingItem` "NewEnumerator1"
            (:`T`
              (`self.DoubleClick` 0.3
                (:`Double`
                  (`self.Drop_Slot` "NewEnumerator1"))))))))
    (:`then_1`
      (`/Engine/EditorBlueprintResources/StandardMacros.Gate` true :!label _label_8))))

(event `Enable_Concentration`
  (`|ExecutionSequence`
    (:`then_0`
      (goto _label_7 :!via `Open`))
    (:`then_1`
      (goto _label_8 :!via `Close`))))

(event `Disable_Concentration`
  (`|ExecutionSequence`
    (:`then_0`
      (goto _label_7 :!via `Close`))
    (:`then_1`
      (goto _label_8 :!via `Open`))))

(event `Equip_Light`
  (`/Engine/EditorBlueprintResources/StandardMacros.FlipFlop`
    (:`A`
      (`KismetSystemLibrary.PrintString` "EquipLight"))
    (:`B`
      (`KismetSystemLibrary.PrintString` "UnequipLight"))))

(event `Toggle_Light`
  (bind (_exist _item) (`self.Get_SlotItem` "NewEnumerator2"))
  (`self.Switch_IsHoldingItem` "NewEnumerator2"
    (:`T`
      (if _exist
        (`/Engine/EditorBlueprintResources/StandardMacros.IsValid` _item
          (:`Is Valid`
            (message `/Game/DarkTaleDemo/Core/Main/Interfaces/Items/BPI_Usable.Use` _item (`self.GetOwner`))))))))

(event `self.Item At Sight Gained`
  (params (`Last Item At Sight` :type "Actor Object Reference"))
  ;[1 1 1] LOS inplementation
  (`parent.Item At Sight Gained` `Last Item At Sight`))

(event `self.Item At Sight Lost`
  (params (`Last Item At Sight` :type "Actor Object Reference"))
  ;[1 1 1] LOS inplementation
  (`parent.Item At Sight Lost` `Last Item At Sight`))

(event `/Game/DarkTaleDemo/Core/Main/Interfaces/Components/BPI_BaseInteraction.Examine_BPIF`
  (bind (_interaction_param_x _interaction_param_y) (`KismetMathLibrary.BreakVector2D` (`self.Interaction_Param`)))
  (`self.Switch_IsExamineItem`
    (:`T`
      (`self.Toggle_Examine`))
    (:`F`
      (bind (_returnvalue _last_hit_actor) (`/Game/DarkTaleDemo/Core/Main/FunctionLibrary/BPFL_Camera.Simple_SphereTrace_BPFL` (`self.Get_OwnerController`) _interaction_param_x _interaction_param_y))
      (if _returnvalue
        (`self.Begin_Examine` _last_hit_actor)))))

(fn `Add_Slot_to_Inventory`
  (params (Slot :type "/Game/DarkTaleDemo/Core/Miscellaneous/Inventory/EHandSlots Enum" :default "NewEnumerator0"))
  (bind (_exist _item) (`self.Get_SlotItem` "NewEnumerator1"))
  (bind (_exist_2 _item_2) (`self.Get_SlotItem` "NewEnumerator2"))
  (bind (_exist_3 _item_3) (`self.Get_SlotItem` (`local.Slot`)))
  (switch `/Game/DarkTaleDemo/Core/Miscellaneous/Inventory/EHandSlots` Slot
    (:`NewEnumerator1`
      (if _exist_3 :!label _label
        (bind _player (`self.Player`)
          (:`then`
            (message `/Game/DarkTaleDemo/Core/Main/Interfaces/Items/BPI_Pickable.Add To Inventory` _item_3 _player))
          (:`else`))))
    (:`NewEnumerator2`
      (goto _label))
    (:`NewEnumerator3`
      (if _exist
        (bind _player_2 (`self.Player`)
          (:`then`
            (message `/Game/DarkTaleDemo/Core/Main/Interfaces/Items/BPI_Pickable.Add To Inventory` _item _player_2)
            (if _exist_2
              (bind _player_3 (`self.Player`)
                (:`then`
                  (message `/Game/DarkTaleDemo/Core/Main/Interfaces/Items/BPI_Pickable.Add To Inventory` _item_2 _player_3))
                (:`else`))))
          (:`else`))))))

(fn `Begin_Examine`
  (params (Actor :type "Actor Object Reference"))
  (locals (Item :type "/Game/DarkTaleDemo/Core/Main/ItemSystem/BP_Item_Master Object Reference") (Inspect_Location :type "SceneComponent Object Reference"))
  (bind _asbp_item_examine (cast `/Game/DarkTaleDemo/Core/Main/ItemSystem/BP_Item_Examine` Actor))
  (set `local.Item` _asbp_item_examine)
  (`self.Disable_LOS`)
  (set `local.Inspect_Location` (`/Game/DarkTaleDemo/Core/Main/Control/PlayerCameraManagers/CM_Default.Inspect_Location` (cast `/Game/DarkTaleDemo/Core/Main/Control/PlayerCameraManagers/CM_Default` (`PlayerController.PlayerCameraManager` (`self.Get_OwnerController`)) :!pure true)))
  (bind _returnvalue (`|SpawnActorFromClass` "/Game/DarkTaleDemo/Core/Main/Components/Player/Interaction/BP_IconAnchor.BP_IconAnchor_C" (`SceneComponent.K2_GetComponentToWorld` (`local.Inspect_Location`)) "Undefined" "OverrideRootScale" (`self.Get_OwnerController`) (`local.Item`) (`self.Player`)))
  (bind _output_get (set `self.Examine_Actor` _returnvalue))
  (`Actor.K2_AttachToComponent` _output_get (`local.Inspect_Location`) "None" "SnapToTarget" "SnapToTarget" "SnapToTarget" true)
  (`/Game/DarkTaleDemo/Core/Main/Components/Player/Interaction/BP_IconAnchor.Begin_Examine` (`self.Examine_Actor`)))

(fn `Component_Initialization`
  (`parent.Component_Initialization`)
  (bind _asbp_human_char (cast `/Game/DarkTaleDemo/Core/Main/Characters/Player/BP_HumanChar` (`self.GetOwner`)))
  (set `self.Player` _asbp_human_char)
  (`|ExecutionSequence`
    (:`then_0`
      (`|ExecutionSequence`
        (:`then_0`
          (bind _player (`self.Player`)
            (:`then`
              (add `/Game/DarkTaleDemo/Core/Main/Characters/Player/BP_HumanChar.EventDisp_SecondarySlotToggle` _player (`|CreateDelegate` :!event `Equip_Light`))
              (bind _player_2 (`self.Player`)
                (:`then`
                  (add `/Game/DarkTaleDemo/Core/Main/Characters/Player/BP_HumanChar.EventDisp_LightToggle` _player_2 (`|CreateDelegate` :!event `Toggle_Light`)))
                (:`else`)))
            (:`else`)))))))

(fn `Drop_Slot`
  (params (Slot :type "/Game/DarkTaleDemo/Core/Miscellaneous/Inventory/EHandSlots Enum" :default "NewEnumerator0"))
  (bind (_exist _item) (`self.Get_SlotItem` Slot))
  (if _exist
    (`self.Hold_Switch` _item)))

(fn `Get_SlotItem`
  (params (Slot :type "/Game/DarkTaleDemo/Core/Miscellaneous/Inventory/EHandSlots Enum" :default "NewEnumerator0"))
  (returns (Exist :type Boolean) (Item :type "/Game/DarkTaleDemo/Core/Main/ItemSystem/Pickable/BP_Item_Pickable Object Reference"))
  (bind (_both_ _value) (`self.Is_BothHands`))
  (bind _handslots (`self.HandSlots`))
  (bind (_value_2 _returnvalue) (`BlueprintMapLibrary.Map_Find` _handslots "VR_LeftHand"))
  (bind (_value_3 _returnvalue_2) (`BlueprintMapLibrary.Map_Find` _handslots "VR_RightHand"))
  (switch `/Game/DarkTaleDemo/Core/Miscellaneous/Inventory/EHandSlots` Slot
    (:`NewEnumerator0`
      (return (`self.Is_HandsEmpty`) null))
    (:`NewEnumerator1`
      (return _returnvalue_2 _value_3))
    (:`NewEnumerator2`
      (return _returnvalue _value_2))
    (:`NewEnumerator3`
      (return _both_ _value))))

(fn `Get_ValidSlots`
  (returns (Keys :type "Array of EHand Enum"))
  (bind _keys (`BlueprintMapLibrary.Map_Keys` (`self.HandSlots`)))
  (return _keys))

(fn `Hold_Switch`
  (params (Item :type "/Game/DarkTaleDemo/Core/Main/ItemSystem/Pickable/BP_Item_Pickable Object Reference") (Hold :type Boolean))
  (locals (DesiredSlot :type "/Game/DarkTaleDemo/Core/Miscellaneous/Inventory/EHandSlots Enum"))
  (bind _returnvalue (`self.GetOwner`))
  (bind ((`SlotPriority_37_BA3499684EAE1C3FD85AB2A7E7E13969` _slotpriority)) (break `/Game/DarkTaleDemo/Core/Miscellaneous/Inventory/InventoryStructure/SItemSignature` (`/Game/DarkTaleDemo/Core/Main/ItemSystem/BP_Item_Master.ItemSignature` Item)))
  (bind (_exist _item) (`self.Get_SlotItem` (`local.DesiredSlot`)))
  (`/Engine/EditorBlueprintResources/StandardMacros.IsValid` Item
    (:`Is Valid`
      (if (`|EnumInequality` _slotpriority "NewEnumerator0")
        (set `local.DesiredSlot` _slotpriority)
        (if (`local.Hold`)
          (`self.Switch_IsHoldingItem` (`local.DesiredSlot`)
            (:`F`
              (bind _success (`self.Set_Slots` (`local.DesiredSlot`) (`local.Item`)))
              (if _success
                (message `/Game/DarkTaleDemo/Core/Main/Interfaces/Items/BPI_Pickable.Pick Up` (`.Item` (`self.Get_SlotItem` (`local.DesiredSlot`))) _returnvalue (`self.Select_SocketName` _returnvalue (`local.DesiredSlot`))))))
          (else
            (`self.Switch_IsHoldingItem` (`local.DesiredSlot`)
              (:`T`
                (if (== _item (`local.Item`))
                  (message `/Game/DarkTaleDemo/Core/Main/Interfaces/Items/BPI_Pickable.Throw` _item)
                  (`self.Remove_Slot` (`local.DesiredSlot`)))))))))))

(fn `Inspect_Slot`
  (params (Slot :type "/Game/DarkTaleDemo/Core/Miscellaneous/Inventory/EHandSlots Enum" :default "NewEnumerator0"))
  (bind (_exist _item) (`self.Get_SlotItem` Slot))
  (if _exist
    (message `/Game/DarkTaleDemo/Core/Main/Interfaces/Items/BPI_Inspectable.Inspect` _item (`self.GetOwner`))))

(fn `Is_BothHands`
  (returns (`Both?` :type Boolean) (Value :type "/Game/DarkTaleDemo/Core/Main/ItemSystem/Pickable/BP_Item_Pickable Object Reference"))
  (bind _handslots (`self.HandSlots`))
  (bind (_value _returnvalue) (`BlueprintMapLibrary.Map_Find` _handslots "VR_LeftHand"))
  (bind (_value_2 _returnvalue_2) (`BlueprintMapLibrary.Map_Find` _handslots "VR_RightHand"))
  (if _returnvalue_2
    (if _returnvalue
      (return (== _value_2 _value) _value_2))))

(fn `Is_HandsEmpty`
  (returns (ReturnValue :type Boolean))
  (return (== (`BlueprintMapLibrary.Map_Length` (`self.HandSlots`)) 0)))

(fn `Remove_Slot`
  (params (Slot :type "/Game/DarkTaleDemo/Core/Miscellaneous/Inventory/EHandSlots Enum" :default "NewEnumerator0"))
  (locals (RightHand :type "EHand Enum" :default "VR_RightHand") (LeftHand :type "EHand Enum"))
  (switch `/Game/DarkTaleDemo/Core/Miscellaneous/Inventory/EHandSlots` Slot
    (:`NewEnumerator1`
      (`BlueprintMapLibrary.Map_Remove` (`self.HandSlots`) (select `/Game/DarkTaleDemo/Core/Miscellaneous/Inventory/EHandSlots` (`local.Slot`) :`NewEnumerator0` "VR_LeftHand" :`NewEnumerator1` (`local.RightHand`) :`NewEnumerator2` (`local.LeftHand`) :`NewEnumerator3` "VR_LeftHand") :!label _label))
    (:`NewEnumerator2`
      (goto _label))
    (:`NewEnumerator3`
      (`BlueprintMapLibrary.Map_Clear` (`self.HandSlots`)))))

(fn `Select_SocketName`
  (params (Actor :type "Actor Object Reference") (Index :type "/Game/DarkTaleDemo/Core/Miscellaneous/Inventory/EHandSlots Enum" :default "NewEnumerator0"))
  (returns (ReturnValue :type Name))
  (bind _asbp_human_char (cast `/Game/DarkTaleDemo/Core/Main/Characters/Player/BP_HumanChar` Actor)
    (:`then`
      (bind (_character_sockets_pelvisbone _character_sockets_headsocket _character_sockets_righthandsocket _character_sockets_lefthandsocket) (break `/Game/DarkTaleDemo/Core/Miscellaneous/CharacterDefaults/Sockets/SCharSockets` (`/Game/DarkTaleDemo/Core/Main/Characters/Player/BP_HumanChar.Character_Sockets` _asbp_human_char)))
      (return (select `/Game/DarkTaleDemo/Core/Miscellaneous/Inventory/EHandSlots` Index :`NewEnumerator1` _character_sockets_righthandsocket :`NewEnumerator2` _character_sockets_lefthandsocket :`NewEnumerator3` _character_sockets_righthandsocket)))
    (:`CastFailed`
      (return "None"))))

(fn `Set_Slots`
  (params (Slot :type "/Game/DarkTaleDemo/Core/Miscellaneous/Inventory/EHandSlots Enum" :default "NewEnumerator0") (Item :type "/Game/DarkTaleDemo/Core/Main/ItemSystem/Pickable/BP_Item_Pickable Object Reference"))
  (returns (Success :type Boolean))
  (bind _handslots (`self.HandSlots`))
  (bind _item (`local.Item`))
  (if (not (`|EnumEquality` Slot "NewEnumerator0"))
    (`/Engine/EditorBlueprintResources/StandardMacros.IsValid` (`local.Item`)
      (:`Is Valid`
        (switch `/Game/DarkTaleDemo/Core/Miscellaneous/Inventory/EHandSlots` (`local.Slot`)
          (:`NewEnumerator0`
            _)
          (:`NewEnumerator1`
            (`BlueprintMapLibrary.Map_Add` _handslots "VR_RightHand" _item)
            (return true))
          (:`NewEnumerator2`
            (`BlueprintMapLibrary.Map_Add` _handslots "VR_LeftHand" _item)
            (return true))
          (:`NewEnumerator3`
            (if (not (`self.Is_HandsEmpty`))
              (`self.Add_Slot_to_Inventory` "NewEnumerator3"))
            (`BlueprintMapLibrary.Map_Add` (`self.HandSlots`) "VR_RightHand" (`local.Item`))
            (`BlueprintMapLibrary.Map_Add` (`self.HandSlots`) "VR_LeftHand" (`local.Item`))
            (return true))))
      (:`Is Not Valid`
        (return false))))
  (`BlueprintMapLibrary.Map_Add` (`self.HandSlots`) "VR_RightHand")
  (`BlueprintMapLibrary.Map_Add` (`self.HandSlots`) "VR_LeftHand")
  (return true))

(fn `Toggle_Examine`
  (bind _examine_actor (`self.Examine_Actor`))
  (`/Engine/EditorBlueprintResources/StandardMacros.IsValid` _examine_actor
    (:`Is Valid`
      (`/Game/DarkTaleDemo/Core/Main/Components/Player/Interaction/BP_IconAnchor.Finish_Examine` _examine_actor))))