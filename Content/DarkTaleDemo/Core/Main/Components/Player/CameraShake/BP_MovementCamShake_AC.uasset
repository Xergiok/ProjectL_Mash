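; Player component that drives movement camera shake and velocity-based camera tilt for BP_HumanChar.
; Character dispatchers for moving, gait, stance and control-type changes trigger switching between idle shakes and layered noise, pitch and roll shakes, over a persistent noise shake.
; Tick scales moving shakes by normalized speed, with roll also weighted by camera-to-velocity angle.
; Tick also interpolates the CMD_Velolcity modifier's additive rotation from character-to-velocity angle and speed, easing to zero when stopped.
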(event `self.ReceiveBeginPlay`
  (`self.Component_Initialization`)
  (bind _camera_manager (`self.Camera_Manager`)
    (:`then`
      (bind _returnvalue (`PlayerCameraManager.PlayCameraShake` :`self` _camera_manager :`ShakeClass` "/Game/DarkTaleDemo/Core/Miscellaneous/CameraShake/Movement/Idle/CS_PersistentNoise.CS_PersistentNoise_C"))
      (set `self.CS_PersistentNoise` _returnvalue)
      (`self.IdleSwitch_CS`))
    (:`else`)))

(event `self.ReceiveTick`
  (params (DeltaSeconds :type "Float (single-precision)"))
  (`self.Update_VelocityModifier`)
  (`self.Update_CameraShakes`))

(event `Update_Set_Gait`
  (bind _playerh_character (`self.PlayerH_Character`)
    (:`then`
      (bind _out_a (`/Game/DarkTaleDemo/Core/Main/MacroLibrary/BPML_Object.DoOnly_IfDifferent(Byte)_BPML` (`/Game/DarkTaleDemo/Core/Main/Characters/Player/BP_HumanChar.Current_GaitType` _playerh_character) (`self.Player_Gait`))
        (:`true`
          (set `self.Player_Gait` _out_a)
          (`self.Switch_IsMoving`
            (:`T`
              (`self.IdleSwitch_CS`))))))
    (:`else`)))

(event `Update_Set_ControlType`
  (bind _playerh_character (`self.PlayerH_Character`)
    (:`then`
      (bind _out_a (`/Game/DarkTaleDemo/Core/Main/MacroLibrary/BPML_Object.DoOnly_IfDifferent(Byte)_BPML` (`/Game/DarkTaleDemo/Core/Main/Characters/Player/BP_HumanChar.Current_PawnControlType` _playerh_character) (`self.Player_ControlType`))
        (:`true`
          (set `self.Player_ControlType` _out_a)
          (`self.Switch_IsMoving`
            (:`T`
              (`self.IdleSwitch_CS`))))))
    (:`else`)))

(event `Update_Set_Stance`
  (bind _playerh_character (`self.PlayerH_Character`)
    (:`then`
      (bind _out_a (`/Game/DarkTaleDemo/Core/Main/MacroLibrary/BPML_Object.DoOnly_IfDifferent(Byte)_BPML` (`/Game/DarkTaleDemo/Core/Main/Characters/Player/BP_HumanChar.Current_Stance` _playerh_character) (`self.Player_Stance`))
        (:`true`
          (set `self.Player_Stance` _out_a)
          (`self.Switch_IsMoving`
            (:`T`
              (`self.IdleSwitch_CS`))))))
    (:`else`)))

(event `Update_Set)IsMoving`
  (bind _playerh_character (`self.PlayerH_Character`)
    (:`then`
      (bind _out_a (`/Game/DarkTaleDemo/Core/Main/MacroLibrary/BPML_Object.DoOnly_IfDifferent(Bool)_BPML` (`/Game/DarkTaleDemo/Core/Main/Characters/Player/BP_HumanChar.IsMoving` _playerh_character) (`self.IsMoving`))
        (:`true`
          (set `self.IsMoving` _out_a)
          (`self.IdleSwitch_CS`))))
    (:`else`)))

(fn `Calculate_SpeedIntensity_Scale`
  (params (FB_Input :type "Float (double-precision)") (RL_Input :type "Float (double-precision)"))
  (returns (ReturnValue :type "Float (double-precision)"))
  (bind (_default_maxspeed_value _coefmax_crouch_speed _coefmax_sprint_speed _coefmax_slowwalk_speed) (break `/Game/DarkTaleDemo/Core/Miscellaneous/CharacterDefaults/Movement/SSpeedCoefs` (`self.Speed_Coef`)))
  (bind ((`CharacterMoveInput_RL_Scale_8_D12A3ED2458183AC5B155782F3C9088B` _charactermoveinput_rl_scale) (`CharacterMoveInput_Backward_Scale_10_2AA8B1A044701216F644BB962219ADEB` _charactermoveinput_backward_scale)) (break `/Game/DarkTaleDemo/Core/Miscellaneous/CharacterDefaults/Movement/SCharInputParams` (`self.Input_Coef`)))
  (return (`KismetMathLibrary.NormalizeToRange` (`KismetMathLibrary.VSize` (`Actor.GetVelocity` (`self.PlayerH_Character`))) 0.0 (* (`KismetMathLibrary.SelectFloat` _charactermoveinput_backward_scale (`KismetMathLibrary.SelectFloat` _charactermoveinput_rl_scale 1.0 (and (!= (`local.RL_Input`) 0.0) (== (`local.FB_Input`) 0.0))) (< (`local.FB_Input`) 0.0)) (select `/Game/DarkTaleDemo/Core/Miscellaneous/MovementEnums/EStance` (`self.Player_Stance`) :`NewEnumerator0` (select `/Game/DarkTaleDemo/Core/Miscellaneous/MovementEnums/EGaitTypes` (`self.Player_Gait`) :`NewEnumerator1` _default_maxspeed_value :`NewEnumerator0` (* _default_maxspeed_value _coefmax_slowwalk_speed) :`NewEnumerator2` (* _default_maxspeed_value _coefmax_sprint_speed)) :`NewEnumerator1` (* _default_maxspeed_value _coefmax_crouch_speed))))))

(fn `Component_Initialization`
  (`parent.Component_Initialization`)
  (bind _asbp_human_char (cast `/Game/DarkTaleDemo/Core/Main/Characters/Player/BP_HumanChar` (`self.GetOwner`)))
  (bind _output_get (set `self.PlayerH_Character` _asbp_human_char))
  (bind (_movement_defaults_inputparams _movement_defaults_speedparams) (break `/Game/DarkTaleDemo/Core/Miscellaneous/CharacterDefaults/Movement/SCharMovementParams` (`/Game/DarkTaleDemo/Core/Main/Characters/Player/BP_HumanChar.Movement_Defaults` _output_get)))
  (set `self.Input_Coef` _movement_defaults_inputparams)
  (set `self.Speed_Coef` _movement_defaults_speedparams)
  (bind _playerh_character (`self.PlayerH_Character`)
    (:`then`
      (bind _aspc_default (cast `/Game/DarkTaleDemo/Core/Main/Control/PlayerControllers/PC_Default` (`Pawn.GetController` _playerh_character)))
      (bind _ascm_default (cast `/Game/DarkTaleDemo/Core/Main/Control/PlayerCameraManagers/CM_Default` (`PlayerController.PlayerCameraManager` _aspc_default)))
      (set `self.Camera_Manager` _ascm_default)
      (bind _returnvalue (`PlayerCameraManager.AddNewCameraModifier` (`self.Camera_Manager`) "/Game/DarkTaleDemo/Core/Miscellaneous/CameraModifiers/Movement/CMD_Velolcity.CMD_Velolcity_C"))
      (bind _ascmd_velolcity (cast `/Game/DarkTaleDemo/Core/Miscellaneous/CameraModifiers/Movement/CMD_Velolcity` _returnvalue))
      (set `self.Velocity_CamMod` _ascmd_velolcity)
      (`|ExecutionSequence`
        (:`then_0`
          (bind _playerh_character_2 (`self.PlayerH_Character`)
            (:`then`
              (add `/Game/DarkTaleDemo/Core/Main/Characters/Player/BP_HumanChar.EventDisp_IsMoving_Changed` _playerh_character_2 (`|CreateDelegate` :!event `Update_Set)IsMoving`))
              (bind _playerh_character_3 (`self.PlayerH_Character`)
                (:`then`
                  (add `/Game/DarkTaleDemo/Core/Main/Characters/Player/BP_HumanChar.EventDisp_PawnControl_Changed` _playerh_character_3 (`|CreateDelegate` :!event `Update_Set_ControlType`))
                  (bind _playerh_character_4 (`self.PlayerH_Character`)
                    (:`then`
                      (add `/Game/DarkTaleDemo/Core/Main/Characters/Player/BP_HumanChar.EventDisp_GateType_Changed` _playerh_character_4 (`|CreateDelegate` :!event `Update_Set_Gait`))
                      (bind _playerh_character_5 (`self.PlayerH_Character`)
                        (:`then`
                          (add `/Game/DarkTaleDemo/Core/Main/Characters/Player/BP_HumanChar.EventDisp_Stance_Changed` _playerh_character_5 (`|CreateDelegate` :!event `Update_Set_Stance`)))
                        (:`else`)))
                    (:`else`)))
                (:`else`)))
            (:`else`)))))
    (:`else`)))

(fn `IdleSwitch_CS`
  (`/Engine/EditorBlueprintResources/StandardMacros.IsValid` (`self.Camera_Manager`)
    (:`Is Valid`
      (`self.Switch_ShakeType`
        (:`Idle`
          (`self.Stop_Idle_CS` false))
        (:`Moving`
          (`self.Stop_Ambient_CS` false)))
      (`self.Switch_IsMoving`
        (:`T`
          (`self.PlayAmbien_CS`))
        (:`F`
          (`self.Play_Idle_CS`))))))

(fn `PawnControlSwitch_CS`
  (bind _playerh_character (`self.PlayerH_Character`)
    (:`then`
      (switch `/Game/DarkTaleDemo/Core/Miscellaneous/MovementEnums/EPawnControl` (`/Game/DarkTaleDemo/Core/Main/Characters/Player/BP_HumanChar.Current_PawnControlType` _playerh_character)))
    (:`else`)))

(fn `Play_Idle_CS`
  (`/Engine/EditorBlueprintResources/StandardMacros.IsValid` (`self.Camera_Manager`)
    (:`Is Valid`
      (set `self.ShakeType` "NewEnumerator0")
      (bind _returnvalue (`PlayerCameraManager.PlayCameraShake` :`self` (`self.Camera_Manager`) :`ShakeClass` (select `/Game/DarkTaleDemo/Core/Miscellaneous/MovementEnums/EStance` (`self.Player_Stance`) :`NewEnumerator0` "/Game/DarkTaleDemo/Core/Miscellaneous/CameraShake/Movement/Idle/Gaits/CS_IdleNoise_Stand.CS_IdleNoise_Stand_C" :`NewEnumerator1` "/Game/DarkTaleDemo/Core/Miscellaneous/CameraShake/Movement/Idle/Gaits/CS_IdleNoise_Crouch.CS_IdleNoise_Crouch_C" :!type "CameraShake Class Reference") :`Scale` 2.0))
      (set `self.Idle_CS` _returnvalue))))

(fn `PlayAmbien_CS`
  (locals (Gait :type "/Game/DarkTaleDemo/Core/Miscellaneous/MovementEnums/EGaitTypes Enum" :default "NewEnumerator1"))
  (`/Engine/EditorBlueprintResources/StandardMacros.IsValid` (`self.Camera_Manager`)
    (:`Is Valid`
      (set `self.ShakeType` "NewEnumerator1")
      (bind _returnvalue (`PlayerCameraManager.PlayCameraShake` :`self` (`self.Camera_Manager`) :`ShakeClass` (select `/Game/DarkTaleDemo/Core/Miscellaneous/MovementEnums/EStance` (`self.Player_Stance`) :`NewEnumerator0` (select `/Game/DarkTaleDemo/Core/Miscellaneous/MovementEnums/EGaitTypes` (`self.Player_Gait`) :`NewEnumerator1` "/Game/DarkTaleDemo/Core/Miscellaneous/CameraShake/Movement/Moving/Running/CS_Noise_Running.CS_Noise_Running_C" :`NewEnumerator0` "/Game/DarkTaleDemo/Core/Miscellaneous/CameraShake/Movement/Moving/Walking/CS_Noise_Walking.CS_Noise_Walking_C" :`NewEnumerator2` "/Game/DarkTaleDemo/Core/Miscellaneous/CameraShake/Movement/Moving/Sprinting/CS_Noise_Sprinting.CS_Noise_Sprinting_C" :!type "CameraShake Class Reference") :`NewEnumerator1` "/Game/DarkTaleDemo/Core/Miscellaneous/CameraShake/Movement/Moving/Crouching/CS_Noise_Crouching.CS_Noise_Crouching_C")))
      (set `self.AmbienNoise_CS` _returnvalue)
      (bind _returnvalue_2 (`PlayerCameraManager.PlayCameraShake` :`self` (`self.Camera_Manager`) :`ShakeClass` (select `/Game/DarkTaleDemo/Core/Miscellaneous/MovementEnums/EStance` (`self.Player_Stance`) :`NewEnumerator0` (select `/Game/DarkTaleDemo/Core/Miscellaneous/MovementEnums/EGaitTypes` (`self.Player_Gait`) :`NewEnumerator1` "/Game/DarkTaleDemo/Core/Miscellaneous/CameraShake/Movement/Moving/Running/CS_ForwardPitch_Running.CS_ForwardPitch_Running_C" :`NewEnumerator0` "/Game/DarkTaleDemo/Core/Miscellaneous/CameraShake/Movement/Moving/Walking/CS_ForwardPitch_Walking.CS_ForwardPitch_Walking_C" :`NewEnumerator2` "/Game/DarkTaleDemo/Core/Miscellaneous/CameraShake/Movement/Moving/Sprinting/CS_ForwardPitch_Sprinting.CS_ForwardPitch_Sprinting_C" :!type "CameraShake Class Reference") :`NewEnumerator1` "/Game/DarkTaleDemo/Core/Miscellaneous/CameraShake/Movement/Moving/Crouching/CS_ForwardPitch_Crouching.CS_ForwardPitch_Crouching_C")))
      (set `self.AmbientForward_CS` _returnvalue_2)
      (bind _returnvalue_3 (`PlayerCameraManager.PlayCameraShake` :`self` (`self.Camera_Manager`) :`ShakeClass` (select `/Game/DarkTaleDemo/Core/Miscellaneous/MovementEnums/EStance` (`self.Player_Stance`) :`NewEnumerator0` (select `/Game/DarkTaleDemo/Core/Miscellaneous/MovementEnums/EGaitTypes` (`self.Player_Gait`) :`NewEnumerator1` "/Game/DarkTaleDemo/Core/Miscellaneous/CameraShake/Movement/Moving/Running/CS_SidewaysRoll_Running.CS_SidewaysRoll_Running_C" :`NewEnumerator0` "/Game/DarkTaleDemo/Core/Miscellaneous/CameraShake/Movement/Moving/Walking/CS_SidewaysRoll_Walking.CS_SidewaysRoll_Walking_C" :`NewEnumerator2` "/Game/DarkTaleDemo/Core/Miscellaneous/CameraShake/Movement/Moving/Sprinting/CS_SidewaysRoll_Sprinting.CS_SidewaysRoll_Sprinting_C" :!type "CameraShake Class Reference") :`NewEnumerator1` "/Game/DarkTaleDemo/Core/Miscellaneous/CameraShake/Movement/Moving/Crouching/CS_SidewaysRoll_Crouching.CS_SidewaysRoll_Crouching_C") :`Scale` 0.001))
      (set `self.AmbientSide_CS` _returnvalue_3))))

(fn `Stop_Ambient_CS`
  (params (Immediately :type Boolean))
  (bind _camera_manager (`self.Camera_Manager`))
  (`PlayerCameraManager.StopAllInstancesOfCameraShake` _camera_manager "/Game/DarkTaleDemo/Core/Miscellaneous/CameraShake/Movement/Moving/CS_AmbientNoise_Parent.CS_AmbientNoise_Parent_C" Immediately)
  (`PlayerCameraManager.StopAllInstancesOfCameraShake` _camera_manager "/Game/DarkTaleDemo/Core/Miscellaneous/CameraShake/Movement/Moving/CS_AmbientForwardPitch_Parent.CS_AmbientForwardPitch_Parent_C" Immediately)
  (`PlayerCameraManager.StopAllInstancesOfCameraShake` _camera_manager "/Game/DarkTaleDemo/Core/Miscellaneous/CameraShake/Movement/Moving/CS_AmbientSidewaysRoll_Parent.CS_AmbientSidewaysRoll_Parent_C" Immediately))

(fn `Stop_Idle_CS`
  (params (bImmediately :type Boolean))
  (`PlayerCameraManager.StopAllInstancesOfCameraShake` (`self.Camera_Manager`) "/Game/DarkTaleDemo/Core/Miscellaneous/CameraShake/Movement/Idle/Gaits/CS_IdleNoiseParent.CS_IdleNoiseParent_C" bImmediately))

(fn `Update_CameraShakes`
  (locals (Input_FB_Value :type "Float (double-precision)") (Input_RL_Value :type "Float (double-precision)"))
  (`/Engine/EditorBlueprintResources/StandardMacros.IsValid` (`self.Camera_Manager`)
    (:`Is Valid`
      (`self.Switch_IsMoving`
        (:`T`
          (bind _playerh_character (`self.PlayerH_Character`)
            (:`then`
              (bind _returnvalue (`self.Calculate_SpeedIntensity_Scale` (`/Game/DarkTaleDemo/Core/Main/Characters/Player/BP_HumanChar.MoveFB` _playerh_character) (`/Game/DarkTaleDemo/Core/Main/Characters/Player/BP_HumanChar.MoveRL` _playerh_character)))
              (`|ExecutionSequence`
                (:`then_0`
                  (bind _ambiennoise_cs (`self.AmbienNoise_CS`)
                    (:`then`
                      (set `CameraShake.ShakeScale` _returnvalue _ambiennoise_cs))
                    (:`else`)))
                (:`then_1`
                  (bind _ambientforward_cs (`self.AmbientForward_CS`)
                    (:`then`
                      (set `CameraShake.ShakeScale` _returnvalue _ambientforward_cs))
                    (:`else`)))
                (:`then_2`
                  (bind _ambientside_cs (`self.AmbientSide_CS`)
                    (:`then`
                      (set `CameraShake.ShakeScale` (* _returnvalue (`self.AmbientRoll_Scale`)) _ambientside_cs))
                    (:`else`)))))
            (:`else`)))))))

(fn `Update_VelocityModifier`
  (locals (Offset :type "Float (double-precision)"))
  (bind _offset (`local.Offset`))
  (if (and (`KismetSystemLibrary.IsValid` (`self.Velocity_CamMod`)) (`KismetSystemLibrary.IsValid` (`self.PlayerH_Character`)))
    (`self.Switch_IsMoving`
      (:`T`
        (set `local.Offset` (`self.CharacterRotation/VelocityDifference`))
        (set `/Game/DarkTaleDemo/Core/Miscellaneous/CameraModifiers/Movement/CMD_Velolcity.AdditiveRotation` (`KismetMathLibrary.ClampAxes2D` (`KismetMathLibrary.Vector2DInterpTo` (`/Game/DarkTaleDemo/Core/Miscellaneous/CameraModifiers/Movement/CMD_Velolcity.AdditiveRotation` (`self.Velocity_CamMod`)) (`KismetMathLibrary.MakeVector2D` (`self.Apply_SpeedCoef` (`self.Calculate_RollIntensity` _offset)) (`self.Apply_SpeedCoef` (`self.Calculate_PitchIntensity` _offset))) (`GameplayStatics.GetWorldDeltaSeconds`) 3.0) 0.0 20.0) (`self.Velocity_CamMod`)))
      (:`F`
        (if (not (`KismetMathLibrary.IsNearlyZero2D` (`/Game/DarkTaleDemo/Core/Miscellaneous/CameraModifiers/Movement/CMD_Velolcity.AdditiveRotation` (`self.Velocity_CamMod`)) 0.001))
          (set `/Game/DarkTaleDemo/Core/Miscellaneous/CameraModifiers/Movement/CMD_Velolcity.AdditiveRotation` (`KismetMathLibrary.Vector2DInterpTo` (`/Game/DarkTaleDemo/Core/Miscellaneous/CameraModifiers/Movement/CMD_Velolcity.AdditiveRotation` (`self.Velocity_CamMod`)) (`KismetMathLibrary.MakeVector2D` 0.0) (`GameplayStatics.GetWorldDeltaSeconds`) 3.0) (`self.Velocity_CamMod`)))))))