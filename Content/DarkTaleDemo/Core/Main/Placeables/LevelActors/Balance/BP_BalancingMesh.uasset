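; BP_BalancingMesh is a placeable level actor that puts the player character into balancing on contact.
; When its BalancingMesh component is hit by a BP_HumanChar, it checks that the player's movement component is moving on the ground.
; It then sends StartBalance through an interface to the player character, fetched via macro library helpers rather than from the hit actor.
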(event `self.ReceiveTick`
  (params (DeltaSeconds :type "Float (single-precision)"))
  (`parent.ReceiveTick` DeltaSeconds))

(event `self.BalancingMesh.OnComponentHit`
  (params (HitComponent :type "PrimitiveComponent Object Reference") (OtherActor :type "Actor Object Reference") (OtherComp :type "PrimitiveComponent Object Reference") (NormalImpulse :type "Vector Structure") (Hit :type "HitResult Structure (by ref)"))
  (cast `/Game/DarkTaleDemo/Core/Main/Characters/Player/BP_HumanChar` OtherActor)
  (if (`NavMovementComponent.IsMovingOnGround` (`/Game/DarkTaleDemo/Core/Main/MacroLibrary/BPML_Actor.Get_PlayerMovComp_BPML`))
    (`self.Start_Balance_BPIF` (`/Game/DarkTaleDemo/Core/Main/MacroLibrary/BPML_Actor.Get_DPlayerCharacter_BPML`))))

(fn `UserConstructionScript`
  (`parent.UserConstructionScript`))