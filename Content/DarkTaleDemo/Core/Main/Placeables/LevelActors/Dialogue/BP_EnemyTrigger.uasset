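; BP_EnemyTrigger is a placeable level actor that, as written, acts as a debug indicator for the player's danger state.
; Every Tick it reads IsInDanger from the default player controller and switches its PointLight bright when true, dark when false.
; A Check_PlayerController helper returns the PC_Default of a player-controlled pawn, but nothing in this graph calls it, and no overlap logic is active.
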(event `self.ReceiveTick`
  (params (DeltaSeconds :type "Float (single-precision)"))
  (bind _pointlight (`self.PointLight`))
  ;[1 1 1] Debug
  (if (`/Game/DarkTaleDemo/Core/Main/Control/Controllers/PC_Default.is_in_danger` (`/Game/DarkTaleDemo/Core/Main/MacroLibrary/BPML_Actor.Get_DPController_BPML`))
    (`LightComponent.SetIntensity` _pointlight 5000.0)
    (else
      (`LightComponent.SetIntensity` _pointlight 0.0))))

(fn `UserConstructionScript`)