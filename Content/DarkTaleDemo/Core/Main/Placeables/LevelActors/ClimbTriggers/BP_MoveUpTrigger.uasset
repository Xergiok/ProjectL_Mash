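; Climb trigger that lets the human player character snap onto and off a ladder with the main action while inside its interaction volume.
; Snapping enables actor input and switches movement to Flying with climb speed and capsule damping; the MouseWheelAxis input moves the character vertically with camera shake.
; Jump detaches and launches the character.
; PushForwardBox flags a top exit, so leaving the interaction volume runs a timeline sliding the character horizontally toward PushLocation.
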(event `/Game/DarkTaleDemo/Core/Main/Interfaces/Components/BPI_BaseInteraction.Main_Action_BPIF`
  (`/Engine/EditorBlueprintResources/StandardMacros.Gate` true :!label _label
    (:`Exit`
      (if (`self.PlayerSnapped`)
        (`self.Get Off Ladder`)
        (else
          (`self.Snap to ladder`))))))

(event `self.InteractionCollision.OnComponentBeginOverlap`
  (params (OverlappedComponent :type "PrimitiveComponent Object Reference") (OtherActor :type "Actor Object Reference") (OtherComp :type "PrimitiveComponent Object Reference") (OtherBodyIndex :type Integer) (bFromSweep :type Boolean) (SweepResult :type "HitResult Structure (by ref)"))
  (cast `/Game/DarkTaleDemo/Core/Main/Characters/Player/BP_HumanChar` OtherActor)
  (goto _label :!via `Open`))

(event `self.InteractionCollision.OnComponentEndOverlap`
  (params (OverlappedComponent :type "PrimitiveComponent Object Reference") (OtherActor :type "Actor Object Reference") (OtherComp :type "PrimitiveComponent Object Reference") (OtherBodyIndex :type Integer))
  (cast `/Game/DarkTaleDemo/Core/Main/Characters/Player/BP_HumanChar` OtherActor)
  (if (`self.Should_get_off_top`)
    (`self.LeaveLadderTop`)
    (elif (`self.PlayerSnapped`)
      (`self.Get Off Ladder`)
      (else
        (goto _label :!via `Close`)))))

(event `Snap to ladder`
  (set `self.PlayerSnapped` true)
  (`/Game/DarkTaleDemo/Core/Main/FunctionLibrary/BPFL_ControlInput.Set_ActorActionInput_BPFL` self true)
  (`CharacterMovementComponent.SetMovementMode` (`Character.CharacterMovement` (`/Game/DarkTaleDemo/Core/Main/MacroLibrary/BPML_Actor.Get_DPlayerCharacter_BPML`)) "MOVE_Flying" 0)
  (`PrimitiveComponent.SetLinearDamping` (`Character.CapsuleComponent` (`/Game/DarkTaleDemo/Core/Main/MacroLibrary/BPML_Actor.Get_DPlayerCharacter_BPML`)) (`self.Capsule_LD`))
  (set `CharacterMovementComponent.MaxFlySpeed` (`self.ClimbSpeed`) (`Character.CharacterMovement` (`/Game/DarkTaleDemo/Core/Main/MacroLibrary/BPML_Actor.Get_DPlayerCharacter_BPML`))))

(event `Get Off Ladder`
  (set `self.PlayerSnapped` false)
  (`/Game/DarkTaleDemo/Core/Main/FunctionLibrary/BPFL_ControlInput.Set_ActorActionInput_BPFL` self)
  (`CharacterMovementComponent.SetMovementMode` (`Character.CharacterMovement` (`/Game/DarkTaleDemo/Core/Main/MacroLibrary/BPML_Actor.Get_DPlayerCharacter_BPML`)) "MOVE_Walking" 0)
  (`PrimitiveComponent.SetLinearDamping` (`Character.CapsuleComponent` (`/Game/DarkTaleDemo/Core/Main/MacroLibrary/BPML_Actor.Get_DPlayerCharacter_BPML`)) 0.01)
  (`PlayerController.ClientStopCameraShake` (`/Game/DarkTaleDemo/Core/Main/MacroLibrary/BPML_Actor.Get_DPController_BPML`) "/Game/DarkTaleDemo/Core/Miscellaneous/CameraShake/CS_Ladder.CS_Ladder_C" false))

(event `InputAxisKey|MouseWheelAxis`
  (params (AxisValue :type "Float (single-precision)"))
  (bind _pclass (`/Game/DarkTaleDemo/Core/Main/MacroLibrary/BPML_Actor.Get_DPlayerCharacter_BPML`))
  (if (== AxisValue 0.0)
    (`PlayerController.ClientStopCameraShake` (`/Game/DarkTaleDemo/Core/Main/MacroLibrary/BPML_Actor.Get_DPController_BPML`) "/Game/DarkTaleDemo/Core/Miscellaneous/CameraShake/CS_Ladder.CS_Ladder_C" false)
    (else
      (`Pawn.AddMovementInput` _pclass (`self.GetActorUpVector` _pclass) AxisValue false)
      (`PlayerController.ClientStartCameraShake` :`self` (`/Game/DarkTaleDemo/Core/Main/MacroLibrary/BPML_Actor.Get_DPController_BPML`) :`Shake` "/Game/DarkTaleDemo/Core/Miscellaneous/CameraShake/CS_Ladder.CS_Ladder_C"))))

(event `InputAction|Jump`
  (params (Key :type "Key Structure"))
  (bind _pclass (`/Game/DarkTaleDemo/Core/Main/MacroLibrary/BPML_Actor.Get_DPlayerCharacter_BPML`))
  (bind _jumpamount (`self.JumpAmount`))
  (bind (_returnvalue_x _returnvalue_y) (`KismetMathLibrary.BreakVector` (* (`SceneComponent.GetForwardVector` (`Character.CapsuleComponent` _pclass)) _jumpamount)))
  (:`Pressed`
    (`self.Get Off Ladder`)
    (`Character.LaunchCharacter` _pclass (`KismetMathLibrary.MakeVector` _returnvalue_x _returnvalue_y _jumpamount) false false)))

(event `self.PushForwardBox.OnComponentBeginOverlap`
  (params (OverlappedComponent :type "PrimitiveComponent Object Reference") (OtherActor :type "Actor Object Reference") (OtherComp :type "PrimitiveComponent Object Reference") (OtherBodyIndex :type Integer) (bFromSweep :type Boolean) (SweepResult :type "HitResult Structure (by ref)"))
  (cast `/Game/DarkTaleDemo/Core/Main/Characters/Player/BP_HumanChar` OtherActor)
  (if (`self.PlayerSnapped`)
    (set `self.Should_get_off_top` true)))

(event `self.PushForwardBox.OnComponentEndOverlap`
  (params (OverlappedComponent :type "PrimitiveComponent Object Reference") (OtherActor :type "Actor Object Reference") (OtherComp :type "PrimitiveComponent Object Reference") (OtherBodyIndex :type Integer))
  (cast `/Game/DarkTaleDemo/Core/Main/Characters/Player/BP_HumanChar` OtherActor)
  (if (`self.PlayerSnapped`)
    (set `self.Should_get_off_top` false)
    (`self.Get Off Ladder`)))

(event `LeaveLadderTop`
  (bind _pclass (`/Game/DarkTaleDemo/Core/Main/MacroLibrary/BPML_Actor.Get_DPlayerCharacter_BPML`))
  (bind (_returnvalue_x _returnvalue_y) (`KismetMathLibrary.BreakVector` (`SceneComponent.K2_GetComponentLocation` (`self.PushLocation`))))
  (bind _returnvalue (`self.K2_GetActorLocation` _pclass))
  (bind (_direction _anim) (`Timeline|LeaveLadder_Timeline` :!via `PlayFromStart`)
    (:`Update`
      (`self.K2_SetActorLocation` _pclass (`KismetMathLibrary.VLerp` _returnvalue (`KismetMathLibrary.MakeVector` _returnvalue_x _returnvalue_y (.z _returnvalue)) _anim) false false))))

(fn `UserConstructionScript`
  (`parent.UserConstructionScript`)
  (set `self.PlayerSnapped` false))