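; BP_PainTrigger is a placeable box trigger that repeatedly applies pure damage to a pawn standing inside it.
; Box overlap stores the most recent pawn, optionally damages it on entry, and starts a looping timer at the configured pain interval.
; Each tick damages that pawn through PureDamageDealtAComponent.
; Only one pawn is tracked at a time, and its exit clears the reference and the current timer.
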(event `self.Box.OnComponentBeginOverlap`
  (params (OverlappedComponent :type "PrimitiveComponent Object Reference") (OtherActor :type "Actor Object Reference") (OtherComp :type "PrimitiveComponent Object Reference") (OtherBodyIndex :type Integer) (bFromSweep :type Boolean) (SweepResult :type "HitResult Structure (by ref)"))
  (bind _aspawn (cast `Pawn` OtherActor))
  (set `self.Last_Overlaped_Pawn` _aspawn)
  (if (`self.EntryPain`)
    (`self.PainTick`))
  (bind _returnvalue (`KismetSystemLibrary.K2_SetTimerDelegate` (delegate `PainTick`) (`self.Pain_Interval`) true))
  (set `self.Pain_Tick_timer` _returnvalue))

(event `PainTick`
  (bind _last_overlaped_pawn (`self.Last_Overlaped_Pawn`))
  (`/Engine/EditorBlueprintResources/StandardMacros.IsValid` _last_overlaped_pawn
    (:`Is Valid`
      (`/Game/DarkTaleDemo/Core/Main/Components/DamageSystem/BP_PureDamageDealt_AC.Apply_PureDamageFC` (`self.PureDamageDealt_AComponent`) _last_overlaped_pawn null))))

(event `self.Box.OnComponentEndOverlap`
  (params (OverlappedComponent :type "PrimitiveComponent Object Reference") (OtherActor :type "Actor Object Reference") (OtherComp :type "PrimitiveComponent Object Reference") (OtherBodyIndex :type Integer))
  (if (== OtherActor (`self.Last_Overlaped_Pawn`))
    (set `self.Last_Overlaped_Pawn` null)
    (`KismetSystemLibrary.K2_ClearAndInvalidateTimerHandle` (`self.Pain_Tick_timer`))))

(fn `UserConstructionScript`)