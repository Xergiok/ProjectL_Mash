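; Temporary-looking dialogue actor that shows a WBP_Options choice widget when interacted with and registers itself as the game instance's SpeakingActor.
; Each tick, the widget is offset by camera rotation and turned to face the camera.
; Interaction swaps action input from player character to actor, whose four dialogue keys trigger the widget's button cases and restore player input.
; Deinitialisation hides the widget; the speech case events only print a placeholder string.
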(event `self.ReceiveTick`
  (params (DeltaSeconds :type "Float (single-precision)"))
  (bind (_location _rotation) (`/Game/DarkTaleDemo/Core/Main/FunctionLibrary/BPFL_Camera.Get_CurrentCamera_Location/Rotation_BPFL` 0))
  (bind _options_act (`self.options_act`))
  ;[1 1 1] widget rotation (can be improved)
  (`SceneComponent.K2_SetRelativeLocationAndRotation` _options_act (`KismetMathLibrary.GreaterGreater_VectorRotator` (0.0 100.0 90.0) _rotation) (`KismetMathLibrary.FindLookAtRotation` (`SceneComponent.K2_GetComponentLocation` _options_act) _location) false false))

(event `self.ReceiveBeginPlay`
  (`Widget.SetVisibility` (`WidgetComponent.GetUserWidgetObject` (`self.options_act`)) "Hidden"))

(event `InputAction|Dialogue1`
  (params (Key :type "Key Structure"))
  ;[1 1 1] dialogue choice (bind 1-4) + cancel
  (:`Pressed`
    (bind _aswbp_options (cast `/Game/DarkTaleDemo/Core/Widget/Dialogue/WBP_Options` (`WidgetComponent.GetUserWidgetObject` (`self.options_act`))))
    (`/Game/DarkTaleDemo/Core/Widget/Dialogue/WBP_Options.buttoncase1` _aswbp_options)
    (`self.Switch_DialogInput` false)))

(event `InputAction|Dialogue2`
  (params (Key :type "Key Structure"))
  ;[1 1 1] dialogue choice (bind 1-4) + cancel
  (:`Pressed`
    (bind _aswbp_options (cast `/Game/DarkTaleDemo/Core/Widget/Dialogue/WBP_Options` (`WidgetComponent.GetUserWidgetObject` (`self.options_act`))))
    (`/Game/DarkTaleDemo/Core/Widget/Dialogue/WBP_Options.buttoncase2` _aswbp_options)
    (`self.Switch_DialogInput` false)))

(event `InputAction|Dialogue3`
  (params (Key :type "Key Structure"))
  ;[1 1 1] dialogue choice (bind 1-4) + cancel
  (:`Pressed`
    (bind _aswbp_options (cast `/Game/DarkTaleDemo/Core/Widget/Dialogue/WBP_Options` (`WidgetComponent.GetUserWidgetObject` (`self.options_act`))))
    (`/Game/DarkTaleDemo/Core/Widget/Dialogue/WBP_Options.buttoncase3` _aswbp_options)
    (`self.Switch_DialogInput` false)))

(event `InputAction|Dialogue4`
  (params (Key :type "Key Structure"))
  ;[1 1 1] dialogue choice (bind 1-4) + cancel
  (:`Pressed`
    (bind _aswbp_options (cast `/Game/DarkTaleDemo/Core/Widget/Dialogue/WBP_Options` (`WidgetComponent.GetUserWidgetObject` (`self.options_act`))))
    (`/Game/DarkTaleDemo/Core/Widget/Dialogue/WBP_Options.buttoncase4` _aswbp_options)
    (`self.Switch_DialogInput` false)))

(event `/Game/DarkTaleDemo/Core/Main/Interfaces/Items/BPI_Interactable.Interact`
  (params (Instigator :type "Actor Object Reference"))
  (bind _returnvalue (`WidgetComponent.GetUserWidgetObject` (`self.options_act`)))
  (bind _asbp_default_game_inst (cast `/Game/DarkTaleDemo/Core/Main/GameBase/BP_DefaultGameInst` (`GameplayStatics.GetGameInstance`)))
  (set `/Game/DarkTaleDemo/Core/Main/GameBase/BP_DefaultGameInst.speaking_actor` self _asbp_default_game_inst)
  (`Widget.SetVisibility` _returnvalue "Visible")
  (bind _aswbp_options (cast `/Game/DarkTaleDemo/Core/Widget/Dialogue/WBP_Options` _returnvalue))
  (`/Game/DarkTaleDemo/Core/Widget/Dialogue/WBP_Options.Initialisation` _aswbp_options)
  (`self.Switch_DialogInput` true))

(event `Deinitialisation`
  (`Widget.SetVisibility` (`WidgetComponent.GetUserWidgetObject` (`self.options_act`)) "Hidden"))

(event `/Game/DarkTaleDemo/Core/Main/Interfaces/BPI_DialogueChoice.speechcase1`
  (`KismetSystemLibrary.PrintString` "cock" :!label _label))

(event `/Game/DarkTaleDemo/Core/Main/Interfaces/BPI_DialogueChoice.speechcase2`
  (goto _label))

(event `/Game/DarkTaleDemo/Core/Main/Interfaces/BPI_DialogueChoice.speechcase3`
  (goto _label))

(event `/Game/DarkTaleDemo/Core/Main/Interfaces/BPI_DialogueChoice.speechcase4`
  (goto _label))

(fn `Switch_DialogInput`
  (params (Enable :type Boolean))
  (`/Game/DarkTaleDemo/Core/Main/FunctionLibrary/BPFL_ControlInput.Set_ActorActionInput_BPFL` self Enable)
  (`/Game/DarkTaleDemo/Core/Main/FunctionLibrary/BPFL_ControlInput.Set_PlayerCharacterActionInput_BPFL` (not Enable)))

(fn `UserConstructionScript`)