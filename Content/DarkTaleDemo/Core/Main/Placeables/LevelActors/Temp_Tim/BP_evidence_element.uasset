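; BP_evidence_element is a placeable evidence object that applies a camera modifier while focused.
; On focus in, it reaches the instigator's CM_Default camera manager through PC_Default, adds a CMD_Evidence modifier and stores it.
; On focus out, it disables that modifier non-immediately, allowing a blend-out, and removes it only if its alpha is already zero at that moment.
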(event `/Game/DarkTaleDemo/Core/Main/Interfaces/Items/BPI_Focusable.FocusedInto_BPIF`
  (params (Instigator :type "Actor Object Reference"))
  (`/Engine/EditorBlueprintResources/StandardMacros.IsValid` Instigator
    (:`Is Valid`
      (bind _aspc_default (cast `/Game/DarkTaleDemo/Core/Main/Control/Controllers/PC_Default` (`self.GetInstigatorController` Instigator)))
      (bind _ascm_default (cast `/Game/DarkTaleDemo/Core/Main/Control/CameraManagers/CM_Default` (`PlayerController.PlayerCameraManager` _aspc_default)))
      (bind _returnvalue (`PlayerCameraManager.AddNewCameraModifier` _ascm_default "/Game/DarkTaleDemo/Core/Miscellaneous/CameraModifiers/Items/CMD_Evidence.CMD_Evidence_C")))))

(event `/Game/DarkTaleDemo/Core/Main/Interfaces/Items/BPI_Focusable.FucusedOut_BPIF`
  (params (Instigator :type "Actor Object Reference"))
  (`/Engine/EditorBlueprintResources/StandardMacros.IsValid` Instigator
    (:`Is Valid`
      (bind _aspc_default (cast `/Game/DarkTaleDemo/Core/Main/Control/Controllers/PC_Default` (`self.GetInstigatorController` Instigator)))
      (bind _ascm_default (cast `/Game/DarkTaleDemo/Core/Main/Control/CameraManagers/CM_Default` (`PlayerController.PlayerCameraManager` _aspc_default)))
      (`CameraModifier.DisableModifier` (stale `/Game/DarkTaleDemo/Core/Main/Interfaces/Items/BPI_Focusable.FocusedInto_BPIF` _returnvalue) false)
      (if (== (`CameraModifier.Alpha` (stale `/Game/DarkTaleDemo/Core/Main/Interfaces/Items/BPI_Focusable.FocusedInto_BPIF` _returnvalue)) 0.0)
        (`PlayerCameraManager.RemoveCameraModifier` _ascm_default (stale `/Game/DarkTaleDemo/Core/Main/Interfaces/Items/BPI_Focusable.FocusedInto_BPIF` _returnvalue))))))

(fn `UserConstructionScript`)