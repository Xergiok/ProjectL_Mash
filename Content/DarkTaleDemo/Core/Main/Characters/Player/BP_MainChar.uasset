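; BP_MainChar is the main player character, a thin child Blueprint that leaves most behavior to its parent class.
; Its construction script makes ClothingMesh follow the body Mesh through master pose, then sets the inherited data table name to "MainCharacter" before running the parent's construction script.
; BeginPlay and Tick only forward to the parent, and the Possessed event is empty.
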(event `self.ReceivePossessed`
  (params (NewController :type "Controller Object Reference")))

(event `self.ReceiveBeginPlay`
  (`parent.ReceiveBeginPlay`))

(event `self.ReceiveTick`
  (params (DeltaSeconds :type "Float (single-precision)"))
  (`parent.ReceiveTick` DeltaSeconds))

(fn `Init Parent Variables`
  (set `self.Child_DataTableName` "MainCharacter"))

(fn `UserConstructionScript`
  (`SkinnedMeshComponent.SetLeaderPoseComponent` (`self.ClothingMesh`) (`self.Mesh`) false)
  (`self.Init Parent Variables`)
  (`parent.UserConstructionScript`))