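; Base NPC Blueprint that provides health, hitbox-scaled damage and ragdoll death, with health set to maximum on BeginPlay.
; CalculateDamage applies a head multiplier, clamps health and calls Death at zero, though nothing in this file actively calls it.
; Death switches the mesh to simulated ragdoll physics, then destroys the actor after a delay.
; The any, point and radial damage interface functions are stubs that report failure.
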(event `self.ReceiveBeginPlay`
  (`parent.ReceiveBeginPlay`)
  (`self.Set_DefaultValues`))

(event `Destroy_with_delay`
  (params (Delay :type "Float (double-precision)") (Target :type "Actor Object Reference"))
  (`KismetSystemLibrary.Delay` Delay)
  (`self.K2_DestroyActor` Target))

(fn `Calculate_Damage`
  (params (`Apply damage` :type "Float (double-precision)") (`Hitbox on enum` :type "/Game/DarkTaleDemo/Core/Miscellaneous/Bones/Hitbox/EHitboxNPC Enum" :default "NewEnumerator0") (Instigator :type "Actor Object Reference"))
  (bind _returnvalue (- (`self.Current_Health`) (`self.Select_AmountofDamage` `Apply damage` `Hitbox on enum`)))
  (bind _output_get (set `self.Current_Health` (`KismetMathLibrary.FClamp` (`KismetMathLibrary.SelectFloat` 0.0 _returnvalue (<= _returnvalue 0.0)) 0.0 (`self.Max_Health`))))
  (if (== _output_get 0.0)
    (`self.Death`)))

(fn `Death`
  (bind _mesh (`self.Mesh`))
  (`PrimitiveComponent.SetCollisionEnabled` _mesh "PhysicsOnly")
  (`PrimitiveComponent.SetCollisionProfileName` _mesh "Ragdoll" true)
  (`SkeletalMeshComponent.SetAllBodiesSimulatePhysics` _mesh true)
  (`SkeletalMeshComponent.SetAllBodiesPhysicsBlendWeight` _mesh 1.0 false)
  (`self.Destroy_with_delay` (`self.TimeDelay`) self))

(fn `Process_AnyDamage_BPIF`
  (params (Scale :type "Float (double-precision)") (Reciever :type "Actor Object Reference") (Instigator :type "Controller Object Reference") (Causer :type "Actor Object Reference"))
  (returns (Successfully :type Boolean) (Amplitude :type "Float (double-precision)") (Form :type "/Game/DarkTaleDemo/Core/Main/Components/DamageSystem/EDamageForm Enum"))
  (return false 0.0 "NewEnumerator0"))

(fn `Process_PointDamage_BPIF`
  (params (Scale :type "Float (double-precision)") (Reciever :type "Actor Object Reference") (Instigator :type "Controller Object Reference") (Causer :type "Actor Object Reference") (Location :type "Vector Structure") (Direction :type "Vector Structure") (Component :type "PrimitiveComponent Object Reference") (Bone :type Name))
  (returns (Successfully :type Boolean) (Amplitude :type "Float (double-precision)") (Form :type "/Game/DarkTaleDemo/Core/Main/Components/DamageSystem/EDamageForm Enum"))
  (return false 0.0 "NewEnumerator0"))

(fn `Process_RadialDamage_BPIF`
  (params (Scale :type "Float (double-precision)") (Reciever :type "Actor Object Reference") (Instigator :type "Controller Object Reference") (Causer :type "Actor Object Reference") (Origin :type "Vector Structure") (HitInfo :type "HitResult Structure"))
  (returns (Successfully :type Boolean) (Amplitude :type "Float (double-precision)") (Form :type "/Game/DarkTaleDemo/Core/Main/Components/DamageSystem/EDamageForm Enum"))
  (return false 0.0 "NewEnumerator0"))

(fn `Select_AmountofDamage`
  (params (Value :type "Float (double-precision)") (Hitbox :type "/Game/DarkTaleDemo/Core/Miscellaneous/Bones/Hitbox/EHitboxNPC Enum" :default "NewEnumerator0"))
  (returns (ReturnValue :type "Float (double-precision)"))
  (return (select `/Game/DarkTaleDemo/Core/Miscellaneous/Bones/Hitbox/EHitboxNPC` Hitbox :`NewEnumerator0` Value :`NewEnumerator1` (* Value (`self.HeadDamage_Multiplier`)))))

(fn `Set_DefaultValues`
  (set `self.Current_Health` (`self.Max_Health`)))

(fn `UserConstructionScript`
  (`parent.UserConstructionScript`))