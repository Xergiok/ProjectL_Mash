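; Camera modifier that applies a vignette when the player's camera looks at an evidence element.
; Each update, a short visibility trace from the camera checks for BP_evidence_element and derives intensity from how directly the view faces the hit surface.
; That intensity becomes the post-process blend weight, dropping to zero without an evidence hit.
; Debug traces and prints remain, including a placeholder message saying screen blur belongs here.
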(fn `BlueprintModifyPostProcess`
  (params (DeltaTime :type "Float (double-precision)"))
  (returns (PostProcessBlendWeight :type "Float (double-precision)") (PostProcessSettings :type "PostProcessSettings Structure"))
  (cast `/Game/DarkTaleDemo/Core/Main/Control/PlayerControllers/PC_Default` (`GameplayStatics.GetPlayerController` 0))
  (bind _intensity (`self.CalculateIntensity`))
  (`|ExecutionSequence`
    (:`then_0`
      (if (!= _intensity 0.0)
        (`KismetSystemLibrary.PrintString` (`KismetStringLibrary.Concat_StrStr` "Intensity: " (`KismetStringLibrary.Conv_DoubleToString` _intensity)) true true (struct :`G` 0.66 :`B` 1.0 :`A` 1.0) 0.0)
        (else
          (return _intensity (make `PostProcessSettings` :`VignetteIntensity` 2.0)))))
    (:`then_1`
      (return _intensity (make `PostProcessSettings` :`VignetteIntensity` 2.0)))))

(fn `CalculateIntensity`
  (returns (Intensity :type "Float (double-precision)"))
  (bind (_location _rotation) (`/Game/DarkTaleDemo/Core/Main/FunctionLibrary/BPFL_Camera.Get_CurrentCamera_Location/Rotation_BPFL` 0))
  (bind _returnvalue (`KismetMathLibrary.GetForwardVector` _rotation))
  (bind _outhit (`KismetSystemLibrary.LineTraceSingle` :`Start` _location :`End` (+ _location (* _returnvalue 500.0)) :`TraceChannel` "TraceTypeQuery1" :`DrawDebugType` "ForDuration" :`TraceColor` (struct :`R` 1.0 :`B` 0.90008 :`A` 1.0)))
  (bind (_bblockinghit _binitialoverlap _time _distance _location_2 _impactpoint _normal _impactnormal _physmat _hitactor) (`GameplayStatics.BreakHitResult` _outhit))
  (cast `/Game/DarkTaleDemo/Core/Main/World/LevelActors/Temp_Tim/BP_evidence_element` _hitactor
    (:`then`
      (`KismetSystemLibrary.PrintString` "здесь должно быть размытие экрана" true true (struct :`G` 0.66 :`B` 1.0 :`A` 1.0) 0.0)
      (return (* (`KismetMathLibrary.Dot_VectorVector` _impactnormal _returnvalue) -1.0)))
    (:`CastFailed`
      (return 0.0))))